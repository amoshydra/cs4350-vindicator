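; BP_Sound_Manager is an actor that switches music between combat and non-combat tracks based on whether enemies are present.
; On BeginPlay it binds CheckEnemyCount to the game instance's enemy added and removed events.
; That check reads the Enemies array length, then starts the matching track if not already playing and fades the other out.
; A separate Start event plays the non-combat track.
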(event Custom|Check%20Enemy%20Count
  (params (AddedEnemy :type BP%20Enemy%20Base%20Object%20Reference))
  (bind _combat (Variables|Default|Getcombat))
  (bind _non_combat (Variables|Default|Getnon%20combat))
  (if (== (Utilities|Array|Length (Variables|/Game/Blueprints/BP_GameInstance.BP_GameInstance_C|GetEnemies (stale EventBeginPlay _asbp_game_instance))) 0)
    (if (not (Audio|Components|Audio|IsPlaying _non_combat))
      (Audio|Components|Audio|Play _non_combat 0.0)
      (Audio|Components|Audio|FadeOut _combat 3.0 0.0 :!class /Script/Engine.AudioComponent))
    (elif (not (Audio|Components|Audio|IsPlaying _combat))
      (Audio|Components|Audio|Play _combat 0.0)
      (Audio|Components|Audio|FadeOut _non_combat 3.0 0.0 :!class /Script/Engine.AudioComponent))))

(event Custom|Start
  (Audio|Components|Audio|Play (Variables|Default|Getnon%20combat) 0.0))

(event EventBeginPlay
  (bind _asbp_game_instance (Utilities|Casting|CastToBP_GameInstance (Game|GetGameInstance)))
  (EventDispatchers|BindEventtoEnemyIsAdded _asbp_game_instance (delegate Custom|Check%20Enemy%20Count))
  (EventDispatchers|BindEventtoEnemyIsRemoved _asbp_game_instance (delegate Custom|Check%20Enemy%20Count)))

(event Collision|EventActorBeginOverlap
  (params (OtherActor :type Actor%20Object%20Reference)))

(event EventTick
  (params (DeltaSeconds :type Float%20%28single-precision%29)))

(fn ConstructionScript)