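; Enemy spawn point actor that spawns AI enemies at its location, once on BeginPlay if auto-activated or on a looping timer once Activate is called.
; Spawns continue up to a limit, where zero means unlimited, and can also trigger when an enemy dies.
; Each enemy's destruction updates the active count and fires EnemyKilled.
; When the limit is reached and none remain, it resets and broadcasts SpawnIsCompleted.
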(event Custom|AttemptToDispatchSpawnIsCompleted
  (Utilities|FlowControl|Sequence
    (:then_0
      (bind _canstillspawnenemy (CallFunction|CanStillSpawnEnemy)))
    (:then_1
      (bind _hasactiveenemy (CallFunction|HasActiveEnemy)))
    (:then_2
      (if (Math|Boolean|NORBoolean _canstillspawnenemy _hasactiveenemy)
        (CallFunction|DeactivateSpawning)
        (Default|CallSpawnIsCompleted)))))

(event Custom|AttemptToSpawnEnemy
  (bind _canstillspawnenemy (CallFunction|CanStillSpawnEnemy))
  (if _canstillspawnenemy
    (CallFunction|SpawnEnemy)))

(event Custom|Reset
  (Utilities|FlowControl|Sequence
    (:then_0
      (Variables|Default|SetCurrentSpawnCount 0)
      (Variables|Default|SetCurrentActiveEnemy 0))
    (:then_1
      (Utilities|Time|ClearandInvalidateTimerbyHandle (Variables|Default|GetTimer)))))

(event Custom|DeactivateSpawning
  (CallFunction|Reset))

(event Custom|OnDestroyed_Event_1
  (params (DestroyedActor :type Actor%20Object%20Reference))
  (CallFunction|OnEnemyDestroy)
  (Default|CallEnemyKilled))

(event Custom|OnEnemyDestroy
  (params (DestroyedActor :type BP%20Enemy%20Base%20Object%20Reference))
  (Utilities|FlowControl|Sequence
    (:then_0
      (Math|Integer|DecrementInt (Variables|Default|GetCurrentActiveEnemy)))
    (:then_1
      (if (Variables|Default|GetRespawnOnEnemyDead)
        (CallFunction|AttempttoSpawnEnemy)))
    (:then_2
      (CallFunction|AttempttoDispatchSpawnIsCompleted))))

(event Custom|SpawnEnemy
  (bind _defaultscenerootnode (Variables|Default|GetDefaultSceneRootNode))
  (bind _returnvalue (AI|SpawnAIFromClass (Variables|Default|GetEnemy) 0 (Transformation|GetWorldLocation _defaultscenerootnode) (Transformation|GetWorldRotation _defaultscenerootnode) true))
  (Utilities|FlowControl|Sequence
    (:then_0
      (Math|Integer|IncrementInt (Variables|Default|GetCurrentSpawnCount)))
    (:then_1
      (Math|Integer|IncrementInt (Variables|Default|GetCurrentActiveEnemy)))
    (:then_2
      (Game|AssignOnDestroyed _returnvalue (delegate Custom|OnDestroyed_Event_1)))))

(event EventBeginPlay
  (|CallParentFunction)
  (if (Variables|Default|GetAutoActivate)
    (CallFunction|AttempttoSpawnEnemy)))

(event Collision|EventActorBeginOverlap
  (params (OtherActor :type Actor%20Object%20Reference))
  (|CallParentFunction OtherActor))

(event EventTick
  (params (DeltaSeconds :type Float%20%28single-precision%29))
  (|CallParentFunction DeltaSeconds))

(event EventActivate
  (params (CurrentCheckpoint :type Integer))
  (if (Variables|Default|GetAutoActivate)
    (Variables|Default|SetAutoActivate false)
    (else
      (CallFunction|DeactivateSpawning)))
  (Utilities|FlowControl|Delay (Variables|Default|GetInitialSpawnDelay))
  (CallFunction|AttempttoSpawnEnemy)
  (bind _returnvalue (Utilities|Time|SetTimerbyFunctionName 0 "AttemptToSpawnEnemy" (Variables|Default|GetSpawnInterval) true))
  (Variables|Default|SetTimer _returnvalue))

(fn ConstructionScript
  (|CallParentFunction)
  (Utilities|FlowControl|Sequence
    (:then_0
      (if (< (Variables|Default|GetSpawnLimit) 0)
        (Variables|Default|SetSpawnLimit 0)))))

(fn CanStillSpawnEnemy
  (bind _spawnlimit (Variables|Default|GetSpawnLimit))
  (return (or (== 0 _spawnlimit) (< (Variables|Default|GetCurrentSpawnCount) _spawnlimit))))

(fn HasActiveEnemy
  (return (!= (Variables|Default|GetCurrentActiveEnemy) 0)))