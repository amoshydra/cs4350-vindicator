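; VR teleport checkpoint that shows a ring as a fixed landing destination for BP_VR_Pawn.
; Activate and Eavesdrop switch the ring, teleport permission and landing-point collision on and off.
; Overlap with the pawn's TeleportCylinder swaps the ring between lure and hover materials.
; RequestTeleportation moves the pawn to LandingTarget, offset by capsule half-height, then hides the ring and increments the checkpoint if it is the last destination.
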(event OnComponentBeginOverlap(ProjectionArcLandingPoint)
  (params (OverlappedComponent :type Primitive%20Component%20Object%20Reference) (OtherActor :type Actor%20Object%20Reference) (OtherComp :type Primitive%20Component%20Object%20Reference) (OtherBodyIndex :type Integer) (bFromSweep :type Boolean) (SweepResult :type Hit%20Result%20Structure%20%28by%20ref%29))
  (CallFunction|FilterValidComponent OtherActor OtherComp)
  (CallFunction|ShowHoverEffect))

(event OnComponentEndOverlap(ProjectionArcLandingPoint)
  (params (OverlappedComponent :type Primitive%20Component%20Object%20Reference) (OtherActor :type Actor%20Object%20Reference) (OtherComp :type Primitive%20Component%20Object%20Reference) (OtherBodyIndex :type Integer))
  (CallFunction|FilterValidComponent OtherActor OtherComp)
  (CallFunction|HideHoverEffect))

(event Custom|PawnTeleported
  (if (Variables|Default|GetisLastDestination)
    (Default|CallIncrementCheckpoint)))

(event EventActivate
  (params (CurrentCheckpoint :type Integer))
  (CallFunction|ShowTeleportationRing)
  (Variables|Default|SetisTeleportationAllow true)
  (Collision|SetCollisionEnabled (Variables|Default|GetProjectionArcLandingPoint) "QueryOnly")
  (CallFunction|HideHoverEffect))

(event EventTick
  (params (DeltaSeconds :type Float%20%28single-precision%29)))

(event EventEavesdrop
  (params (OtherCheckpoint :type Integer))
  (CallFunction|HideTeleportationRing)
  (Variables|Default|SetisTeleportationAllow false)
  (Collision|SetCollisionEnabled (Variables|Default|GetProjectionArcLandingPoint) "NoCollision"))

(fn ConstructionScript
  (Rendering|Material|SetMaterial (Variables|Default|GetVisualCylinder) 0 (Variables|Default|GetTextureOnLure))
  (CallFunction|HideTeleportationRing))

(fn RequestTeleportation
  (params (Pawn :type Pawn%20Object%20Reference))
  (bind _asbp_vr_pawn (Utilities|Casting|CastToBP_VR_Pawn Pawn)
    (:then
      _)
    (:CastFailed
      _))
  (if (Variables|Default|GetisTeleportationAllow)
    (bind _returnvalue (Transformation|Teleport _asbp_vr_pawn (+ (Transformation|GetWorldLocation (Variables|Default|GetLandingTarget)) (Math|Vector|MakeVector 0.0 0.0 (Variables|/Script/Engine.CapsuleComponent|GetCapsuleHalfHeight (Variables|/Game/PlayerController/BP_VR_Pawn.BP_VR_Pawn_C|GetCapsule _asbp_vr_pawn)))) (Transformation|GetActorRotation _asbp_vr_pawn)))
    (if _returnvalue
      (CallFunction|PawnTeleported)
      (CallFunction|HideTeleportationRing)))
  (return (or _returnvalue (Variables|Default|GetisTeleportationAllow))))

(fn FilterValidComponent
  (params (Other%20Actor :type Object%20Object%20Reference) (Other%20Component :type Object%20Object%20Reference))
  (bind _asbp_vr_pawn (Utilities|Casting|CastToBP_VR_Pawn Other%20Actor))
  (if (== (Variables|/Game/PlayerController/BP_VR_Pawn.BP_VR_Pawn_C|GetTeleportCylinder _asbp_vr_pawn) Other%20Component)
    (return)))

(fn ShowTeleportationRing
  (Rendering|SetVisibility (Variables|Default|GetVisualCylinder) true false))

(fn HideTeleportationRing
  (Rendering|SetVisibility (Variables|Default|GetVisualCylinder) false false))

(fn ShowHoverEffect
  (Rendering|Material|SetMaterial (Variables|Default|GetVisualCylinder) 0 (Variables|Default|GetTextureOnHover)))

(fn HideHoverEffect
  (Rendering|Material|SetMaterial (Variables|Default|GetVisualCylinder) 0 (Variables|Default|GetTextureOnLure)))