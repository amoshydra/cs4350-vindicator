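; BP_LevelActor_IceGate is an ice gate level actor that slides its GateY component vertically between EndY and zero.
; Each Activate stores the current height, flips a FlipFlop to pick the target, and restarts a timeline that lerps relative Z there, so retriggering mid-move reverses from the current position.
; BeginPlay calls Activate three times on hardcoded delays, toggling the gate automatically.
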(event EventBeginPlay
  (|CallParentFunction)
  (Utilities|FlowControl|Delay 1.0)
  (CallFunction|Activate)
  (Utilities|FlowControl|Delay 0.2)
  (CallFunction|Activate)
  (Utilities|FlowControl|Delay 5.0)
  (CallFunction|Activate))

(event Collision|EventActorBeginOverlap
  (params (OtherActor :type Actor%20Object%20Reference))
  (|CallParentFunction OtherActor))

(event EventTick
  (params (DeltaSeconds :type Float%20%28single-precision%29))
  (|CallParentFunction DeltaSeconds))

(event EventActivate
  (params (CurrentCheckpoint :type Integer))
  (Variables|Default|SetOldY (.z (Variables|/Script/Engine.SceneComponent|GetRelativeLocation (Variables|Default|GetGateY))))
  (bind _isa (Utilities|FlowControl|FlipFlop)
    (:A
      (bind _newtrack_0 (Timeline|Timeline_0 PlayFromStart)
        (:Update
          (Transformation|SetRelativeLocation (Variables|Default|GetGateY) (Math|Vector|MakeVector 0.0 0.0 (Math|Float|Lerp (Variables|Default|GetOldY) (Math|Float|SelectFloat (Variables|Default|GetEndY) 0.0 _isa) _newtrack_0)) false false))))
    (:B
      (Timeline|Timeline_0 PlayFromStart))))

(fn ConstructionScript
  (|CallParentFunction))