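; BP_LevelCheckpoint is a VR teleport checkpoint that highlights itself when the teleport marker overlaps its landing point.
; Begin and end overlaps on ProjectionArcLandingPoint show and hide VisualCylinder.
; Both events first call CheckIsValidComponent, which tests whether the overlapping component is the TeleportCylinder of a BP_VR_Pawn.
; GetLandingWorldTransform exposes the LandingTarget world transform as the landing destination.
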(event OnComponentBeginOverlap(ProjectionArcLandingPoint)
  (params (OverlappedComponent :type Primitive%20Component%20Object%20Reference) (OtherActor :type Actor%20Object%20Reference) (OtherComp :type Primitive%20Component%20Object%20Reference) (OtherBodyIndex :type Integer) (bFromSweep :type Boolean) (SweepResult :type Hit%20Result%20Structure%20%28by%20ref%29))
  (CallFunction|CheckIsValidComponent OtherActor OtherComp)
  (Rendering|SetVisibility (Variables|Default|GetVisualCylinder) true false))

(event OnComponentEndOverlap(ProjectionArcLandingPoint)
  (params (OverlappedComponent :type Primitive%20Component%20Object%20Reference) (OtherActor :type Actor%20Object%20Reference) (OtherComp :type Primitive%20Component%20Object%20Reference) (OtherBodyIndex :type Integer))
  (CallFunction|CheckIsValidComponent OtherActor OtherComp)
  (Rendering|SetVisibility (Variables|Default|GetVisualCylinder) false false))

(event EventBeginPlay)

(event EventTick
  (params (DeltaSeconds :type Float%20%28single-precision%29)))

(fn ConstructionScript)

(fn GetLandingWorldTransform
  (return (Transformation|GetWorldTransform (Variables|Default|GetLandingTarget))))

(fn CheckIsValidComponent
  (params (Other%20Actor :type Object%20Object%20Reference) (Other%20Component :type Object%20Object%20Reference))
  (bind _asbp_vr_pawn (Utilities|Casting|CastToBP_VR_Pawn Other%20Actor))
  (if (== (Variables|/Game/PlayerController/BP_VR_Pawn.BP_VR_Pawn_C|GetTeleportCylinder _asbp_vr_pawn) Other%20Component)
    (return)))