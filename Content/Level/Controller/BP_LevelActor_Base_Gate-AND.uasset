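; BP_LevelActor_Base_Gate-AND is a level logic actor that acts as an AND gate between input and output level actors.
; On BeginPlay it stores the input count, and each Activate call decrements it.
; At zero or below it activates every output actor.
; The counter never resets and does not track callers, so repeated calls from one input also count and later calls fire the outputs again.
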(event EventBeginPlay
  (|CallParentFunction)
  (Variables|Default|SetLength (Utilities|Array|Length (Variables|Default|GetLevelActorsInput))))

(event Collision|EventActorBeginOverlap
  (params (OtherActor :type Actor%20Object%20Reference))
  (|CallParentFunction OtherActor))

(event EventTick
  (params (DeltaSeconds :type Float%20%28single-precision%29))
  (|CallParentFunction DeltaSeconds))

(event EventActivate
  (params (CurrentCheckpoint :type Integer))
  (bind _length (Variables|Default|GetLength))
  (Math|Integer|DecrementInt _length
    (:%20%20
      (if (<= _length 0)
        (for _array_element (Variables|Default|GetLevelActorsOutput)
          (Default|Activate _array_element))))))

(fn ConstructionScript
  (|CallParentFunction))