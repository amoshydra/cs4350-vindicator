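; Level actor for a broken step in the Ice Land level that drops away when activated.
; The Activate event runs only once, switching the PlayerBlockingVolume to query-only collision and starting a timeline.
; The timeline lerps the relative Z of the OriginalZ component from zero to far below its origin.
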(event EventBeginPlay
  (|CallParentFunction))

(event Collision|EventActorBeginOverlap
  (params (OtherActor :type Actor%20Object%20Reference))
  (|CallParentFunction OtherActor))

(event EventTick
  (params (DeltaSeconds :type Float%20%28single-precision%29))
  (|CallParentFunction DeltaSeconds))

(event EventActivate
  (params (CurrentCheckpoint :type Integer))
  (Utilities|FlowControl|DoOnce false
    (:Completed
      (Collision|SetCollisionEnabled (Variables|Default|GetPlayerBlockingVolume) "QueryOnly")
      (bind _newtrack_0 (Timeline|Timeline_0 PlayFromStart)
        (:Update
          (Transformation|SetRelativeLocation (Variables|Default|GetOriginalZ) (Math|Vector|MakeVector 0.0 0.0 (Math|Float|Lerp 0.0 -5e+03 _newtrack_0)) false false))))))

(fn ConstructionScript
  (|CallParentFunction))