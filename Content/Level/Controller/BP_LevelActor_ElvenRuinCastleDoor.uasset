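; Double castle door level actor for the elven ruins that swings open and shut when activated.
; Activate alternates OpenDoor and CloseDoor through a FlipFlop, playing or reversing one timeline.
; The timeline lerps between closed and opened rotations, applying the result to RightAoR and its negation to LeftAoR.
; IsOpened poses both leaves open in the construction script, but the FlipFlop ignores it, so the first activation always calls OpenDoor.
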(event Custom|OpenDoor
  (bind _newtrack_0 (Timeline|Timeline_0 Play)
    (:Update
      (Utilities|FlowControl|Sequence
        (:then_0
          (Transformation|SetRelativeRotation (Variables|Default|GetRightAoR) (Math|Rotator|Lerp(Rotator) (Variables|Default|GetClosedRotation) (Variables|Default|GetOpenedRotation) _newtrack_0) false false))
        (:then_1
          (Transformation|SetRelativeRotation (Variables|Default|GetLeftAoR) (* (Math|Rotator|Lerp(Rotator) (Variables|Default|GetClosedRotation) (Variables|Default|GetOpenedRotation) _newtrack_0) -1) false false))))))

(event Custom|CloseDoor
  (bind _newtrack_0 (Timeline|Timeline_0 Reverse)
    (:Update
      (Utilities|FlowControl|Sequence
        (:then_0
          (Transformation|SetRelativeRotation (Variables|Default|GetRightAoR) (Math|Rotator|Lerp(Rotator) (Variables|Default|GetClosedRotation) (Variables|Default|GetOpenedRotation) _newtrack_0) false false))
        (:then_1
          (Transformation|SetRelativeRotation (Variables|Default|GetLeftAoR) (* (Math|Rotator|Lerp(Rotator) (Variables|Default|GetClosedRotation) (Variables|Default|GetOpenedRotation) _newtrack_0) -1) false false))))))

(event EventBeginPlay
  (|CallParentFunction))

(event Collision|EventActorBeginOverlap
  (params (OtherActor :type Actor%20Object%20Reference))
  (|CallParentFunction OtherActor))

(event EventTick
  (params (DeltaSeconds :type Float%20%28single-precision%29))
  (|CallParentFunction DeltaSeconds))

(event EventActivate
  (params (CurrentCheckpoint :type Integer))
  (Utilities|FlowControl|FlipFlop
    (:A
      (CallFunction|OpenDoor))
    (:B
      (CallFunction|CloseDoor))))

(event EventEavesdrop
  (params (OtherCheckpoint :type Integer)))

(fn ConstructionScript
  (bind _openedrotation (Variables|Default|GetOpenedRotation))
  (bind _closedrotation (Variables|Default|GetClosedRotation))
  (bind _returnvalue (Math|Rotator|Lerp(Rotator) _closedrotation _openedrotation 1.0))
  (|CallParentFunction)
  (if (Variables|Default|GetisOpened)
    (Utilities|FlowControl|Sequence
      (:then_0
        (Transformation|SetRelativeRotation (Variables|Default|GetRightAoR) _returnvalue false false))
      (:then_1
        (Transformation|SetRelativeRotation (Variables|Default|GetLeftAoR) (* _returnvalue -1) false false)))))