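; BP_LevelActor_Text is a level actor that shows configurable 3D text which grows into view when activated.
; The construction script applies the text, world size and color to a TextRender and shrinks it to a near-zero scale.
; The Activate event plays a timeline from the start that lerps the text's relative scale up to full size.
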(event EventBeginPlay
  (|CallParentFunction))

(event Collision|EventActorBeginOverlap
  (params (OtherActor :type Actor%20Object%20Reference))
  (|CallParentFunction OtherActor))

(event EventTick
  (params (DeltaSeconds :type Float%20%28single-precision%29))
  (|CallParentFunction DeltaSeconds))

(event EventActivate
  (params (CurrentCheckpoint :type Integer))
  (bind _newtrack_0 (Timeline|Timeline_0 PlayFromStart)
    (:Update
      (Transformation|SetRelativeScale3D (Variables|Default|GetTextRender) (Math|Vector|Lerp(Vector) "0.010000,0.010000,0.010000" "1.000000,1.000000,1.000000" _newtrack_0)))))

(fn ConstructionScript
  (bind _textrender (Variables|Default|GetTextRender))
  (|CallParentFunction)
  (Rendering|Components|TextRender|SetText _textrender (Variables|Default|GetText))
  (Rendering|Components|TextRender|SetWorldSize _textrender (Variables|Default|GetWorldSize))
  (Rendering|Components|TextRender|SetTextRenderColor _textrender (Variables|Default|GetTextColor))
  (Transformation|SetRelativeScale3D (Variables|Default|GetTextRender) "0.010000,0.010000,0.010000"))