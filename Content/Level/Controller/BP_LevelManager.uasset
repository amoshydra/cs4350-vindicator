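; BP_LevelManager drives level progression by coordinating checkpoints and enemy spawn points.
; On BeginPlay it gathers and sorts level actors, then binds to their dispatchers and the GameInstance's enemy-removed event.
; Each checkpoint increment messages spawn points with the new index and counts those that activate.
; Checkpoints receive the current index only when no enemies remain and all active spawns have completed.
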(event Custom|IncrementCheckpoint_Event_0
  (Math|Integer|IncrementInt (Variables|Default|GetCurrentCheckpoint)
    (:%20%20
      (CallFunction|ActivateSpawnPoint))))

(event Custom|SpawnIsCompleted_Event_0
  (Math|Integer|DecrementInt (Variables|Default|GetNumberOfActiveSpawn)
    (:%20%20
      (CallFunction|ActivateCheckpoints))))

(event Custom|ActivateSpawnPoint
  (Variables|Default|SetNumberOfActiveSpawn 0)
  (for _array_element (Variables|Default|GetLevelActor_EnemySpawns)
    (bind _acknowledgemessage (Default|ReceiveMessage _array_element (Variables|Default|GetCurrentCheckpoint)))
    (if _acknowledgemessage
      (Math|Integer|IncrementInt (Variables|Default|GetNumberOfActiveSpawn)))))

(event Custom|EnemyIsRemoved_Event_0
  (params (RemovedEnemy :type BP%20Enemy%20Base%20Object%20Reference))
  (CallFunction|ActivateCheckpoints))

(event Custom|ActivateCheckpoints
  (bind _asbp_game_instance (Utilities|Casting|CastToBP_GameInstance (Game|GetGameInstance)))
  (if (and (<= (Utilities|Array|Length (Variables|/Game/Blueprints/BP_GameInstance.BP_GameInstance_C|GetEnemies _asbp_game_instance)) 0) (<= (Variables|Default|GetNumberOfActiveSpawn) 0))
    (for _array_element (Variables|Default|GetLevelActor_Checkpoints)
      (Default|ReceiveMessage _array_element (Variables|Default|GetCurrentCheckpoint)))))

(event EventBeginPlay
  ;[1 1 1] Initialise Array
  (Utilities|FlowControl|Sequence
    (:then_0
      (Utilities|FlowControl|Sequence
        (:then_0
          (bind _outactors (Actor|GetAllActorsOfClass "/Game/Level/Controller/BP_LevelActor_Base.BP_LevelActor_Base_C"))
          (bind _output_get (Variables|Default|SetLevelActors _outactors))
          (for _array_element _output_get
            (bind _asbp_level_actor_checkpoint (Utilities|Casting|CastToBP_LevelActor_Checkpoint _array_element)
              (:then
                (Utilities|Array|Add (Variables|Default|GetLevelActor_Checkpoints) _asbp_level_actor_checkpoint))
              (:CastFailed
                (bind _asbp_level_actor_enemy_spawn_point (Utilities|Casting|CastToBP_LevelActor_EnemySpawnPoint _array_element))
                (Utilities|Array|Add (Variables|Default|GetLevelActor_EnemySpawns) _asbp_level_actor_enemy_spawn_point)))))
        (:then_1
          (Development|PrintString (Utilities|String|Append (Utilities|String|ToString(Integer) (Utilities|Array|Length (Variables|Default|GetLevelActors))) " actors in the map") true true "(R=0.000000,G=0.660000,B=1.000000,A=1.000000)" 0.05))))
    (:then_1
      (Utilities|FlowControl|Sequence
        (:then_0
          (bind _asbp_game_instance (Utilities|Casting|CastToBP_GameInstance (Game|GetGameInstance)))
          (EventDispatchers|AssignEnemyIsRemoved _asbp_game_instance (delegate Custom|EnemyIsRemoved_Event_0)))
        (:then_1
          (for _array_element_2 (Variables|Default|GetLevelActor_Checkpoints)
            (EventDispatchers|AssignIncrementCheckpoint _array_element_2 (delegate Custom|IncrementCheckpoint_Event_0))))
        (:then_2
          (for _array_element_3 (Variables|Default|GetLevelActor_EnemySpawns)
            (EventDispatchers|AssignSpawnIsCompleted _array_element_3 (delegate Custom|SpawnIsCompleted_Event_0))))
        (:then_3
          (CallFunction|ActivateSpawnPoint)
          (CallFunction|ActivateCheckpoints))))))

(fn ConstructionScript)