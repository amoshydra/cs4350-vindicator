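; Castle ramp level actor that rotates in steps as it is activated, swinging between closed and fully open.
; Each Activate steps the index up or down, reversing at either limit; OpenGate and CloseGate jump it to the ends.
; MoveDoor animates roll with the DropTime timeline and lifts TraceLineBlocker's InvisibleWall collision only at full activation.
; Construction derives the step angle and initial index, and pre-rotates a separate nav axis to the destination angle.
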(event Custom|CloseGate
  (Variables|Default|SetactivationIndexPosition 0)
  (CallFunction|MoveDoor))

(event Custom|CheckIfDoorIsOpened
  (Collision|SetCollisionProfileName (Variables|Default|GetTraceLineBlocker) (select (== (Variables|Default|GetactivationIndexPosition) (Variables|Default|GetnumberOfActivationNeeded)) "NoCollision" "InvisibleWall") :!class /Script/Engine.PrimitiveComponent))

(event Custom|OpenGate
  (Variables|Default|SetactivationIndexPosition (Variables|Default|GetnumberOfActivationNeeded))
  (CallFunction|MoveDoor))

(event Custom|MoveDoor
  (bind _activationindexposition (Variables|Default|GetactivationIndexPosition))
  (bind _peractivationopenangle (Variables|Default|GetPerActivationOpenAngle))
  (bind _returnvalue (* _activationindexposition _peractivationopenangle))
  (CallFunction|CheckifDoorIsOpened)
  (Variables|Default|SettemporaryRoll (.roll (Variables|/Script/Engine.SceneComponent|GetRelativeRotation (Variables|Default|GetRampAxisOfRotation))))
  (bind _ramprotation (Timeline|DropTime PlayFromStart)
    (:Update
      (Transformation|SetRelativeRotation (Variables|Default|GetRampAxisOfRotation) (Math|Rotator|MakeRotator (Math|Float|Lerp (Variables|Default|GettemporaryRoll) (select (Variables|Default|GetonBeginOpen) (Math|Float|SelectFloat _returnvalue (Variables|Default|GetDestinationAngle) (> (- (Variables|Default|GetDestinationAngle) (Variables|Default|GettemporaryRoll)) (Variables|Default|GetPerActivationOpenAngle))) (Math|Float|SelectFloat _returnvalue 0.0 (> (Variables|Default|GettemporaryRoll) (Variables|Default|GetPerActivationOpenAngle)))) _ramprotation) 0.0 0.0) false false))))

(event EventBeginPlay
  (|CallParentFunction))

(event Collision|EventActorBeginOverlap
  (params (OtherActor :type Actor%20Object%20Reference))
  (|CallParentFunction OtherActor))

(event EventTick
  (params (DeltaSeconds :type Float%20%28single-precision%29))
  (|CallParentFunction DeltaSeconds))

(event EventActivate
  (params (CurrentCheckpoint :type Integer))
  (if (Variables|Default|GetonBeginOpen)
    (bind _result (Math|Integer|IncrementInt (Variables|Default|GetactivationIndexPosition))
      (:%20%20
        (Variables|Default|SetactivationIndexPosition (Math|Integer|Min(Integer) _result (Variables|Default|GetnumberOfActivationNeeded)))
        (if (== (Variables|Default|GetactivationIndexPosition) (Variables|Default|GetnumberOfActivationNeeded))
          (Variables|Default|SetonBeginOpen false))))
    (else
      (bind _result_2 (Math|Integer|DecrementInt (Variables|Default|GetactivationIndexPosition))
        (:%20%20
          (Variables|Default|SetactivationIndexPosition (Math|Integer|Max(Integer) _result_2))
          (if (== (Variables|Default|GetactivationIndexPosition) 0)
            (Variables|Default|SetonBeginOpen true))))))
  (CallFunction|MoveDoor))

(fn ConstructionScript
  (bind _ramp (Variables|Default|GetRamp))
  (bind _relativelocation (Variables|/Script/Engine.SceneComponent|GetRelativeLocation _ramp))
  (|CallParentFunction)
  (Utilities|FlowControl|Sequence
    (:then_0
      (Transformation|SetRelativeLocation _ramp (Math|Vector|MakeVector (.x _relativelocation) (.y _relativelocation) (* (.z (Variables|/Script/Engine.SceneComponent|GetRelativeScale3D (Variables|Default|GetRamp))) 5e+01)) false false))
    (:then_1
      (Variables|Default|SetPerActivationOpenAngle (/ (Variables|Default|GetDestinationAngle) (Math|Conversions|ToFloat(Integer) (Variables|Default|GetnumberOfActivationNeeded)))))
    (:then_2
      (Transformation|SetRelativeRotation (Variables|Default|GetRampAxisOfRotation) (Math|Rotator|MakeRotator (Variables|Default|GetInitialAngle) 0.0 0.0) false false)
      (Variables|Default|SetactivationIndexPosition (Math|Float|Round (/ (Variables|Default|GetInitialAngle) (Variables|Default|GetPerActivationOpenAngle)))))
    (:then_3
      (Transformation|SetRelativeRotation (Variables|Default|GetRampAxisOfRatationForNav) (Math|Rotator|MakeRotator (Variables|Default|GetDestinationAngle) 0.0 0.0) false false))
    (:then_4
      (Components|Box|SetBoxExtent (Variables|Default|GetTraceLineBlocker) (Variables|/Script/Engine.BoxComponent|GetBoxExtent (Variables|Default|GetNavMeshPlane)) true))))