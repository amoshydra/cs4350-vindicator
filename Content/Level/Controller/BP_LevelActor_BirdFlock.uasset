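; BP_LevelActor_BirdFlock is a level actor that spawns a flock of birds when activated.
; Its Activate event spawns a BP_BirdFlock at the actor's own transform, passing along its bird count, flying speed, spawn distance and lifespan settings.
; It has no other active logic, so any flight behavior is left to the spawned flock actor.
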(event EventBeginPlay
  (|CallParentFunction))

(event Collision|EventActorBeginOverlap
  (params (OtherActor :type Actor%20Object%20Reference))
  (|CallParentFunction OtherActor))

(event EventTick
  (params (DeltaSeconds :type Float%20%28single-precision%29))
  (|CallParentFunction DeltaSeconds))

(event EventActivate
  (params (CurrentCheckpoint :type Integer))
  (Game|SpawnActorfromClass "/Game/Level/CustomAssets/BP_BirdFlock.BP_BirdFlock_C" (Transformation|GetActorTransform) "Undefined" 0 (Variables|Default|GetNumberOfBirdToSpawn) (Variables|Default|GetFlyingSpeed) (Variables|Default|GetSpawnDistance) (Variables|Default|GetBirdsLifespan) 0))

(fn ConstructionScript
  (|CallParentFunction))