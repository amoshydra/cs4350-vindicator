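; VR teleport checkpoint that gates player progression through the level.
; Reaching it by teleport or overlap hides it, activates linked level actors and spawns enemies, subject to a respawn time limit.
; Once all spawn points report completion or spawning is skipped, it activates the next checkpoints; using one deactivates all of them.
; The construction script sets up the hover-tinted cylinder and can draw debug arrows flagging overly distant links.
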(event OnComponentBeginOverlap(PlayerTriggerVolumen)
  (params (OverlappedComponent :type Primitive%20Component%20Object%20Reference) (OtherActor :type Actor%20Object%20Reference) (OtherComp :type Primitive%20Component%20Object%20Reference) (OtherBodyIndex :type Integer) (bFromSweep :type Boolean) (SweepResult :type Hit%20Result%20Structure%20%28by%20ref%29))
  (if (Variables|Default|GetisTeleportationAllow)
    (Utilities|Casting|CastToBP_VR_Pawn OtherActor)
    (CallFunction|PawnTeleported)))

(event Custom|PawnTeleported
  (Default|CallCheckpointUsed)
  (CallFunction|DeactivateCheckpoint)
  (CallFunction|AttemptoSpawnEnemy)
  (CallFunction|ActivateLevelActors))

(event Custom|TeleporterEnter
  (CallFunction|ShowHoverEffect))

(event Custom|TeleporterExit
  (CallFunction|HideHoverEffect))

(event Custom|ActivateLevelActors
  ;[1 1 1] Simply activate without eavesdropping
  (for _array_element (Variables|Default|GetLevelActors)
    (Default|Activate _array_element)))

(event Custom|CheckpointUsed_Event_0
  ;[1 1 1] Deactivate the previous checkpoint if a checkpoint is used
  (for _array_element (Variables|Default|GetNextCheckpoint)
    (CallFunction|DeactivateCheckpoint _array_element)))

(event Custom|SpawnIsCompleted_Event_0
  (Math|Integer|DecrementInt (Variables|Default|GetActiveEnemySpawnPoint)
    (:%20%20
      (CallFunction|AttempttoActivateNextCheckpoint))))

(event Custom|ActivateNextCheckpoint
  (for _array_element (Variables|Default|GetNextCheckpoint)
    (Utilities|FlowControl|Sequence
      (:then_0
        ;[1 1 1] Deactivate the previous checkpoint if a checkpoint is used
        (EventDispatchers|BindEventtoCheckpointUsed _array_element (delegate Custom|CheckpointUsed_Event_0)))
      (:then_1
        (CallFunction|ActivateCheckpoint _array_element)))))

(event Custom|SpawnEnemies
  (bind _output_get (Variables|Default|SetActiveEnemySpawnPoint (Utilities|Array|Length (Variables|Default|GetEnemySpawnPoints))))
  (if (!= _output_get 0)
    (for _array_element (Variables|Default|GetEnemySpawnPoints)
      (Utilities|FlowControl|Sequence
        (:then_0
          (EventDispatchers|AssignSpawnIsCompleted _array_element (delegate Custom|SpawnIsCompleted_Event_0)))
        (:then_1
          (Default|Activate _array_element))))
    (else
      (CallFunction|AttempttoActivateNextCheckpoint))))

(event Custom|RecordLastSpawnFinishTimestamp
  ;[1 1 1] Handle respawn limiting mechanism
  (Variables|Default|SetlastTeleportedTime (Utilities|Time|GetGameTimeinSeconds)))

(event Custom|AttemptToActivateNextCheckpoint
  (if (== (Variables|Default|GetActiveEnemySpawnPoint) 0)
    (CallFunction|ActivateNextCheckpoint)
    (CallFunction|RecordLastSpawnFinishTimestamp)))

(event Custom|AttempToSpawnEnemy
  ;[1 1 1] Handle respawn limiting mechanism
  (if (or (Math|Float|NearlyEqual(Float) (Variables|Default|GetlastTeleportedTime) 0.0 0.1) (> (- (Utilities|Time|GetGameTimeinSeconds) (Variables|Default|GetlastTeleportedTime)) (Variables|Default|GetEnemyRespawnTimeLimit)))
    (CallFunction|SpawnEnemies)
    (else
      (CallFunction|AttempttoActivateNextCheckpoint))))

(event EventActivate
  (params (CurrentCheckpoint :type Integer))
  (CallFunction|ActivateCheckpoint))

(event EventTick
  (params (DeltaSeconds :type Float%20%28single-precision%29)))

(event EventEavesdrop
  (params (OtherCheckpoint :type Integer))
  (CallFunction|DeactivateCheckpoint))

(fn ConstructionScript
  (bind _nextcheckpoint (Variables|Default|GetNextCheckpoint))
  (bind _enemyspawnpoints (Variables|Default|GetEnemySpawnPoints))
  (Utilities|FlowControl|Sequence
    (:then_0
      (Transformation|SetRelativeRotation (Variables|Default|GetVisualCylinder) (Variables|Default|GetCustomRotation) false false))
    (:then_1
      (Utilities|FlowControl|Sequence
        (:then_0
          (bind _returnvalue (Rendering|Material|CreateDynamicMaterialInstance (Variables|Default|GetVisualCylinder) 0 "/Game/VirtualReality/Materials/M_TeleporterCylinder.M_TeleporterCylinder" :!class /Script/Engine.PrimitiveComponent))
          (Variables|Default|SetMaterialInstance _returnvalue)
          (CallFunction|HideHoverEffect)
          (if (Variables|Default|GetAutoActivate)
            (CallFunction|Activate)
            (else
              (CallFunction|Eavesdrop))))
        (:then_1
          (if (Variables|Default|GetcheckConnection)
            (Variables|Default|SetcheckConnection false)
            (CallFunction|ShowDebugCheckpointConnection)))
        (:then_2
          (if false
            (Utilities|FlowControl|Sequence
              (:then_0
                (for _array_element _nextcheckpoint
                  (Utilities|IsValid _array_element
                    (:Is%20Not%20Valid
                      (Utilities|Array|RemoveItem _nextcheckpoint _array_element)))))
              (:then_1
                (for _array_element_2 _enemyspawnpoints
                  (Utilities|IsValid _array_element_2
                    (:Is%20Not%20Valid
                      (Utilities|Array|RemoveItem _enemyspawnpoints _array_element_2))))))))))))

(fn RequestTeleportation
  (params (Pawn :type Pawn%20Object%20Reference))
  (bind _asbp_vr_pawn (Utilities|Casting|CastToBP_VR_Pawn Pawn)
    (:then
      _)
    (:CastFailed
      _))
  (if (Variables|Default|GetisTeleportationAllow)
    (bind _landinglocation (CallFunction|RequestLandingLocation))
    (CallFunction|PawnTeleported)
    (return true (+ _landinglocation (Math|Vector|MakeVector 0.0 0.0 (Variables|/Script/Engine.CapsuleComponent|GetCapsuleHalfHeight (Variables|/Game/PlayerController/BP_VR_Pawn.BP_VR_Pawn_C|GetCapsule _asbp_vr_pawn)))) (Transformation|GetActorRotation _asbp_vr_pawn))
    (else
      ;[1 1 1] Reject: Return actor's own transform
      (return false (.location (Transformation|GetActorTransform _asbp_vr_pawn)) (.rotation (Transformation|GetActorTransform _asbp_vr_pawn))))))

(fn ShowTeleportationRing
  (Rendering|SetVisibility (Variables|Default|GetVisualCylinder) true false))

(fn HideTeleportationRing
  (Rendering|SetVisibility (Variables|Default|GetVisualCylinder) false false))

(fn ShowHoverEffect
  (Rendering|Material|SetVectorParameterValue (Variables|Default|GetMaterialInstance) "Color" (Variables|Default|GetColorOnHover) :!class /Script/Engine.MaterialInstanceDynamic))

(fn HideHoverEffect
  (Rendering|Material|SetVectorParameterValue (Variables|Default|GetMaterialInstance) "Color" (Variables|Default|GetColorOnLure) :!class /Script/Engine.MaterialInstanceDynamic))

(fn ActivateCheckpoint
  (CallFunction|ShowTeleportationRing)
  (Variables|Default|SetisTeleportationAllow true)
  (Collision|SetCollisionEnabled (Variables|Default|GetProjectionArcLandingPoint) "QueryOnly")
  (return))

(fn DeactivateCheckpoint
  (CallFunction|HideTeleportationRing)
  (Variables|Default|SetisTeleportationAllow false)
  (Collision|SetCollisionEnabled (Variables|Default|GetProjectionArcLandingPoint) "NoCollision"))

(fn ShowDebugCheckpointConnection
  (bind _defaultscenerootnode (Variables|Default|GetDefaultSceneRootNode))
  (bind _returnvalue (Transformation|GetWorldLocation _defaultscenerootnode))
  (bind _returnvalue_2 (+ _returnvalue "0, 0,150.000000"))
  (for _array_element (Variables|Default|GetNextCheckpoint)
    (if (<= (Math|Vector|VectorLength (- _returnvalue_2 (+ (Transformation|GetWorldLocation (Variables|/Game/Level/Controller/BP_LevelActor_Base.BP_LevelActor_Base_C|GetDefaultSceneRootNode _array_element)) "0, 0,150.000000"))) (LocalVariables|GetAcceptable%20Distance%20Between%20Checkpoint))
      (Rendering|Debug|DrawDebugArrow _returnvalue_2 (+ (Transformation|GetWorldLocation (Variables|/Game/Level/Controller/BP_LevelActor_Base.BP_LevelActor_Base_C|GetDefaultSceneRootNode _array_element)) "0, 0,150.000000") 1e+02 "(R=0.238286,G=0.973958,B=0.015218,A=1.000000)" 5.0 8.0)
      (else
        (Rendering|Debug|DrawDebugArrow _returnvalue_2 (+ (Transformation|GetWorldLocation (Variables|/Game/Level/Controller/BP_LevelActor_Base.BP_LevelActor_Base_C|GetDefaultSceneRootNode _array_element)) "0, 0,150.000000") 1e+02 "(R=1.000000,G=0.000000,B=0.000000,A=1.000000)" 5.0 8.0)
        (Development|PrintString (Utilities|String|Append "Distance may be too far for the player to teleport: " (Utilities|String|ToString(Float) (Math|Vector|VectorLength (- _returnvalue_2 (+ (Transformation|GetWorldLocation (Variables|/Game/Level/Controller/BP_LevelActor_Base.BP_LevelActor_Base_C|GetDefaultSceneRootNode _array_element)) "0, 0,150.000000"))))) true true "(R=1.000000,G=0.000000,B=0.000000,A=1.000000)" 5.0)))))

(fn RequestLandingLocation
  (return (Transformation|GetWorldLocation (Variables|Default|GetLandingTarget))))