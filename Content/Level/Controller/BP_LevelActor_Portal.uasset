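; BP_LevelActor_Portal is a portal actor that moves the player to another level or quits the game.
; It handles the PawnTeleported event, calling the parent implementation, then fading the first player's camera out and holding it.
; After a delay matching the fade, it opens the level named by LevelName, treating the special name "Exit" as a quit command.
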(event EventBeginPlay
  (|CallParentFunction))

(event Collision|EventActorBeginOverlap
  (params (OtherActor :type Actor%20Object%20Reference))
  (|CallParentFunction OtherActor))

(event EventTick
  (params (DeltaSeconds :type Float%20%28single-precision%29))
  (|CallParentFunction DeltaSeconds))

(event EventPawnTeleported
  (bind _returnvalue (Math|Float|MakeLiteralFloat 0.5))
  (bind _levelname (Variables|Default|GetLevelName))
  (|CallParentFunction)
  (CameraFades|StartCameraFade :self (Game|GetPlayerCameraManager 0) :ToAlpha 1.0 :Duration _returnvalue :bHoldWhenFinished true)
  (Utilities|FlowControl|Delay _returnvalue)
  (if (Utilities|Name|Equal(Name) _levelname "Exit")
    (Game|QuitGame 0 "Quit")
    (else
      (Game|OpenLevel(byName) _levelname))))

(fn ConstructionScript
  (|CallParentFunction))