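; Level actor for an IceLand archer point that moves its OriginalZScene component vertically between two heights when activated.
; Each Activate call caches the current relative Z, then a FlipFlop alternates the target between zero and OriginalZ, starting with zero.
; A single timeline drives the lerp from the cached height to that target.
; The construction script places the component at OriginalZ when Check is set.
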(event EventBeginPlay
  (|CallParentFunction))

(event Collision|EventActorBeginOverlap
  (params (OtherActor :type Actor%20Object%20Reference))
  (|CallParentFunction OtherActor))

(event EventTick
  (params (DeltaSeconds :type Float%20%28single-precision%29))
  (|CallParentFunction DeltaSeconds))

(event EventActivate
  (params (CurrentCheckpoint :type Integer))
  (Variables|Default|SetOldZ (.z (Variables|/Script/Engine.SceneComponent|GetRelativeLocation (Variables|Default|GetOriginalZScene))))
  (bind _isa (Utilities|FlowControl|FlipFlop)
    (:A
      (bind _newtrack_0 (Timeline|Timeline_0 PlayFromStart)
        (:Update
          (Transformation|SetRelativeLocation (Variables|Default|GetOriginalZScene) (Math|Vector|MakeVector 0.0 0.0 (Math|Float|Lerp (Variables|Default|GetOldZ) (Math|Float|SelectFloat 0.0 (Variables|Default|GetOriginalZ) _isa) _newtrack_0)) false false))))
    (:B
      (Timeline|Timeline_0 PlayFromStart))))

(fn ConstructionScript
  (|CallParentFunction)
  (if (Variables|Default|GetCheck)
    (Transformation|SetRelativeLocation (Variables|Default|GetOriginalZScene) (Math|Vector|MakeVector 0.0 0.0 (Variables|Default|GetOriginalZ)) false false)))