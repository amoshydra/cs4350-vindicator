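; Level actor for an Elven ruin gate that swings between closed and opened rotations.
; Each Activate event alternates between opening and closing through a FlipFlop.
; A single timeline plays forward to open and reverses to close, interpolating the relative rotation of the AxisOfRotation component.
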(event Custom|OpenDoor
  (bind _newtrack_0 (Timeline|OpenDoorTimeline Play)
    (:Update
      (Transformation|SetRelativeRotation (Variables|Default|GetAxisOfRotation) (Math|Rotator|Lerp(Rotator) (Variables|Default|GetClosedRotation) (Variables|Default|GetOpenedRotation) _newtrack_0) false false))))

(event Custom|CloseDoor
  (bind _newtrack_0 (Timeline|OpenDoorTimeline Reverse)
    (:Update
      (Transformation|SetRelativeRotation (Variables|Default|GetAxisOfRotation) (Math|Rotator|Lerp(Rotator) (Variables|Default|GetClosedRotation) (Variables|Default|GetOpenedRotation) _newtrack_0) false false))))

(event EventBeginPlay
  (|CallParentFunction))

(event Collision|EventActorBeginOverlap
  (params (OtherActor :type Actor%20Object%20Reference))
  (|CallParentFunction OtherActor))

(event EventTick
  (params (DeltaSeconds :type Float%20%28single-precision%29))
  (|CallParentFunction DeltaSeconds))

(event EventActivate
  (params (CurrentCheckpoint :type Integer))
  (Utilities|FlowControl|FlipFlop
    (:A
      (CallFunction|OpenDoor))
    (:B
      (CallFunction|CloseDoor))))

(fn ConstructionScript
  (|CallParentFunction))