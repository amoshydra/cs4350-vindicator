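; BP_LevelActor_VisibilityToggler is a level controller actor that flips the visibility of a set of actors when activated.
; Its Activate event loops over the Actors array and sets each actor's hidden-in-game state to the opposite of its current value.
; Each actor toggles independently, so a mix of shown and hidden actors swaps rather than syncing to one state.
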(event EventBeginPlay
  (|CallParentFunction))

(event Collision|EventActorBeginOverlap
  (params (OtherActor :type Actor%20Object%20Reference))
  (|CallParentFunction OtherActor))

(event EventTick
  (params (DeltaSeconds :type Float%20%28single-precision%29))
  (|CallParentFunction DeltaSeconds))

(event EventActivate
  (params (CurrentCheckpoint :type Integer))
  (for _array_element (Variables|Default|GetActors)
    (Rendering|SetActorHiddenInGame _array_element (not (Variables|/Script/Engine.Actor|GetbHidden _array_element)))))

(fn ConstructionScript
  (|CallParentFunction))