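; Tutorial level actor that checks whether the VR player casts the intended spell on its platform.
; On overlap it binds to the pawn's spell controller and shows guides; the correct spell activates the checkpoint once.
; An overlapping shield spell has projectile hits counted, destroying tutorial grunts after three.
; Activate reveals any portal and runs a timeline raising the bridge, statue and one-way or two-way platform.
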(event OnComponentBeginOverlap(Spellchecker)
  (params (OverlappedComponent :type Primitive%20Component%20Object%20Reference) (OtherActor :type Actor%20Object%20Reference) (OtherComp :type Primitive%20Component%20Object%20Reference) (OtherBodyIndex :type Integer) (bFromSweep :type Boolean) (SweepResult :type Hit%20Result%20Structure%20%28by%20ref%29))
  (bind _visualguide (Variables|Default|GetVisualGuide))
  (bind _statue (Variables|Default|GetStatue))
  (bind _asbp_vr_pawn (Utilities|Casting|CastToBP_VR_Pawn OtherActor)
    (:then
      ;[1 1 1] Detect Player Casting Spell Within Respective Tutorial Platforms To Differentiate Spell Being Cast By Statue
      (Utilities|FlowControl|Sequence
        (:then_0
          ;;[1 1 1] Upon Detecting Correct Spell Being Cast, Send Event Activate To Checkpoint For Starting Tutorial
          (EventDispatchers|AssignCastSpell (Variables|/Game/PlayerController/BP_VR_Pawn.BP_VR_Pawn_C|GetSpellController _asbp_vr_pawn) (delegate Custom|SignalCheckpointActivate)))
        (:then_1
          ;;[1 1 1] Show Tutorial Platform Instructions And Visual Guides
          (if (!= _visualguide 0)
            (Default|ShowGuide _visualguide (Variables|Default|GetTutorialName))))
        (:then_2
          (if (!= _statue 0)
            (Default|ShowText _statue)))))
    (:CastFailed
      ;[1 1 1] Used For Shield Tutorial Platform To Track Progress Of Shield Tutorial Completion
      (bind _asbp_spell_shield (Utilities|Casting|CastToBP_Spell_Shield OtherActor))
      (Collision|AssignOnComponentBeginOverlap (Variables|/Game/SpellSystem/SpellComponents/Spells/BP_Spell_Shield.BP_Spell_Shield_C|GetBlockingZone _asbp_spell_shield) (delegate Custom|OnComponentBeginOverlap_Event_0)))))

(event Custom|SignalCheckpointActivate
  (params (Spell :type BP%20Spell%20Base%20Class%20Reference))
  (bind _statue (Variables|Default|GetStatue))
  ;[1 1 1] Detect Player Casting Spell Within Respective Tutorial Platforms To Differentiate Spell Being Cast By Statue
  ;;[1 1 1] Upon Detecting Correct Spell Being Cast, Send Event Activate To Checkpoint For Starting Tutorial
  (if (and (== (Variables|Default|GetIntended) Spell) (not (Variables|Default|GetActivatedTutorial)))
    (Default|Activate (Variables|Default|GetCurrentCheckpoint))
    (Variables|Default|SetActivatedTutorial true)
    (if (!= _statue 0)
      (Default|ShowDirection _statue))))

(event Custom|OnComponentBeginOverlap_Event_0
  (params (OverlappedComponent :type Primitive%20Component%20Object%20Reference) (OtherActor :type Actor%20Object%20Reference) (OtherComp :type Primitive%20Component%20Object%20Reference) (OtherBodyIndex :type Integer) (bFromSweep :type Boolean) (SweepResult :type Hit%20Result%20Structure%20%28by%20ref%29))
  ;[1 1 1] Used For Shield Tutorial Platform To Track Progress Of Shield Tutorial Completion
  (Utilities|Casting|CastToBP_Enemy_Range_Projectile OtherActor)
  (bind _output_get (Variables|Default|SetShieldHitCounter (+ (Variables|Default|GetShieldHitCounter) 1)))
  (if (>= _output_get 3)
    (bind _outactors (Actor|GetAllActorsOfClass "/Game/AI/Enemy_Grunt_Range/BP_Enemy_Grunt_Tutorial.BP_Enemy_Grunt_Tutorial_C"))
    (Actor|DestroyActor _outactors)))

(event EventBeginPlay
  (bind _platformoneway (Variables|Default|GetPlatformOneWay))
  (bind _portal (Variables|Default|GetPortal))
  (bind _statue (Variables|Default|GetStatue))
  ;[1 1 1] Initialise Position Vector Variable For Use Later To Bring Up Platform, Bridges, Statues and Portal If Any
  (if (!= _statue 0)
    (Variables|Default|SetStatuePosition (Transformation|GetActorLocation _statue)))
  (Variables|Default|SetBridgePosition (Variables|/Script/Engine.SceneComponent|GetRelativeLocation (Variables|/Game/Level/CustomAssets/BP_LevelActors/BP_TutorialBridge.BP_TutorialBridge_C|GetBridgeScene (Variables|Default|GetBridge))))
  (if (!= _platformoneway 0)
    (Variables|Default|SetPlatformPosition (Variables|/Script/Engine.SceneComponent|GetRelativeLocation (Variables|/Game/Level/CustomAssets/BP_LevelActors/BP_TutorialPlatform_OneWay.BP_TutorialPlatform_OneWay_C|GetPlatform _platformoneway)))
    (else
      (Variables|Default|SetPlatformPosition (Variables|/Script/Engine.SceneComponent|GetRelativeLocation (Variables|/Game/Level/CustomAssets/BP_LevelActors/BP_TutorialPlatform_TwoWay.BP_TutorialPlatform_TwoWay_C|GetPlatform (Variables|Default|GetPlatformTwoWay))))))
  (if (!= _portal 0)
    (Variables|Default|SetPortalPosition (Variables|/Script/Engine.SceneComponent|GetRelativeLocation (Variables|/Game/Level/Controller/BP_LevelActor_Portal.BP_LevelActor_Portal_C|GetPortalEffect _portal)))))

(event EventActivate
  (params (CurrentCheckpoint :type Integer))
  (bind _platformoneway (Variables|Default|GetPlatformOneWay))
  (bind _statue (Variables|Default|GetStatue))
  (bind _portal (Variables|Default|GetPortal))
  (bind _statue_2 (Variables|Default|GetStatue))
  ;[1 1 1] Handles Logic For Each Spell's Tutorial Completion
  (Utilities|FlowControl|Sequence
    (:then_0
      (if (!= _statue 0)
        (Default|HideDirection _statue)))
    (:then_1
      ;;[1 1 1] For End Platform To Show Portal
      (if (!= _portal 0)
        (Rendering|SetVisibility (Variables|/Game/Level/Controller/BP_LevelActor_Portal.BP_LevelActor_Portal_C|GetPortalEffect _portal) true false)))
    (:then_2
      ;;[1 1 1] Activate/Enable Next Spell Tutorial  Platform
      (bind _moveup (Timeline|BringUp Play)
        (:Update
          (Utilities|FlowControl|Sequence
            (:then_0
              (Transformation|SetRelativeLocation (Variables|/Game/Level/CustomAssets/BP_LevelActors/BP_TutorialBridge.BP_TutorialBridge_C|GetBridgeScene (Variables|Default|GetBridge)) (+ (Variables|Default|GetBridgePosition) (Math|Vector|MakeVector 0.0 0.0 _moveup)) false false)
              (if (!= _statue_2 0)
                (Transformation|SetActorLocation _statue_2 (+ (Variables|Default|GetStatuePosition) (Math|Vector|MakeVector 0.0 0.0 _moveup)) false false)))
            (:then_1
              (if (!= _platformoneway 0)
                (Transformation|SetRelativeLocation (Variables|/Game/Level/CustomAssets/BP_LevelActors/BP_TutorialPlatform_OneWay.BP_TutorialPlatform_OneWay_C|GetPlatform _platformoneway) (+ (Math|Vector|MakeVector 0.0 0.0 _moveup) (Variables|Default|GetPlatformPosition)) false false)
                (else
                  (Transformation|SetRelativeLocation (Variables|/Game/Level/CustomAssets/BP_LevelActors/BP_TutorialPlatform_TwoWay.BP_TutorialPlatform_TwoWay_C|GetPlatform (Variables|Default|GetPlatformTwoWay)) (+ (Math|Vector|MakeVector 0.0 0.0 _moveup) (Variables|Default|GetPlatformPosition)) false false))))))))))

(fn ConstructionScript)