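; Tutorial trigger volume that shows VR players instructional text and demo hands for movement and sword, shield and fireball spells.
; On pawn overlap, flags select timed welcome messages or a hand demo, where timelines drive grab poses on fixed hand orientations.
; Spell tutorials set completion flags on a linked merge-spell volume, which shows its text only once all three are set.
; Leaving the volume hides text, widget and hands.
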(event OnComponentBeginOverlap(TutorialTrigger)
  (params (OverlappedComponent :type Primitive%20Component%20Object%20Reference) (OtherActor :type Actor%20Object%20Reference) (OtherComp :type Primitive%20Component%20Object%20Reference) (OtherBodyIndex :type Integer) (bFromSweep :type Boolean) (SweepResult :type Hit%20Result%20Structure%20%28by%20ref%29))
  (bind _asbp_vr_pawn (Utilities|Casting|CastToBP_VR_Pawn OtherActor))
  (Variables|Default|SetBP_VR_Pawn _asbp_vr_pawn)
  (if (Variables|Default|GetIsMergeSpell)
    (if (Math|Boolean|ANDBoolean (Variables|Default|GetSwordTutComplete) (Variables|Default|GetShieldTutComplete) (Variables|Default|GetFireballTutComplete))
      (Rendering|SetVisibility (Variables|Default|GetTutorialText) true false :!label _label))
    (else
      (CallFunction|SelectTutorial)
      (goto _label))))

(event OnComponentEndOverlap(TutorialTrigger)
  (params (OverlappedComponent :type Primitive%20Component%20Object%20Reference) (OtherActor :type Actor%20Object%20Reference) (OtherComp :type Primitive%20Component%20Object%20Reference) (OtherBodyIndex :type Integer))
  (Utilities|Casting|CastToBP_VR_Pawn OtherActor)
  (Rendering|SetVisibility (Variables|Default|GetTutorialText) false true)
  (Rendering|SetVisibility (Variables|Default|GetTutorialWidget) false true)
  (Rendering|SetVisibility (Variables|Default|GetTutRHand) false true)
  (Rendering|SetVisibility (Variables|Default|GetTutLHand) false true))

(event Custom|FireballTutorial
  (bind _showlocation (CallFunction|GetShowLocation))
  (Utilities|FlowControl|Delay 2.5)
  (|SetupFireballTut _showlocation)
  (|FireballHandAnim))

(event Custom|ShieldTutorial
  (bind _showlocation (CallFunction|GetShowLocation))
  (Utilities|FlowControl|Delay 2.5)
  (|SetupShieldTut _showlocation)
  (|ShieldHandAnim))

(event Custom|MovementTutorial
  (Rendering|Components|TextRender|SetText (Variables|Default|GetTutorialText) (Utilities|Text|ToText(String) (Utilities|String|MakeLiteralString "Welcome, Young Wizard! 
Before you embark on your  
journey to save our Kingdom,")))
  (Utilities|FlowControl|Delay 5.0)
  (Rendering|Components|TextRender|SetText (Variables|Default|GetTutorialText) (Utilities|Text|ToText(String) (Utilities|String|MakeLiteralString "Let us refresh your magical  
skills, as well as loosen those 
rusty muscles and joints of yours!")))
  (Utilities|FlowControl|Delay 5.0)
  (Rendering|Components|TextRender|SetText (Variables|Default|GetTutorialText) (Utilities|Text|ToText(String) (Utilities|String|MakeLiteralString "Head left to the Tutorial Room 
to practice your magic. 
Practice makes perfect!")))
  (Utilities|FlowControl|Delay 5.0)
  (Rendering|Components|TextRender|SetText (Variables|Default|GetTutorialText) (Utilities|Text|ToText(String) (Utilities|String|MakeLiteralString "Head straight to the portal 
infront whenever you are ready!")))
  (Utilities|FlowControl|Delay 5.0)
  (Rendering|Components|TextRender|SetText (Variables|Default|GetTutorialText) (Utilities|Text|ToText(String) (Utilities|String|MakeLiteralString "Godspeed in your quest 
to safeguard our Kingdom.")))
  (Utilities|FlowControl|Delay 5.0)
  (Rendering|SetVisibility (Variables|Default|GetTutorialText) false false)
  (Rendering|SetVisibility (Variables|Default|GetTutorialWidget) true false))

(event Custom|SwordTutorial
  (bind _showlocation (CallFunction|GetShowLocation))
  (Utilities|FlowControl|Delay 2.5)
  (|SetupSwordTut _showlocation)
  (|SwordHandAnim))

(event EventTick
  (params (DeltaSeconds :type Float%20%28single-precision%29))
  ;[1 1 1] FOR TESTING
)

(fn ConstructionScript)

(fn GetShowLocation
  (bind _bp_vr_pawn (Variables|Default|GetBP_VR_Pawn))
  (if (Class|HeadMountedDisplayFunctionLibrary|IsHeadMountedDisplayEnabled)
    (return (.DevicePosition (Class|HeadMountedDisplayFunctionLibrary|GetOrientationandPosition)))
    (else
      (bind _camera_component (Default|GetCamera _bp_vr_pawn))
      (return (+ (Transformation|GetActorLocation _bp_vr_pawn) (* (Math|Vector|GetForwardVector _camera_component) 2e+02))))))

(fn SelectTutorial
  (if (Variables|Default|GetIsMovementTutorial)
    (CallFunction|MovementTutorial)
    (elif (Variables|Default|GetIsFireballTutorial)
      (CallFunction|FireballTutorial)
      (Rendering|Components|TextRender|SetText (Variables|Default|GetTutorialText) (Utilities|Text|ToText(String) (Utilities|String|MakeLiteralString "Follow the hand orientation. 
Press and Hold the  
'Trigger' button.")))
      (Variables|BP_TutorialVolume_C|SetFireballTutComplete (Variables|Default|GetMergeSpellTutorial) true)
      (elif (Variables|Default|GetIsShieldTutorial)
        (CallFunction|ShieldTutorial)
        (Rendering|Components|TextRender|SetText (Variables|Default|GetTutorialText) (Utilities|Text|ToText(String) (Utilities|String|MakeLiteralString "Follow the hand orientation. 
Press and Hold the  
'Trigger' button.")))
        (Variables|BP_TutorialVolume_C|SetShieldTutComplete (Variables|Default|GetMergeSpellTutorial) true)
        (elif (Variables|Default|GetIsSwordTutorial)
          (CallFunction|SwordTutorial)
          (Rendering|Components|TextRender|SetText (Variables|Default|GetTutorialText) (Utilities|Text|ToText(String) (Utilities|String|MakeLiteralString "Follow the hand orientation. 
Press and Hold the  
'Trigger' button.")))
          (Variables|BP_TutorialVolume_C|SetSwordTutComplete (Variables|Default|GetMergeSpellTutorial) true)
          (else
            (Collision|SetActorEnableCollision false)
            (Actor|Tick|SetActorTickEnabled false)
            (Components|Activation|SetActive (Variables|Default|GetTutorialTrigger) false false)))))))