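; BP_TutorialWidget is a world-space tutorial sign actor that shows the player control guides with an image and text.
; ShowGuide switches on the image name to set the trigger, movement or pause material and text, then reveals the background and its children.
; HideGuide hides them again, while FacePlayer rotates the actor every tick and on show to look at the player camera, billboard-style.
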(event Custom|HideGuide
  (Rendering|SetVisibility (Variables|Default|GetBG) false true))

(event Custom|ShowGuide
  (params (ImageName :type String))
  (switch string ImageName
    (:M_Trigger
      (Rendering|Material|SetMaterial (Variables|Default|GetImage) 0 (Variables|Default|GetM_Trigger))
      (Rendering|Components|TextRender|SetText (Variables|Default|GetTextRender) (Variables|Default|GetTriggerText)))
    (:M_Movement
      (Rendering|Material|SetMaterial (Variables|Default|GetImage) 0 (Variables|Default|GetM_Movement))
      (Rendering|Components|TextRender|SetText (Variables|Default|GetTextRender) (Variables|Default|GetMovementText)))
    (:M_Pause
      (Rendering|Material|SetMaterial (Variables|Default|GetImage) 0 (Variables|Default|GetM_Pause))
      (Rendering|Components|TextRender|SetText (Variables|Default|GetTextRender) (Variables|Default|GetPauseText))))
  (Rendering|SetVisibility (Variables|Default|GetBG) true true)
  (CallFunction|FacePlayer))

(event EventBeginPlay)

(event Collision|EventActorBeginOverlap
  (params (OtherActor :type Actor%20Object%20Reference)))

(event EventTick
  (params (DeltaSeconds :type Float%20%28single-precision%29))
  (CallFunction|FacePlayer))

(fn ConstructionScript)

(fn FacePlayer
  (Transformation|SetActorRotation (Math|Rotator|FindLookatRotation (Transformation|GetActorLocation) (Transformation|GetActorLocation (Game|GetPlayerCameraManager 0)))))