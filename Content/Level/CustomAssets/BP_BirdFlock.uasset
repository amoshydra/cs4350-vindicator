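; BP_BirdFlock is a flock actor that flies a group of birds in a straight line for a limited lifespan.
; The construction script sets the lifespan and adds BP_Bird child actor components at random directions, each SpawnDistance from the flock's origin.
; Tick moves the whole flock along its forward vector at FlyingSpeed, scaled by delta time and without sweeping for collision.
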(event EventBeginPlay)

(event Collision|EventActorBeginOverlap
  (params (OtherActor :type Actor%20Object%20Reference)))

(event EventTick
  (params (DeltaSeconds :type Float%20%28single-precision%29))
  (Transformation|AddActorWorldOffset (* (Transformation|GetActorForwardVector) (* DeltaSeconds (Variables|Default|GetFlyingSpeed)))))

(fn ConstructionScript
  (Actor|SetLifeSpan (Variables|Default|GetLifespan))
  (for _index (range 0 (Variables|Default|GetNumberOfBirdToSpawn))
    (bind _returnvalue (AddComponent|AddChildActorComponent false (Math|Transform|MakeTransform (* (Math|Random|RandomUnitVector) (Variables|Default|GetSpawnDistance)) "0, 0, 0" "1,1,1")))
    (ChildActorComponent|SetChildActorClass _returnvalue "/Game/Level/CustomAssets/BP_Bird.BP_Bird_C")))