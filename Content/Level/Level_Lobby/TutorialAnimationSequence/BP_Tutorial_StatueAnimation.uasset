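; Lobby tutorial statue that demonstrates a spell on an animated skeletal mesh, configured in the construction script.
; A timeline scrubs the AnimBP's progress and can replay after a timer delay.
; AnimBP notify dispatchers, gated by DoOnce nodes reset each run, spawn and create the spell, cast it and signal the gesture.
; A state value lets Pause and Resume re-enter interrupted steps, while Activate rotates the statue and ends looping.
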(event Custom|CastTutorialSpell
  (bind _relatedspellactor (Variables|Default|GetRelatedSpellActor))
  (Default|CallBeforeCast)
  (Variables|Default|Setstate 3)
  (Utilities|FlowControl|Delay 0.08)
  (if (not (Variables|Default|GetisInterupted))
    (Actor|SetLifeSpan _relatedspellactor 3.0)
    (Default|Cast _relatedspellactor)
    (Variables|Default|Setstate 4)))

(event Custom|DispatchAnimNotify_Casted_Event_0
  (Utilities|FlowControl|DoOnce false
    (:Completed
      (CallFunction|CastTutorialSpell))))

(event Custom|Deactivate
  (Variables|Default|SetisLooping false)
  (Utilities|Time|ClearandInvalidateTimerbyHandle (stale Custom|Pause _returnvalue)))

(event Custom|Pause
  (Variables|Default|SetisInterupted true)
  (bind _lerpfactor (Timeline|TimelineCreate Stop)
    (:Update
      (Class|BPISKChar|SyncProgress(Message) (Variables|Default|GetAnimationInstance) (Math|Float|Lerp 0.0 1e+02 _lerpfactor)))
    (:Finished
      (Default|CallFinishedAnimation)
      (Variables|Default|Setstate 0)
      ;[1 1 1] Looping Mechanism
      (if (Variables|Default|GetisLooping)
        (bind _returnvalue (Utilities|Time|SetTimerbyEvent (delegate Custom|ActivateAnimation) (Variables|Default|GetDelayInterval)))))))

(event Custom|Resume
  (Variables|Default|SetisInterupted false)
  (Utilities|FlowControl|Sequence
    (:then_0
      ;[1 1 1] Resume existing state
      (switch int (Variables|Default|Getstate)
        (:1
          (CallFunction|CreateSpell))
        (:3
          (CallFunction|CastSpell))))
    (:then_1
      (bind _lerpfactor (Timeline|TimelineCreate Play)
        (:Update
          (Class|BPISKChar|SyncProgress(Message) (Variables|Default|GetAnimationInstance) (Math|Float|Lerp 0.0 1e+02 _lerpfactor)))
        (:Finished
          (Default|CallFinishedAnimation)
          (Variables|Default|Setstate 0)
          ;[1 1 1] Looping Mechanism
          (if (Variables|Default|GetisLooping)
            (bind _returnvalue (Utilities|Time|SetTimerbyEvent (delegate Custom|ActivateAnimation) (Variables|Default|GetDelayInterval)))))))))

(event Custom|DispatchAnimNotify_Created_Event_0
  (Utilities|FlowControl|DoOnce false
    (:Completed
      (CallFunction|CreateTutorialSpell))))

(event Custom|ActivateAnimation
  (CallFunction|ResetAnimation)
  (bind _lerpfactor (Timeline|TimelineCreate PlayFromStart)
    (:Update
      (Class|BPISKChar|SyncProgress(Message) (Variables|Default|GetAnimationInstance) (Math|Float|Lerp 0.0 1e+02 _lerpfactor)))
    (:Finished
      (Default|CallFinishedAnimation)
      (Variables|Default|Setstate 0)
      ;[1 1 1] Looping Mechanism
      (if (Variables|Default|GetisLooping)
        (bind _returnvalue (Utilities|Time|SetTimerbyEvent (delegate Custom|ActivateAnimation) (Variables|Default|GetDelayInterval)))))))

(event Custom|CastSpell
  (bind _relatedspellactor (Variables|Default|GetRelatedSpellActor))
  (Utilities|FlowControl|Delay 0.08)
  (if (not (Variables|Default|GetisInterupted))
    (Actor|SetLifeSpan _relatedspellactor 3.0)
    (Default|Cast _relatedspellactor)
    (Variables|Default|Setstate 4)))

(event Custom|CreateSpell
  (bind _customtransform (Variables|Default|GetCustomTransform))
  (Utilities|FlowControl|Delay 0.15)
  (if (not (Variables|Default|GetisInterupted))
    (bind _returnvalue (Game|SpawnActorfromClass (Variables|Default|GetRelatedSpell) (Math|Transform|MakeTransform (+ (Transformation|GetWorldLocation (Variables|Default|GetSpellSpawnPoint)) (.location _customtransform)) (.rotation _customtransform) (.scale _customtransform)) "Undefined" self 0))
    (bind _output_get (Variables|Default|SetRelatedSpellActor _returnvalue))
    (Transformation|AttachComponentToComponent _output_get (Variables|Default|GetSpellSpawnPoint) "None" "KeepWorld" "KeepWorld" "KeepRelative" true)
    (Default|Create _output_get)
    (Variables|Default|Setstate 2)))

(event Custom|ClearTutorial
  (bind _defaultscenerootnode (Variables|Default|GetDefaultSceneRootNode))
  (bind _output_get (Variables|Default|SetoriginRot (Variables|/Script/Engine.SceneComponent|GetRelativeRotation _defaultscenerootnode)))
  (bind _rotate (Timeline|RotateClear Play)
    (:Update
      (Transformation|SetRelativeRotation _defaultscenerootnode (Math|Rotator|MakeRotator (.Roll (Math|Rotator|BreakRotator _output_get)) (.Pitch (Math|Rotator|BreakRotator _output_get)) (+ (.Yaw (Math|Rotator|BreakRotator _output_get)) _rotate)) false false))))

(event Custom|CreateTutorialSpell
  (bind _customtransform (Variables|Default|GetCustomTransform))
  (Default|CallBeforeCreate)
  (Variables|Default|Setstate 1)
  (Utilities|FlowControl|Delay 0.15)
  (if (not (Variables|Default|GetisInterupted))
    (bind _returnvalue (Game|SpawnActorfromClass (Variables|Default|GetRelatedSpell) (Math|Transform|MakeTransform (+ (Transformation|GetWorldLocation (Variables|Default|GetSpellSpawnPoint)) (.location _customtransform)) (.rotation _customtransform) (.scale _customtransform)) "Undefined" self 0))
    (bind _output_get (Variables|Default|SetRelatedSpellActor _returnvalue))
    (Transformation|AttachComponentToComponent _output_get (Variables|Default|GetSpellSpawnPoint) "None" "KeepWorld" "KeepWorld" "KeepRelative" true)
    (Default|Create _output_get)
    (Variables|Default|Setstate 2)))

(event Custom|ResetAnimation
  (Utilities|FlowControl|Sequence
    (:then_0
      (Utilities|FlowControl|DoOnce false) ; enters at Reset
    )
    (:then_1
      (Utilities|FlowControl|DoOnce false) ; enters at Reset
    )
    (:then_2
      (Utilities|FlowControl|DoOnce false) ; enters at Reset
    )))

(event Custom|DispatchAnimNotify_Ready_Event_0
  (Utilities|FlowControl|DoOnce false
    (:Completed
      (Utilities|FlowControl|Delay 0.5)
      (Default|CallGestureinPosition))))

(event EventBeginPlay
  (Utilities|FlowControl|Sequence
    (:then_0
      (bind _output_get (Variables|Default|SetAnimationInstance (.AsABP%20SKChar%20Tutorial%20Spell (Utilities|Casting|CastToABP_SKChar_Tutorial_Spell (Components|SkeletalMesh|GetAnimInstance (Variables|Default|GetSkeletalMesh))))))
      (Utilities|FlowControl|Sequence
        (:then_0
          (EventDispatchers|AssignDispatchAnimNotifyCreated _output_get (delegate Custom|DispatchAnimNotify_Created_Event_0)))
        (:then_1
          (EventDispatchers|AssignDispatchAnimNotifyCasted _output_get (delegate Custom|DispatchAnimNotify_Casted_Event_0)))
        (:then_2
          (EventDispatchers|AssignDispatchAnimNotifyReady _output_get (delegate Custom|DispatchAnimNotify_Ready_Event_0)))))
    (:then_1
      (if (Variables|Default|GetAutoActivate)
        (CallFunction|ActivateAnimation)
        (Utilities|FlowControl|Delay 5.0)))))

(event Collision|EventActorBeginOverlap
  (params (OtherActor :type Actor%20Object%20Reference)))

(event EventActivate
  (params (CurrentCheckpoint :type Integer))
  (CallFunction|ClearTutorial)
  (Variables|Default|SetisLooping false))

(fn ConstructionScript
  (bind _stand (Variables|Default|GetStand))
  (bind _skeletalmesh (Variables|Default|GetSkeletalMesh))
  (bind _box (Variables|Default|GetBox))
  (bind _skeletalmesh_2 (Variables|Default|GetSkeletalMesh))
  (Utilities|FlowControl|Sequence
    (:then_0
      (Components|Animation|SetAnimationMode _skeletalmesh "AnimationBlueprint")
      (Components|SkeletalMesh|SetAnimInstanceClass _skeletalmesh (Variables|Default|GetAnimationBP)))
    (:then_1
      (Class|SkinnedMeshComponent|SetSkeletalMesh _skeletalmesh (Variables|Default|GetSkeletal%20Mesh) true)
      (Rendering|Material|SetMaterial _skeletalmesh 0 (Variables|Default|GetSkeletal%20Material)))
    (:then_2
      (Transformation|SetRelativeLocation _skeletalmesh_2 (+ (Variables|/Script/Engine.SceneComponent|GetRelativeLocation _skeletalmesh_2) (Variables|Default|GetoffsetTutorial)) false false)
      (Transformation|SetRelativeLocation _stand (+ (Variables|/Script/Engine.SceneComponent|GetRelativeLocation _stand) (Variables|Default|GetoffsetTutorial)) false false)
      (Transformation|SetRelativeLocation _box (+ (Variables|/Script/Engine.SceneComponent|GetRelativeLocation _box) (Variables|Default|GetoffsetTutorial)) false false))))