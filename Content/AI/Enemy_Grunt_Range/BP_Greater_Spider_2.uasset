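; Ranged Greater Spider enemy for a VR game that turns in place toward the player and fires projectiles, with the base knockback overridden to do nothing.
; MoveTo start binds a tick listener that interpolates yaw toward a sampled player direction and drives left/right turn animations.
; Once aligned, it stores the camera location as the projectile target and briefly raises InAttackRange.
; The movement range check also requires a line trace hit on the VR pawn.
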(event Custom|SetRotateAnimation
  (params (rotateAngle :type Float%20%28single-precision%29))
  (bind _mesh (Variables|Character|GetMesh))
  (bind _returnvalue (Components|SkeletalMesh|GetAnimInstance _mesh))
  ;[1 1 1] Set Rotate animation
  (if (Math|Float|NearlyEqual(Float) rotateAngle 0.0 (Variables|Default|GetAcceptanceRotationTolerance))
    (Class|BPIEnemyAnimation|SetRotateLeft(Message) _returnvalue false)
    (Class|BPIEnemyAnimation|SetRotateRight(Message) _returnvalue false)
    (elif (< rotateAngle 0.0)
      (Class|BPIEnemyAnimation|SetRotateLeft(Message) _returnvalue true)
      (else
        (Class|BPIEnemyAnimation|SetRotateRight(Message) _returnvalue true)))))

(event Custom|EventTickListener_Event_0
  (params (DeltaSecond :type Float%20%28single-precision%29))
  ;[1 1 1] Rotate Enemy
  (bind _output_get (Variables|Default|SetEnemyRotationTickSecond (+ DeltaSecond (Variables|Default|GetEnemyRotationTickSecond))))
  (Transformation|SetActorRotation (Math|Rotator|MakeRotator 0.0 0.0 (.yaw (Math|Interpolation|RInterpTo (Variables|Default|GetEnemyTempRotation) (Variables|Default|GetPlayerTempRotation) _output_get (Variables|Default|GetInterpSpeed)))))
  (CallFunction|SetRotateAnimation (- (.Yaw (Math|Rotator|BreakRotator (Variables|Default|GetPlayerTempRotation))) (.Yaw (Math|Rotator|BreakRotator (Transformation|GetActorRotation)))))
  (if (Math|Float|NearlyEqual(Float) (- (.Yaw (Math|Rotator|BreakRotator (Variables|Default|GetPlayerTempRotation))) (.Yaw (Math|Rotator|BreakRotator (Transformation|GetActorRotation)))) 0.0 (Variables|Default|GetAcceptanceRotationTolerance))
    (if (Math|Float|NearlyEqual(Float) (.yaw (Transformation|GetActorRotation)) (.yaw (Math|Rotator|FindLookatRotation (Transformation|GetActorLocation) (Transformation|GetActorLocation (Game|Player|GetPlayerPawn 0)))) (Variables|Default|GetAcceptanceRotationTolerance))
      (Variables|Default|SetAttackLocation (Transformation|GetActorLocation (Game|GetPlayerCameraManager 0)))
      ;[1 1 1] Prepare to attack Player
      (Utilities|FlowControl|DoOnce false :!label _label
        (:Completed
          (Variables|Default|SetinAttackRange true)
          (Utilities|FlowControl|Delay 2.2)
          (Variables|Default|SetinAttackRange false)
          (Utilities|FlowControl|Sequence
            (:then_0
              (Utilities|FlowControl|DoOnce false) ; enters at Reset
            )
            (:then_1
              (goto _label Reset)))))
      (else
        (Utilities|FlowControl|DoOnce false) ; enters at Reset
      ))))

(event Custom|RotateEnemy
  ;[1 1 1] Rotate Enemy
  (Utilities|FlowControl|DoOnce false
    (:Completed
      (Variables|Default|SetEnemyTempRotation (Transformation|GetActorRotation))
      (Variables|Default|SetPlayerTempRotation (Math|Rotator|FindLookatRotation (Transformation|GetActorLocation) (Transformation|GetActorLocation (Game|Player|GetPlayerPawn 0))))
      (EventDispatchers|AssignEventTickListener (delegate Custom|EventTickListener_Event_0)))))

(event EventBeginPlay
  (|CallParentFunction))

(event EventSetIsDamaged
  (params (isDamaged :type Boolean) (DamagePoint :type Float%20%28single-precision%29))
  ;[1 1 1] Overwrite Base KnockBack function
)

(event EventTick
  (params (DeltaSeconds :type Float%20%28single-precision%29))
  (|CallParentFunction DeltaSeconds)
  (Default|CallEventTickListener DeltaSeconds))

(event EventMoveTo:Stop
  ;[1 1 1] Overwrite MoveTo:Stop function to stop rotate
  (EventDispatchers|UnbindEventfromEventTickListener (delegate Custom|EventTickListener_Event_0))
  (CallFunction|SetRotateAnimation 0.0)
  (Variables|Default|SetEnemyRotationTickSecond 0.0)
  ;[1 1 1] Rotate Enemy
  (Utilities|FlowControl|DoOnce false) ; enters at Reset
)

(event EventMoveTo:Start
  ;[1 1 1] Overwrite MoveTo:Start function to rotate grunt
  (CallFunction|RotateEnemy))

(fn ConstructionScript
  (|CallParentFunction))

(fn ShootProjectile
  (bind _returnvalue (Game|SpawnActorfromClass "/Game/AI/Enemy_Grunt_Range/BP_Enemy_Range_Projectile.BP_Enemy_Range_Projectile_C" (Transformation|GetWorldTransform (Variables|Default|GetProjectileSpawnPoint)) "Undefined" 0 0))
  (Default|ReceiveFinalDestination _returnvalue (Variables|Default|GetAttackLocation))
  (Default|Create _returnvalue))

(fn CheckinMovementRange
  (bind _inmovementrange (|CallParentFunction))
  (if _inmovementrange
    (bind _outhit (Collision|LineTraceForObjects (Transformation|GetActorLocation self) (Transformation|GetActorLocation (Game|Player|GetPlayerPawn 0)) (Utilities|Array|MakeArray "ObjectTypeQuery1" "ObjectTypeQuery3") false 0 "None"))
    (return (.bSuccess (Utilities|Casting|CastToBP_VR_Pawn (.hitactor _outhit))))
    (else
      (return false))))