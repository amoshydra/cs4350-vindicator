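; Ranged grunt enemy that turns to face the player and can spawn projectiles from its spawn point.
; Each tick it checks player distance, then updates its attack flag from a narrow yaw tolerance.
; MoveTo overrides start and stop turning: a temporary tick listener interpolates yaw, drives left/right turn animations and unbinds once nearly aligned.
; ShootProjectile spawns and initializes the projectile, but nothing in this Blueprint calls it.
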(event Custom|SetRotate
  (params (rotateAngle :type Float%20%28single-precision%29))
  (bind _mesh (Variables|Character|GetMesh))
  (bind _returnvalue (Components|SkeletalMesh|GetAnimInstance _mesh))
  ;[1 1 1] Set Rotate
  (if (< rotateAngle 0.0)
    (Class|BPIEnemyAnimation|SetRotateLeft(Message) (Components|SkeletalMesh|GetAnimInstance (Variables|Character|GetMesh)) true)
    (elif (== rotateAngle 0.0)
      (Class|BPIEnemyAnimation|SetRotateLeft(Message) _returnvalue false)
      (Class|BPIEnemyAnimation|SetRotateRight(Message) _returnvalue false)
      (else
        (Class|BPIEnemyAnimation|SetRotateRight(Message) _returnvalue true)))))

(event Custom|EventTickListener_Event_0
  (params (DeltaSecond :type Float%20%28single-precision%29))
  (bind _returnvalue (Transformation|GetActorRotation))
  (bind _returnvalue_2 (Transformation|GetActorLocation))
  (bind _returnvalue_3 (Game|Player|GetPlayerPawn 0))
  (bind _returnvalue_4 (Transformation|GetActorLocation _returnvalue_3))
  (bind _returnvalue_5 (Math|Rotator|FindLookatRotation _returnvalue_2 _returnvalue_4))
  ;[1 1 1] Rotate Enemy
  (Transformation|SetActorRotation (Math|Rotator|MakeRotator 0.0 0.0 (.yaw (Math|Interpolation|RInterpTo _returnvalue _returnvalue_5 DeltaSecond 1.5))))
  (CallFunction|CheckifPawninSight)
  (CallFunction|SetRotate (- (.Yaw (Math|Rotator|BreakRotator _returnvalue_5)) (.Yaw (Math|Rotator|BreakRotator _returnvalue))))
  (if (Math|Rotator|Equal(Rotator) _returnvalue_5 _returnvalue 5.0)
    (EventDispatchers|UnbindEventfromEventTickListener (delegate Custom|EventTickListener_Event_0))))

(event Custom|RotatePlayer
  ;[1 1 1] Rotate Enemy
  (EventDispatchers|AssignEventTickListener (delegate Custom|EventTickListener_Event_0)))

(event EventBeginPlay
  (|CallParentFunction))

(event Collision|EventActorBeginOverlap
  (params (OtherActor :type Actor%20Object%20Reference)))

(event EventTick
  (params (DeltaSeconds :type Float%20%28single-precision%29))
  (|CallParentFunction DeltaSeconds)
  (Default|CallEventTickListener DeltaSeconds)
  (bind _inrange (CallFunction|CheckifPawninRange))
  (if _inrange
    (CallFunction|CheckifPawninSight)))

(event EventMoveTo:Stop
  ;[1 1 1] Overwrite MoveTo:Stop function to stop rotate
  (CallFunction|SetRotate 0.0))

(event EventMoveTo:Start
  ;[1 1 1] Overwrite MoveTo:Start function to rotate grunt
  (CallFunction|RotatePlayer))

(fn ConstructionScript
  (|CallParentFunction))

(fn GetLookatRotationDifference
  (bind _returnvalue (Game|Player|GetPlayerPawn 0))
  (bind _returnvalue_2 (Transformation|GetActorLocation))
  (bind _returnvalue_3 (Transformation|GetActorRotation))
  (bind _returnvalue_4 (Transformation|GetActorLocation _returnvalue))
  (bind _returnvalue_5 (Math|Rotator|FindLookatRotation _returnvalue_2 _returnvalue_4))
  (return _returnvalue_3 _returnvalue_5 (Math|Float|InRange(Float) (- (.Yaw (Math|Rotator|BreakRotator _returnvalue_3)) (.Yaw (Math|Rotator|BreakRotator _returnvalue_5))) -2.5 2.5)))

(fn CheckifPawninRange
  (bind _output_get (Variables|Default|SetinMovementRange (< (Math|Vector|VectorLength (- (Transformation|GetActorLocation) (Transformation|GetActorLocation (Game|Player|GetPlayerPawn 0)))) (Variables|Default|GetAvailableRange))))
  (return _output_get))

(fn CheckifPawninSight
  (Variables|Default|SetinAttackRange (Math|Float|InRange(Float) (- (.yaw (Transformation|GetActorRotation)) (.yaw (Math|Rotator|FindLookatRotation (Transformation|GetActorLocation) (Transformation|GetActorLocation (Game|Player|GetPlayerPawn 0))))) -2.5 2.5)))

(fn ShootProjectile
  (bind _returnvalue (Game|SpawnActorfromClass "/Game/AI/Enemy_Grunt_Range/BP_Enemy_Range_Projectile.BP_Enemy_Range_Projectile_C" (Transformation|GetWorldTransform (Variables|Default|GetProjectileSpawnPoint)) "Undefined" 0 0))
  (Default|Create _returnvalue))