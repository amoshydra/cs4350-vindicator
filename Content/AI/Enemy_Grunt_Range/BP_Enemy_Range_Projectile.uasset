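; Projectile for the ranged grunt enemy that arcs toward a supplied destination and damages the VR player on contact.
; When Create runs, it computes a toss velocity with launch speed scaled to distance, applies it to the projectile movement, then resets the trail effect's time dilation after a short delay.
; Overlapping the VR pawn applies damage and activates the explosion effect, without destroying the projectile.
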(event OnComponentBeginOverlap(CollisionVolume)
  (params (OverlappedComponent :type Primitive%20Component%20Object%20Reference) (OtherActor :type Actor%20Object%20Reference) (OtherComp :type Primitive%20Component%20Object%20Reference) (OtherBodyIndex :type Integer) (bFromSweep :type Boolean) (SweepResult :type Hit%20Result%20Structure%20%28by%20ref%29))
  ;[1 1 1] Damage Player
  (bind _asbp_vr_pawn (Utilities|Casting|CastToBP_VR_Pawn OtherActor))
  (Default|DamagePlayer _asbp_vr_pawn 5.0)
  (Components|Activation|Activate (Variables|Default|GetExplosionEffect) false))

(event EventBeginPlay
  (|CallParentFunction))

(event EventTick
  (params (DeltaSeconds :type Float%20%28single-precision%29))
  (|CallParentFunction DeltaSeconds))

(event EventCreate
  (bind _returnvalue (Transformation|GetActorLocation))
  (bind _finaldestination (Variables|Default|GetFinalDestination))
  (bind (_tossvelocity _returnvalue_2) (Class|GameplayStatics|BlueprintSuggestProjectileVelocity _returnvalue _finaldestination (* (Math|Vector|VectorLength (- _returnvalue _finaldestination)) 1.0) 0.0 "DoNotTrace" 0.0 false true))
  (if _returnvalue_2
    (Variables|/Script/Engine.MovementComponent|SetVelocity (Variables|Default|GetProjectileMovement) _tossvelocity)
    (Utilities|FlowControl|Delay 1.0)
    (Variables|/Script/Engine.ParticleSystemComponent|SetCustomTimeDilation (Variables|Default|GetTrailingParticleEffect) 1.0)))

(fn ConstructionScript
  (|CallParentFunction))

(fn ReceiveFinalDestination
  (params (FinalDestination :type Vector))
  (Variables|Default|SetFinalDestination FinalDestination))