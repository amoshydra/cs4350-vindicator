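; Tutorial enemy that serves as a ranged target, reacting only to fireball spell overlaps.
; On overlap, it adds the fireball to ExistingEnemy and uses the result to gate damage feedback and a SetHealth call with one third of default health.
; With a valid HP bar, it updates the bar and destroys itself at zero health.
; DamageEnemyEvent is left empty, and BeginPlay and Tick are disabled.
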(event EventBeginPlay
  (|CallParentFunction))

(event EventTick
  (params (DeltaSeconds :type Float%20%28single-precision%29))
  (|CallParentFunction DeltaSeconds))

(event Collision|EventActorBeginOverlap
  (params (OtherActor :type Actor%20Object%20Reference))
  (bind _asbp_spell_fireball (Utilities|Casting|CastToBP_Spell_Fireball OtherActor))
  (bind _returnvalue (Utilities|Set|Add (Variables|Default|GetExistingEnemy) _asbp_spell_fireball))
  (if _returnvalue
    (CallFunction|DamageEnemyFeedbackEvent)
    (CallFunction|SetHealth (/ (Variables|Default|GetDefaultHealth) 3.0))
    (bind _hpbarref (Variables|Default|GetHPBarRef)
      (:then
        (Default|UpdateHP _hpbarref (Variables|Default|GetCurrentHealth))
        (if (<= (Variables|Default|GetCurrentHealth) 0.0)
          (Actor|DestroyActor)))
      (:else))))

(event EventDamageEnemyEvent
  (params (DamagePoints :type Float%20%28single-precision%29)))

(fn ConstructionScript
  (|CallParentFunction))