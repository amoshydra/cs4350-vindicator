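; Tutorial enemy that serves as a target for the Lightning Blade melee spell.
; Its MoveTo start and DamageEnemyEvent handlers are empty, leaving overlap with BP_Spell_LightningBlade as the only hit logic here.
; Each such overlap fires damage feedback and passes a fifteenth of default health to SetHealth.
; If the HP bar reference is valid, it updates the bar and destroys the actor at zero health.
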(event EventBeginPlay
  (|CallParentFunction))

(event EventTick
  (params (DeltaSeconds :type Float%20%28single-precision%29))
  (|CallParentFunction DeltaSeconds))

(event Collision|EventActorBeginOverlap
  (params (OtherActor :type Actor%20Object%20Reference))
  (Utilities|Casting|CastToBP_Spell_LightningBlade OtherActor)
  (CallFunction|DamageEnemyFeedbackEvent)
  (CallFunction|SetHealth (/ (Variables|Default|GetDefaultHealth) 15.0))
  (bind _hpbarref (Variables|Default|GetHPBarRef)
    (:then
      (Default|UpdateHP _hpbarref (Variables|Default|GetCurrentHealth))
      (if (<= (Variables|Default|GetCurrentHealth) 0.0)
        (Actor|DestroyActor)))
    (:else)))

(event EventMoveTo:Start)

(event EventDamageEnemyEvent
  (params (DamagePoints :type Float%20%28single-precision%29)))

(fn ConstructionScript
  (|CallParentFunction))