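; Base enemy character for a VR game that chases and attacks the player pawn, registering itself with the game instance while alive.
; It exposes move, attack and range-check functions, using overlaps for attack range and distance for movement range.
; Damage lowers health, updates a child-actor HP bar, flashes a point light and flags death.
; Speed, health, attack and damaged states are pushed to the AnimInstance through message calls.
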(event Custom|SetHealth
  (params (DamagePoints :type Float%20%28single-precision%29))
  ;[1 1 1] Set Health
  (bind _output_get (Variables|Default|SetCurrentHealth (- (Variables|Default|GetCurrentHealth) DamagePoints)))
  (Class|BPIEnemyAnimation|SetHealth(Message) (Components|SkeletalMesh|GetAnimInstance (Variables|Character|GetMesh)) _output_get))

(event Custom|DamageEnemyFeedback_Event
  ;[1 1 1] Feedback for Damaging Enemy
  (CallFunction|SetIsDamaged true)
  (Rendering|SetVisibility (Variables|Default|GetPointLight) true false)
  (Utilities|FlowControl|Delay 0.1)
  (Rendering|SetVisibility (Variables|Default|GetPointLight) false false))

(event Custom|SetSpeedFactor
  (params (SpeedFactor :type Float%20%28single-precision%29))
  ;[1 1 1] Set Speed Factor
  (Variables|/Script/Engine.CharacterMovementComponent|SetMaxWalkSpeed (Variables|Character|GetCharacterMovement) (* SpeedFactor (Variables|Default|GetDefaultSpeed))))

(event Custom|SetIsDamaged
  (params (isDamaged :type Boolean))
  ;[1 1 1] Set Is Damaged
  (bind _output_get (Variables|Default|SetisDamaged isDamaged))
  (Class|BPIEnemyAnimation|SetIsDamaged(Message) (Components|SkeletalMesh|GetAnimInstance (Variables|Character|GetMesh)) _output_get))

(event Custom|AIMoveToWrapper
  (params (Pawn :type Pawn%20Object%20Reference) (Destination :type Vector) (TargetActor :type Actor%20Object%20Reference) (AcceptanceRadius :type Float%20%28single-precision%29) (Stop%20on%20Overlap :type Boolean))
  ;[1 1 1] AI MoveTo Wrapper
  (AI|AIMoveTo Pawn Destination TargetActor AcceptanceRadius Stop%20on%20Overlap))

(event Custom|AddToGameInstance
  ;[1 1 1] Manage Game Instance
  (bind _asbp_game_instance (Utilities|Casting|CastToBP_GameInstance (Game|GetGameInstance)))
  (Default|AddEnemy _asbp_game_instance self))

(event Custom|RemoveFromGameInstance
  ;[1 1 1] Manage Game Instance
  (bind _asbp_game_instance (Utilities|Casting|CastToBP_GameInstance (Game|GetGameInstance)))
  (Default|RemoveEnemy _asbp_game_instance self))

(event Custom|DamageEnemy_Event
  (params (DamagePoints :type Float%20%28single-precision%29))
  ;[1 1 1] Damage Enemy
  (CallFunction|DamageEnemyFeedbackEvent)
  (CallFunction|SetHealth DamagePoints)
  (bind _hpbarref (Variables|Default|GetHPBarRef)
    (:then
      (Default|UpdateHP _hpbarref (Variables|Default|GetCurrentHealth))
      (CallFunction|CheckIsAlive))
    (:else)))

(event Custom|SetSpeed
  (params (Speed :type Float%20%28single-precision%29))
  ;[1 1 1] Set Speed
  (Class|BPIEnemyAnimation|SetSpeed(Message) (Components|SkeletalMesh|GetAnimInstance (Variables|Character|GetMesh)) Speed))

(event Custom|CheckIsAlive
  ;[1 1 1] Check Enemy Is Alive
  (if (<= (Variables|Default|GetCurrentHealth) 0.0)
    (Variables|Default|SetisDead true)))

(event Custom|DestroyEnemy
  ;[1 1 1] Destory Enemy
  (Actor|DestroyActor))

(event Custom|SetAttack
  (params (isAttacking :type Boolean))
  ;[1 1 1] Set Attack
  (bind _output_get (Variables|Default|SetisAttacking isAttacking))
  (Class|BPIEnemyAnimation|SetAttack(Message) (Components|SkeletalMesh|GetAnimInstance (Variables|Character|GetMesh)) _output_get))

(event EventBeginPlay
  (CallFunction|AddtoGameInstance)
  (CallFunction|SetSpeedFactor 1.0)
  (CallFunction|SetSpeed (Variables|Default|GetDefaultSpeed))
  (CallFunction|SetHealth 0.0)
  (CallFunction|InitializeHealthBar))

(event EventDestroyed
  (CallFunction|RemovefromGameInstance))

(event Collision|EventActorBeginOverlap
  (params (OtherActor :type Actor%20Object%20Reference))
  ;[1 1 1] Set Attack Range
  (Utilities|Casting|CastToBP_VR_Pawn OtherActor)
  (Variables|Default|SetinAttackRange true))

(event EventTick
  (params (DeltaSeconds :type Float%20%28single-precision%29)))

(event Collision|EventActorEndOverlap
  (params (OtherActor :type Actor%20Object%20Reference))
  ;[1 1 1] Set Attack Range
  (Utilities|Casting|CastToBP_VR_Pawn OtherActor)
  (Variables|Default|SetinAttackRange false))

(fn ConstructionScript
  (bind _healthindicator_interface (Variables|Default|GetHealthIndicator_Interface))
  (bind _capsulecomponent (Variables|Collision|GetCapsuleComponent))
  (bind _capsulehalfheight (Variables|/Script/Engine.CapsuleComponent|GetCapsuleHalfHeight _capsulecomponent))
  (Utilities|FlowControl|Sequence
    (:then_0
      (Variables|Default|SetCurrentHealth (Variables|Default|GetDefaultHealth)))
    (:then_1
      ;[1 1 1] If Interface height is not adjusted, automatically set its height
      (if (== (.z (Variables|/Script/Engine.SceneComponent|GetRelativeLocation _healthindicator_interface)) 0.0)
        (Transformation|SetRelativeLocation _healthindicator_interface (Math|Vector|MakeVector 0.0 0.0 (+ _capsulehalfheight (* _capsulehalfheight 0.3))) false false)))))

(fn AttackPlayer:Start
  (CallFunction|SetAttack true))

(fn AttackPlayer:Stop
  (CallFunction|SetAttack false))

(fn InitializeHealthBar
  (bind _output_get (Variables|Default|SetHPBarRef (.AsBP%20UI%20HPBar (Utilities|Casting|CastToBP_UI_HPBar (Variables|/Script/Engine.ChildActorComponent|GetChildActor (Variables|Default|GetHealthIndicator_Interface))))))
  (Default|Initialise _output_get (Variables|Default|GetDefaultHealth)))

(fn MoveTo:Start
  (bind _asbp_vr_pawn (Utilities|Casting|CastToBP_VR_Pawn (Game|Player|GetPlayerPawn 0)))
  (CallFunction|AIMovetoWrapper self "0, 0, 0" _asbp_vr_pawn 0.0 false))

(fn MoveTo:Stop
  (Components|Movement|StopMovementImmediately (Variables|Character|GetCharacterMovement self)))

(fn CheckinMovementRange
  (bind _output_get (Variables|Default|SetinMovementRange (< (Math|Vector|VectorLength (- (Transformation|GetActorLocation) (Transformation|GetActorLocation (Game|Player|GetPlayerPawn 0)))) (Variables|Default|GetAvailableMovementRange))))
  (return _output_get))