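; Troll boss enemy that extends a parent enemy Blueprint with a ground-breaking attack against the VR player.
; Starting an attack sets IsInAttack, which blocks move starts and attack stops until cleared externally through SetIsInAttack.
; The hit check launches a sound and Timeline-driven particle, then immediately damages the player if inside the Box.
; The construction script derives particle travel distance from the Box extent and particle offset.
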(event Custom|CheckIsPlayerInHitRange
  (CallFunction|CreateAttackParticleEffect)
  (bind _asbp_vr_pawn (Utilities|Casting|CastToBP_VR_Pawn (Game|Player|GetPlayerPawn 0)))
  (if (Collision|IsOverlappingActor (Variables|Default|GetBox) _asbp_vr_pawn :!class /Script/Engine.PrimitiveComponent)
    (Default|DamagePlayer _asbp_vr_pawn (Variables|Default|GetPlayerDamagePoints))))

(event Custom|CreateAttackParticleEffect
  (bind _particleoriginalrelativeoffset (Variables|Default|GetParticleOriginalRelativeOffset))
  (Components|Activation|Activate (Variables|Default|GetParticleSystem) false)
  (Audio|PlaySoundatLocation "/Game/SoundAsset/Enemy/Monster_GroundBreaking.Monster_GroundBreaking" (Transformation|GetActorLocation))
  (bind _newtrack_0 (Timeline|Timeline_0 PlayFromStart)
    (:Update
      (Transformation|SetRelativeLocation (Variables|Default|GetParticleSystem) (Math|Vector|MakeVector (+ (Math|Float|Lerp 0.0 (Variables|Default|GetParticleTravelDistance) _newtrack_0) (.x _particleoriginalrelativeoffset)) 0.0 (.z _particleoriginalrelativeoffset)) false false))
    (:Finished
      (Components|Activation|Deactivate (Variables|Default|GetParticleSystem)))))

(event EventBeginPlay
  (|CallParentFunction))

(event Collision|EventActorBeginOverlap
  (params (OtherActor :type Actor%20Object%20Reference))
  (|CallParentFunction OtherActor))

(event EventTick
  (params (DeltaSeconds :type Float%20%28single-precision%29))
  (|CallParentFunction DeltaSeconds))

(event EventMoveTo:Start
  (if (not (Variables|Default|GetisInAttack))
    (|CallParentFunction)))

(event EventAttackPlayer:Start
  (|CallParentFunction)
  (Variables|Default|SetisInAttack true))

(event EventAttackPlayer:Stop
  (if (not (Variables|Default|GetisInAttack))
    (|CallParentFunction)))

(fn ConstructionScript
  (|CallParentFunction)
  (Utilities|FlowControl|Sequence
    (:then_0
      (Variables|Default|SetParticleTravelDistance (* (+ (.x (Variables|/Script/Engine.BoxComponent|GetBoxExtent (Variables|Default|GetBox))) (* -1 (.x (Variables|/Script/Engine.SceneComponent|GetRelativeLocation (Variables|Default|GetParticleSystem))))) 0.9)))
    (:then_1
      (Variables|Default|SetParticleOriginalRelativeOffset (Variables|/Script/Engine.SceneComponent|GetRelativeLocation (Variables|Default|GetParticleSystem))))))

(fn SetIsinAttack
  (params (isInAttack :type Boolean))
  (Variables|Default|SetisInAttack isInAttack))