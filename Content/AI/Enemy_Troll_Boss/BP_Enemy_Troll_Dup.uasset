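; Troll boss enemy Blueprint that extends a parent enemy's move-to and attack-player behavior with an attack-state guard.
; Starting an attack sets IsInAttack, which blocks move-to start and attack stop from reaching the parent; nothing in this graph clears the flag.
; Attack start also runs a forward capsule trace on the Pawn profile, with debug drawing and a printed hit actor name.
; BeginPlay sets InterpSpeed after parent initialization.
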(event EventBeginPlay
  (|CallParentFunction)
  (Variables|Default|SetInterpSpeed 0.4))

(event Collision|EventActorBeginOverlap
  (params (OtherActor :type Actor%20Object%20Reference))
  (|CallParentFunction OtherActor))

(event EventMoveTo:Start
  ;[1 1 1] Start Move To only when enemy is not currently attacking
  (if (not (Variables|Default|GetisInAttack))
    (|CallParentFunction)))

(event EventAttackPlayer:Stop
  ;[1 1 1] Stop move to only when enemy is not currently attacking
  (if (not (Variables|Default|GetisInAttack))
    (|CallParentFunction)))

(event EventAttackPlayer:Start
  (bind _returnvalue (Transformation|GetActorLocation))
  ;[1 1 1] Set enemy to is currently attacking
  (|CallParentFunction)
  (Variables|Default|SetisInAttack true)
  (bind _outhit (Class|KismetSystemLibrary|CapsuleTraceSinglebyProfile _returnvalue (+ _returnvalue (* (Transformation|GetActorForwardVector) 1e+03)) 5e+01 5e+01 "Pawn" false 0 "ForDuration" true))
  (Development|PrintString (Utilities|GetDisplayName (.hitactor _outhit))))

(event EventTick
  (params (DeltaSeconds :type Float%20%28single-precision%29))
  (|CallParentFunction DeltaSeconds))

(fn ConstructionScript
  (|CallParentFunction))