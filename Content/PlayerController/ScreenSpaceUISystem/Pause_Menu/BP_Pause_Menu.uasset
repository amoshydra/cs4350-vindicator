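; Pause menu actor that builds a vertical list of items from 3D cubes and text components instead of widgets.
; The construction script creates a cube and label per TextArray entry, maps cubes to indices, and enables custom depth on both.
; Cube overlaps swap the hover color through dynamic materials and set or reset SelectedItemIndex.
; Tick prints that index for debugging; nothing here acts on the selection.
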(event Custom|OnComponentBeginOverlap_Event_0
  (params (OverlappedComponent :type Primitive%20Component%20Object%20Reference) (OtherActor :type Actor%20Object%20Reference) (OtherComp :type Primitive%20Component%20Object%20Reference) (OtherBodyIndex :type Integer) (bFromSweep :type Boolean) (SweepResult :type Hit%20Result%20Structure%20%28by%20ref%29))
  (bind _returnvalue (Rendering|Material|CreateDynamicMaterialInstance OverlappedComponent 0 (Rendering|Material|GetMaterial OverlappedComponent 0) :!class /Script/Engine.PrimitiveComponent))
  (Rendering|Material|SetVectorParameterValue _returnvalue "Base Color" (Variables|Default|GetItemColor-Hover) :!class /Script/Engine.MaterialInstanceDynamic)
  (Variables|Default|SetSelectedItemIndex (.Value (Utilities|Map|Find (Variables|Default|GetItemMap) 0))))

(event Custom|OnComponentEndOverlap_Event_0
  (params (OverlappedComponent :type Primitive%20Component%20Object%20Reference) (OtherActor :type Actor%20Object%20Reference) (OtherComp :type Primitive%20Component%20Object%20Reference) (OtherBodyIndex :type Integer))
  (bind _returnvalue (Rendering|Material|CreateDynamicMaterialInstance OverlappedComponent 0 (Rendering|Material|GetMaterial OverlappedComponent 0) :!class /Script/Engine.PrimitiveComponent))
  (Rendering|Material|SetVectorParameterValue _returnvalue "Base Color" (Variables|Default|GetItemColor) :!class /Script/Engine.MaterialInstanceDynamic)
  (Variables|Default|SetSelectedItemIndex -1))

(event EventBeginPlay)

(event Collision|EventActorBeginOverlap
  (params (OtherActor :type Actor%20Object%20Reference)))

(event Collision|EventActorEndOverlap
  (params (OtherActor :type Actor%20Object%20Reference)))

(event EventTick
  (params (DeltaSeconds :type Float%20%28single-precision%29))
  (Development|PrintString (Utilities|String|ToString(Integer) (Variables|Default|GetSelectedItemIndex)) true true "(R=0.000000,G=0.660000,B=1.000000,A=1.000000)" 0.1))

(fn ConstructionScript
  (Utilities|Map|Clear (Variables|Default|GetItemMap))
  (for (_array_element _array_index) (Variables|Default|GetTextArray)
    (bind _returnvalue (AddComponent|AddStaticMeshComponent false (Math|Transform|MakeTransform (Math|Vector|MakeVector -5.0 0.0 (* (* _array_index -1) (Variables|Default|GetItemSpacing))) "-90.000000, 0, 0" (Variables|Default|GetItemScale))))
    (Utilities|FlowControl|Sequence
      (:then_0
        (Utilities|FlowControl|Sequence
          (:then_0
            (Components|StaticMesh|SetStaticMesh _returnvalue "/Engine/BasicShapes/Cube.Cube"))
          (:then_1
            (bind _returnvalue_2 (Rendering|Material|CreateDynamicMaterialInstance "/Game/PlayerController/ScreenSpaceUISystem/TextMaterials/MenuBackgroundMaterial.MenuBackgroundMaterial" :!class /Script/Engine.KismetMaterialLibrary))
            (Rendering|Material|SetVectorParameterValue _returnvalue_2 "Base Color" (Variables|Default|GetItemColor) :!class /Script/Engine.MaterialInstanceDynamic)
            (Rendering|Material|SetMaterial _returnvalue 0 _returnvalue_2))
          (:then_2
            (Rendering|SetRenderCustomDepth _returnvalue true)
            (Rendering|SetCustomDepthStencilValue _returnvalue 2)
            (Variables|/Script/Engine.PrimitiveComponent|SetbGenerateOverlapEvents _returnvalue true)
            (Collision|SetCollisionEnabled _returnvalue "QueryOnly")
            (Collision|SetCollisionObjectType _returnvalue "ECC_WorldDynamic"))
          (:then_3
            (Utilities|Map|Add (Variables|Default|GetItemMap) _returnvalue _array_index))
          (:then_4
            (Utilities|FlowControl|Sequence
              (:then_0
                (Collision|BindEventtoOnComponentBeginOverlap _returnvalue (EventDispatchers|CreateEvent :!event Custom|OnComponentBeginOverlap_Event_0)))
              (:then_1
                (Collision|BindEventtoOnComponentEndOverlap _returnvalue (EventDispatchers|CreateEvent :!event Custom|OnComponentEndOverlap_Event_0)))))))
      (:then_1
        (bind _returnvalue_3 (AddComponent|AddTextRenderComponent false (Math|Transform|MakeTransform (Math|Vector|MakeVector 0.0 0.0 (* (* _array_index -1) (Variables|Default|GetItemSpacing))) "0, 0, 0" "1,1,1")))
        (Utilities|FlowControl|Sequence
          (:then_0
            (Rendering|Components|TextRender|SetText _returnvalue_3 (Utilities|Text|ToText(String) _array_element)))
          (:then_1
            (Rendering|Components|TextRender|SetHorizontalAlignment _returnvalue_3 "EHTA_Center"))
          (:then_2
            (Class|TextRenderComponent|SetVerticalAlignment _returnvalue_3 "EVRTA_TextCenter"))
          (:then_3
            (Rendering|Components|TextRender|SetTextRenderColor _returnvalue_3 (Variables|Default|GetTextColor)))
          (:then_4
            (Class|TextRenderComponent|SetTextMaterial _returnvalue_3 "/Game/PlayerController/ScreenSpaceUISystem/TextMaterials/AntiAliasedTextMaterialTranslucent_Emissive.AntiAliasedTextMaterialTranslucent_Emissive"))
          (:then_5
            (Rendering|SetRenderCustomDepth _returnvalue_3 true))
          (:then_6
            (Rendering|Components|TextRender|SetWorldSize _returnvalue_3 (Variables|Default|GetTextSize))))))))