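; Screen-space feedback actor for the parent VR pawn, handling death, pause and damage effects.
; It caches the pawn camera's post-process settings, then darkens and tints them for pause or a timeline-driven death fade with slowing time.
; Left shoulder presses flip-flop pause; damage triggers camera fades scaled by damage.
; CreateUIMenu builds no widget: it stops time and, through a hardcoded true branch, reloads the level.
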(event Custom|Dead:Activate
  (bind _newtrack_0 (Timeline|Timeline_0 PlayFromStart)
    (:Update
      (CallFunction|DarkenScreen (Math|Float|Lerp 1.0 0.0 _newtrack_0) (Math|Color|Lerp(LinearColor) "(R=1.000000,G=1.000000,B=1.000000,A=1.000000)" "(R=1.000000,G=0.000000,B=0.000000,A=1.000000)" _newtrack_0))
      (Utilities|Time|SetGlobalTimeDilation (Math|Float|Lerp 1.0 0.0 _newtrack_0))
      (if (< (Math|Float|Lerp 1.0 0.0 _newtrack_0) 0.05)
        (Utilities|FlowControl|Sequence
          (:then_0
            (Timeline|Timeline_0 Stop))
          (:then_1
            (CallFunction|CreateUIMenu)))))))

(event Custom|Pause:Activate
  (CallFunction|DarkenScreen 0.0)
  (CallFunction|CreateUIMenu))

(event Custom|Pause:Deactivate
  (CallFunction|ResetSettings)
  (CallFunction|DestroyUIMenu))

(event Custom|__DarkenScreen
  (params (Alpha :type Float%20%28single-precision%29) (SceneColor%20%28Optional%29 :type Linear%20Color%20Structure :default "(R=1.000000,G=1.000000,B=1.000000,A=1.000000)"))
  (bind _returnvalue (/ Alpha 2.0))
  (bind _returnvalue_2 (* Alpha 0.3))
  (bind _returnvalue_3 (+ _returnvalue 0.5))
  (bind _returnvalue_4 (+ _returnvalue_2 0.7))
  (CallFunction|SetSettings (Utilities|Struct|MakePostProcessSettings (Math|Vector4|MakeVector4 _returnvalue_3 _returnvalue_3 _returnvalue_3 _returnvalue_3) (Math|Vector4|MakeVector4 _returnvalue_4 _returnvalue_4 _returnvalue_4 _returnvalue_4) SceneColor%20%28Optional%29)))

(event Custom|CreateUIMenu
  (Utilities|Time|SetGlobalTimeDilation 0.0)
  (if true
    (CallFunction|RestartLevel)))

(event Custom|DestroyUIMenu
  (Utilities|Time|SetGlobalTimeDilation 1.0))

(event Custom|LHand_Shoulder_Pressed_Event_0
  (params (Key :type Key%20Structure))
  (Utilities|FlowControl|FlipFlop
    (:A
      (CallFunction|Pause:Activate))
    (:B
      (CallFunction|Pause:Deactivate))))

(event Custom|LHand_Shoulder_Pressed_Event_1
  (params (Key :type Key%20Structure))
  (Utilities|FlowControl|FlipFlop
    (:A
      (CallFunction|Pause:Activate))
    (:B
      (CallFunction|Pause:Deactivate))))

(event Custom|RestartLevel
  (bind _returnvalue (Game|GetCurrentLevelName true))
  (Game|OpenLevel(byName) (Utilities|String|StringToName _returnvalue)))

(event Custom|Damage:Activate
  (params (DamageFactor :type Float%20%28single-precision%29))
  (bind _returnvalue (Game|GetPlayerCameraManager 0))
  (bind _returnvalue_2 (* 20 DamageFactor))
  (bind _returnvalue_3 (* DamageFactor 4.0))
  (bind _returnvalue_4 (Math|Float|MakeLiteralFloat _returnvalue_2))
  (bind _returnvalue_5 (Math|Float|Clamp(Float) _returnvalue_3 0.6))
  (bind _returnvalue_6 (Math|Float|MakeLiteralFloat _returnvalue_5))
  (Utilities|FlowControl|DoOnce false
    (:Completed
      (CameraFades|StartCameraFade _returnvalue 0.0 _returnvalue_6 _returnvalue_4 "(R=0.129412,G=0.000000,B=0.000000,A=1.000000)" false true)
      (Utilities|FlowControl|Delay (Math|Float|MakeLiteralFloat 0.1))
      (CameraFades|StartCameraFade _returnvalue _returnvalue_6 0.0 _returnvalue_4 "(R=0.129412,G=0.000000,B=0.000000,A=1.000000)" false false)
      (Utilities|FlowControl|Delay _returnvalue_4))))

(event EventBeginPlay
  (Utilities|FlowControl|Sequence
    (:then_0
      (bind _asbp_vr_pawn (Utilities|Casting|CastToBP_VR_Pawn (Actor|GetParentActor)))
      (bind _output_get (Variables|Default|SetBP_VR_Pawn _asbp_vr_pawn))
      (bind _camera_component (Default|GetCamera _output_get))
      (bind _output_get_2 (Variables|Default|SetPlayerCamera _camera_component))
      (Variables|Default|SetDefaultPPSettings (Variables|/Script/Engine.CameraComponent|GetPostProcessSettings _output_get_2)))
    (:then_1
      (Utilities|FlowControl|Sequence
        (:then_0
          (EventDispatchers|AssignLHandShoulderPressed (Variables|/Game/PlayerController/BP_VR_Pawn.BP_VR_Pawn_C|GetBPAC_Controller (Variables|Default|GetBP_VR_Pawn)) (delegate Custom|LHand_Shoulder_Pressed_Event_0)))
        (:then_1
          (EventDispatchers|AssignLHandShoulderPressed (Variables|/Game/PlayerController/BP_VR_Pawn.BP_VR_Pawn_C|GetBPAC_Controller (Variables|Default|GetBP_VR_Pawn)) (delegate Custom|LHand_Shoulder_Pressed_Event_1)))))))

(event Collision|EventActorBeginOverlap
  (params (OtherActor :type Actor%20Object%20Reference)))

(event EventTick
  (params (DeltaSeconds :type Float%20%28single-precision%29)))

(fn ConstructionScript)

(fn SetSettings
  (params (Settings :type Post%20Process%20Settings%20Structure))
  (Variables|/Script/Engine.CameraComponent|SetPostProcessSettings (Variables|Default|GetPlayerCamera) Settings))

(fn ResetSettings
  (CallFunction|SetSettings (Variables|Default|GetDefaultPPSettings)))