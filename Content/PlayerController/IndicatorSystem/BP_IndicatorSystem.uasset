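; Indicator actor for the VR pawn that shows the spell on each hand as a colored light.
; On BeginPlay it casts its parent actor to BP_VR_Pawn and attaches a left and a right light to the controller's hand target points.
; Per-hand Activate events map the spell (Fireball, Lightning Blade or Shield) to a light color and show that light, while Deactivate events hide it.
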(event Custom|Activate_R_Indicator
  (params (Spell :type Name))
  (switch name Spell
    (:Fireball
      (Variables|Default|SetR_Color "(R=1.000000,G=0.325490,B=0.000000,A=1.000000)"))
    (:LightningBlade
      (Variables|Default|SetR_Color "(R=0.000000,G=0.921569,B=1.000000,A=1.000000)"))
    (:Shield
      (Variables|Default|SetR_Color "(R=1.000000,G=1.000000,B=1.000000,A=1.000000)")))
  (Rendering|Components|Light|SetLightColor (Variables|Default|GetR_Indicator) (Variables|Default|GetR_Color) true)
  (Rendering|SetVisibility (Variables|Default|GetR_Indicator) true false))

(event Custom|Activate_L_Indicator
  (params (Spell :type Name))
  (switch name Spell
    (:Fireball
      (Variables|Default|SetL_Color "(R=1.000000,G=0.325490,B=0.000000,A=1.000000)"))
    (:LightningBlade
      (Variables|Default|SetL_Color "(R=0.000000,G=0.921569,B=1.000000,A=1.000000)"))
    (:Shield
      (Variables|Default|SetL_Color "(R=1.000000,G=1.000000,B=1.000000,A=1.000000)")))
  (Rendering|Components|Light|SetLightColor (Variables|Default|GetL_Indicator) (Variables|Default|GetL_Color) true)
  (Rendering|SetVisibility (Variables|Default|GetL_Indicator) true false))

(event Custom|Deactivate_R_Indicator
  (Rendering|SetVisibility (Variables|Default|GetR_Indicator) false false))

(event Custom|Deactivate_L_Indicator
  (Rendering|SetVisibility (Variables|Default|GetL_Indicator) false false))

(event EventBeginPlay
  (bind _asbp_vr_pawn (Utilities|Casting|CastToBP_VR_Pawn (Actor|GetParentActor)))
  (Variables|Default|SetBP_VR_Pawn _asbp_vr_pawn)
  (Utilities|FlowControl|Sequence
    (:then_0
      (Transformation|AttachComponentToComponent (Variables|Default|GetL_Indicator) (Variables|/Game/PlayerController/ControllerInterfaces/BPAC_Controller.BPAC_Controller_C|GetLeftHandTargetPoint (Variables|/Game/PlayerController/BP_VR_Pawn.BP_VR_Pawn_C|GetBPAC_Controller (Variables|Default|GetBP_VR_Pawn))) "None" "KeepRelative" "KeepRelative" "KeepRelative" true))
    (:then_1
      (Transformation|AttachComponentToComponent (Variables|Default|GetR_Indicator) (Variables|/Game/PlayerController/ControllerInterfaces/BPAC_Controller.BPAC_Controller_C|GetRightHandTargetPoint (Variables|/Game/PlayerController/BP_VR_Pawn.BP_VR_Pawn_C|GetBPAC_Controller (Variables|Default|GetBP_VR_Pawn))) "None" "KeepRelative" "KeepRelative" "KeepRelative" true))))

(event Collision|EventActorBeginOverlap
  (params (OtherActor :type Actor%20Object%20Reference)))

(event EventTick
  (params (DeltaSeconds :type Float%20%28single-precision%29)))

(fn ConstructionScript)