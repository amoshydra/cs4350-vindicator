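; BP_HealthSystem is the player's health actor, spawned as a child actor of BP_VR_Pawn, showing health through an orb at each hand.
; On BeginPlay it attaches both BP_UI_PlayerHP orbs to the pawn's hand target points.
; Heal and damage pass through a gated update that clamps health to 0–100, then pushes the percentage to both orbs.
; At zero health, KillPlayer closes the gate and only prints placeholder death messages.
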(event Custom|KillPlayer
  (CallFunction|PreventHealthfromBeingUpdated)
  (Development|PrintString "You dead")
  (Development|PrintString "Show dead screen / pause menu"))

(event Custom|HealPlayer
  (params (HealthPoints :type Float%20%28single-precision%29))
  (CallFunction|UpdatePlayerHealth HealthPoints))

(event Custom|DamagePlayer
  (params (HealthPoints :type Float%20%28single-precision%29))
  (CallFunction|UpdatePlayerHealth (* -1 HealthPoints)))

(event Custom|_CheckHealthLogic
  (Utilities|FlowControl|Sequence
    (:then_0
      (if (<= (Variables|Default|GetCurrentHealth) 0.0) :!label _label
        (CallFunction|KillPlayer)))
    (:then_1
      (goto _label))
    (:then_3
      (bind _percentage (CallFunction|GetHealthPercentage))
      (Default|UpdateHealthPercentage (Variables|Default|GetLeftHandOrbActor) _percentage)
      (Default|UpdateHealthPercentage (Variables|Default|GetRightHandOrbActor) _percentage))))

(event Custom|_UpdatePlayerHealth
  (params (HealthPoints :type Float%20%28single-precision%29))
  (Utilities|FlowControl|Gate false
    (:Exit
      (Variables|Default|SetCurrentHealth (Math|Float|Clamp(Float) (+ (Variables|Default|GetCurrentHealth) HealthPoints) 0.0 1e+02))
      (CallFunction|CheckHealthLogic))))

(event Custom|_PreventHealthFromBeingUpdated
  (Utilities|FlowControl|Gate false) ; enters at Close
)

(event EventBeginPlay
  (bind _asbp_vr_pawn (Utilities|Casting|CastToBP_VR_Pawn (Actor|GetParentActor)))
  (Variables|Default|SetBP_VR_Pawn _asbp_vr_pawn)
  (Utilities|FlowControl|Sequence
    (:then_0
      (Variables|Default|SetLeftHandOrbActor (.AsBP%20UI%20Player%20HP (Utilities|Casting|CastToBP_UI_PlayerHP (Variables|/Script/Engine.ChildActorComponent|GetChildActor (Variables|Default|GetLeftHandOrb)))))
      (Variables|Default|SetRightHandOrbActor (.AsBP%20UI%20Player%20HP (Utilities|Casting|CastToBP_UI_PlayerHP (Variables|/Script/Engine.ChildActorComponent|GetChildActor (Variables|Default|GetRightHandOrb))))))
    (:then_1
      (Utilities|FlowControl|Sequence
        (:then_0
          (Transformation|AttachComponentToComponent (Variables|Default|GetLeftHandOrb) (Variables|/Game/PlayerController/ControllerInterfaces/BPAC_Controller.BPAC_Controller_C|GetLeftHandTargetPoint (Variables|/Game/PlayerController/BP_VR_Pawn.BP_VR_Pawn_C|GetBPAC_Controller (Variables|Default|GetBP_VR_Pawn))) "None" "KeepRelative" "KeepRelative" "KeepRelative" true))
        (:then_1
          (Transformation|AttachComponentToComponent (Variables|Default|GetRightHandOrb) (Variables|/Game/PlayerController/ControllerInterfaces/BPAC_Controller.BPAC_Controller_C|GetRightHandTargetPoint (Variables|/Game/PlayerController/BP_VR_Pawn.BP_VR_Pawn_C|GetBPAC_Controller (Variables|Default|GetBP_VR_Pawn))) "None" "KeepRelative" "KeepRelative" "KeepRelative" true))))))

(event Collision|EventActorBeginOverlap
  (params (OtherActor :type Actor%20Object%20Reference)))

(event EventTick
  (params (DeltaSeconds :type Float%20%28single-precision%29)))

(fn ConstructionScript
  (bind _orbtohanddistance (Variables|Default|GetOrbToHandDistance))
  (bind _orbscaling (Variables|Default|GetOrbScaling))
  (Utilities|FlowControl|Sequence
    (:then_0
      (Variables|Default|SetCurrentHealth (Variables|Default|GetPlayerMaxHealth)))
    (:then_1
      (Transformation|SetRelativeLocation (Variables|Default|GetLeftHandOrb) (Math|Vector|MakeVector 0.0 (* -1 _orbtohanddistance) 0.0) false false)
      (Transformation|SetRelativeLocation (Variables|Default|GetRightHandOrb) (Math|Vector|MakeVector 0.0 _orbtohanddistance 0.0) false false))
    (:then_2
      (Transformation|SetRelativeScale3D (Variables|Default|GetLeftHandOrb) _orbscaling)
      (Transformation|SetRelativeScale3D (Variables|Default|GetRightHandOrb) _orbscaling))))

(fn GetHealthPercentage
  (return (/ (Variables|Default|GetCurrentHealth) (Variables|Default|GetPlayerMaxHealth))))