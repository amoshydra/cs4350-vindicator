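; Player health display that shows HP as a spinning ring of eight 3D orbs.
; UpdateHealthPercentage stores the health fraction, and Tick rotates the Orbs parent and rescales every orb from that value.
; A nested range chain gives each orb an eighth of health, shrinking them in turn from Orb1 to Orb8.
; BeginPlay fills OrbArray, but the loop that would aim each orb at the center is disconnected.
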(event EventBeginPlay
  (bind _orbarray (Variables|Default|GetOrbArray))
  (Utilities|Array|Add _orbarray (Variables|Default|Getorb1))
  (Utilities|Array|Add _orbarray (Variables|Default|Getorb2))
  (Utilities|Array|Add _orbarray (Variables|Default|Getorb3))
  (Utilities|Array|Add _orbarray (Variables|Default|Getorb4))
  (Utilities|Array|Add _orbarray (Variables|Default|Getorb5))
  (Utilities|Array|Add _orbarray (Variables|Default|Getorb6))
  (Utilities|Array|Add _orbarray (Variables|Default|Getorb7))
  (Utilities|Array|Add _orbarray (Variables|Default|Getorb8)))

(event EventTick
  (params (DeltaSeconds :type Float%20%28single-precision%29))
  (bind _orb1 (Variables|Default|Getorb1))
  (bind _orb3 (Variables|Default|Getorb3))
  (bind _healthpercentage (Variables|Default|GetHealthPercentage))
  (bind _returnvalue (- _healthpercentage 0.875))
  (bind _returnvalue_2 (- _healthpercentage 0.75))
  (bind _returnvalue_3 (- _healthpercentage 0.625))
  (bind _returnvalue_4 (- _healthpercentage 0.5))
  (bind _returnvalue_5 (- _healthpercentage 0.375))
  (bind _returnvalue_6 (- _healthpercentage 0.25))
  (bind _returnvalue_7 (- _healthpercentage 0.125))
  (bind _returnvalue_8 (/ _healthpercentage 0.125))
  (bind _returnvalue_9 (/ _returnvalue 0.125))
  (bind _returnvalue_10 (/ _returnvalue_7 0.125))
  (bind _returnvalue_11 (/ _returnvalue_2 0.125))
  (bind _returnvalue_12 (/ _returnvalue_3 0.125))
  (bind _returnvalue_13 (/ _returnvalue_4 0.125))
  (bind _returnvalue_14 (/ _returnvalue_5 0.125))
  (bind _returnvalue_15 (/ _returnvalue_6 0.125))
  (Transformation|AddRelativeRotation (Variables|Default|Getorbs) (Math|Rotator|MakeRotator (* DeltaSeconds 9e+01) 0.0 0.0) false false)
  (if (Math|Float|InRange(Float) _healthpercentage 0.875 1.0 false)
    (Transformation|SetRelativeScale3D (Variables|Default|Getorb1) (Math|Vector|MakeVector _returnvalue_9 _returnvalue_9 _returnvalue_9))
    (Transformation|SetRelativeScale3D _orb3 "1.000000,1.000000,1.000000")
    (elif (Math|Float|InRange(Float) _healthpercentage 0.75 0.875 false)
      (Transformation|SetRelativeScale3D (Variables|Default|Getorb2) (Math|Vector|MakeVector _returnvalue_11 _returnvalue_11 _returnvalue_11))
      (Transformation|SetRelativeScale3D _orb3 "1.000000,1.000000,1.000000")
      (Transformation|SetRelativeScale3D _orb1 "0, 0, 0")
      (elif (Math|Float|InRange(Float) _healthpercentage 0.625 0.75 false)
        (Transformation|SetRelativeScale3D (Variables|Default|Getorb3) (Math|Vector|MakeVector _returnvalue_12 _returnvalue_12 _returnvalue_12))
        (Transformation|SetRelativeScale3D (Variables|Default|Getorb4) "1.000000,1.000000,1.000000")
        (Transformation|SetRelativeScale3D _orb1 "0, 0, 0")
        (elif (Math|Float|InRange(Float) _healthpercentage 0.5 0.625 false)
          (Transformation|SetRelativeScale3D (Variables|Default|Getorb4) (Math|Vector|MakeVector _returnvalue_13 _returnvalue_13 _returnvalue_13))
          (Transformation|SetRelativeScale3D (Variables|Default|Getorb5) "1.000000,1.000000,1.000000")
          (Transformation|SetRelativeScale3D _orb1 "0, 0, 0")
          (elif (Math|Float|InRange(Float) _healthpercentage 0.375 0.5 false)
            (Transformation|SetRelativeScale3D (Variables|Default|Getorb5) (Math|Vector|MakeVector _returnvalue_14 _returnvalue_14 _returnvalue_14))
            (Transformation|SetRelativeScale3D (Variables|Default|Getorb6) "1.000000,1.000000,1.000000")
            (Transformation|SetRelativeScale3D _orb1 "0, 0, 0")
            (elif (Math|Float|InRange(Float) _healthpercentage 0.25 0.375 false)
              (Transformation|SetRelativeScale3D (Variables|Default|Getorb6) (Math|Vector|MakeVector _returnvalue_15 _returnvalue_15 _returnvalue_15))
              (Transformation|SetRelativeScale3D (Variables|Default|Getorb7) "1.000000,1.000000,1.000000")
              (Transformation|SetRelativeScale3D _orb1 "0, 0, 0")
              (elif (Math|Float|InRange(Float) _healthpercentage 0.125 0.25 false)
                (Transformation|SetRelativeScale3D (Variables|Default|Getorb7) (Math|Vector|MakeVector _returnvalue_10 _returnvalue_10 _returnvalue_10))
                (Transformation|SetRelativeScale3D (Variables|Default|Getorb8) "1.000000,1.000000,1.000000")
                (Transformation|SetRelativeScale3D _orb1 "0, 0, 0")
                (else
                  (Transformation|SetRelativeScale3D (Variables|Default|Getorb8) (Math|Vector|MakeVector _returnvalue_8 _returnvalue_8 _returnvalue_8))
                  (Transformation|SetRelativeScale3D _orb1 "0, 0, 0"))))))))))

(fn ConstructionScript)

(fn UpdateHealthPercentage
  (params (HealthPercentage :type Float%20%28single-precision%29))
  (Variables|Default|SetHealthPercentage HealthPercentage))