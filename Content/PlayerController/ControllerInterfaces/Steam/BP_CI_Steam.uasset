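; BP_CI_Steam is the Steam controller interface, translating VR motion controller input into hand-specific interface calls.
; It enables input from player 0 on BeginPlay, then forwards triggers, grips, thumbsticks, shoulders and face buttons to CallInterface functions.
; Face buttons route to the opposite hand, with some left-controller press and release events mapped to different button numbers.
; GetLeftHand and GetRightHand expose each hand's mesh and motion controller.
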(event EventBeginPlay
  (Input|EnableInput (Game|GetPlayerController 0)))

(event Input|KeyboardEvents|MotionControllerLeftThumbstickX
  (params (AxisValue :type Float%20%28single-precision%29))
  (Default|CallInterfaceLHandThumbstickX AxisValue))

(event Input|KeyboardEvents|MotionControllerLeftThumbstickY
  (params (AxisValue :type Float%20%28single-precision%29))
  (Default|CallInterfaceLHandThumbstickY AxisValue))

(event Input|KeyboardEvents|MotionControllerRightTriggerAxis
  (params (AxisValue :type Float%20%28single-precision%29))
  (Default|CallInterfaceRHandTriggerAxis AxisValue))

(event Input|KeyboardEvents|MotionControllerLeftTriggerAxis
  (params (AxisValue :type Float%20%28single-precision%29))
  (Default|CallInterfaceLHandTriggerAxis AxisValue))

(event Input|KeyboardEvents|MotionControllerRightThumbstickX
  (params (AxisValue :type Float%20%28single-precision%29))
  (Default|CallInterfaceRHandThumbstickX AxisValue))

(event Input|KeyboardEvents|MotionControllerRightThumbstickY
  (params (AxisValue :type Float%20%28single-precision%29))
  (Default|CallInterfaceRHandThumbstickY AxisValue))

(event Input|KeyboardEvents|MotionControllerRightTrigger
  (params (Key :type Key%20Structure))
  (:Pressed
    (Default|CallInterfaceRHandTriggerPressed))
  (:Released
    (Default|CallInterfaceRHandTriggerReleased)))

(event Input|KeyboardEvents|MotionControllerRightFaceButton1
  (params (Key :type Key%20Structure))
  (:Pressed
    (Default|CallInterfaceLHandFaceButton1Pressed Key))
  (:Released
    (Default|CallInterfaceLHandFaceButton1Released Key)))

(event Input|KeyboardEvents|MotionControllerLeftShoulder
  (params (Key :type Key%20Structure))
  (:Pressed
    (Default|CallInterfaceLHandShoulderPressed Key))
  (:Released
    (Default|CallInterfaceLHandShoulderReleased Key)))

(event Input|KeyboardEvents|MotionControllerRightShoulder
  (params (Key :type Key%20Structure))
  (:Pressed
    (Default|CallInterfaceRHandShoulderPressed Key))
  (:Released
    (Default|CallInterfaceRHandShoulderReleased Key)))

(event Input|KeyboardEvents|MotionControllerLeftTrigger
  (params (Key :type Key%20Structure))
  (:Pressed
    (Default|CallInterfaceLHandTriggerPressed))
  (:Released
    (Default|CallInterfaceLHandTriggerReleased)))

(event Input|KeyboardEvents|MotionControllerLeftFaceButton1
  (params (Key :type Key%20Structure))
  (:Pressed
    (Default|CallInterfaceRHandFaceButton1Pressed Key))
  (:Released
    (Default|CallInterfaceRHandFaceButton1Released Key)))

(event Input|KeyboardEvents|MotionControllerLeftFaceButton2
  (params (Key :type Key%20Structure))
  (:Pressed
    (Default|CallInterfaceRHandFaceButton3Pressed Key))
  (:Released
    (Default|CallInterfaceRHandFaceButton2Released Key)))

(event Input|KeyboardEvents|MotionControllerRightFaceButton2
  (params (Key :type Key%20Structure))
  (:Pressed
    (Default|CallInterfaceLHandFaceButton2Pressed Key))
  (:Released
    (Default|CallInterfaceLHandFaceButton2Released Key)))

(event Input|KeyboardEvents|MotionControllerLeftFaceButton4
  (params (Key :type Key%20Structure))
  (:Pressed
    (Default|CallInterfaceRHandFaceButton2Pressed Key))
  (:Released
    (Default|CallInterfaceRHandFaceButton3Released Key)))

(event Input|KeyboardEvents|MotionControllerLeftFaceButton3
  (params (Key :type Key%20Structure))
  (:Pressed
    (Default|CallInterfaceRHandFaceButton4Pressed Key))
  (:Released
    (Default|CallInterfaceRHandFaceButton4Released Key)))

(event Input|KeyboardEvents|MotionControllerRightFaceButton4
  (params (Key :type Key%20Structure))
  (:Pressed
    (Default|CallInterfaceLHandFaceButton4Pressed Key))
  (:Released
    (Default|CallInterfaceLHandFaceButton4Released Key)))

(event Input|KeyboardEvents|MotionControllerRightGrip1
  (params (Key :type Key%20Structure))
  (:Pressed
    (Default|CallInterfaceRHandGripPressed))
  (:Released
    (Default|CallInterfaceRHandGripReleased)))

(event Input|KeyboardEvents|MotionControllerLeftGrip1
  (params (Key :type Key%20Structure))
  (:Pressed
    (Default|CallInterfaceLHandGripPressed))
  (:Released
    (Default|CallInterfaceLHandGripReleased)))

(event Input|KeyboardEvents|MotionControllerRightFaceButton3
  (params (Key :type Key%20Structure))
  (:Pressed
    (Default|CallInterfaceLHandFaceButton3Pressed Key))
  (:Released
    (Default|CallInterfaceLHandFaceButton3Released Key)))

(fn ConstructionScript)

(fn GetLeftHand
  (return (Variables|Default|GetL_Hand) (Variables|Default|GetL_MotionController) 0))

(fn GetRightHand
  (return (Variables|Default|GetR_Hand) (Variables|Default|GetR_MotionController) 0))