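; Leap Motion controller interface that turns hand gestures into the player's motion-controller style inputs.
; On BeginPlay it adds a Leap controller and optimizes it for HMD, using top-down tracking only when a headset is detected.
; Grab and release events map to trigger calls and pinch and unpinch to grip calls, split by hand.
; Getter functions expose each hand's mesh and target point.
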(event EventBeginPlay
  (|CallParentFunction)
  (bind _returnvalue (AddComponent|AddLeapController))
  (Class|LeapController|OptimizeforHMD _returnvalue (Utilities|Name|NotEqual(Name) (Class|HeadMountedDisplayFunctionLibrary|GetHMDDeviceName) "None") true true))

(event Collision|EventActorBeginOverlap
  (params (OtherActor :type Actor%20Object%20Reference))
  (|CallParentFunction OtherActor))

(event EventLeapHandReleased
  (params (strength :type Float%20%28single-precision%29) (hand :type Leap%20Hand%20Object%20Reference))
  (switch Utilities|FlowControl|Switch|SwitchonLeapHandType (Variables|/Script/LeapMotion.LeapHand|GetHandType hand)
    (:HAND_LEFT
      (Default|CallInterfaceLHandTriggerReleased))
    (:HAND_RIGHT
      (Default|CallInterfaceRHandTriggerReleased))))

(event EventLeapHandPinched
  (params (strength :type Float%20%28single-precision%29) (hand :type Leap%20Hand%20Object%20Reference))
  (switch Utilities|FlowControl|Switch|SwitchonLeapHandType (Variables|/Script/LeapMotion.LeapHand|GetHandType hand)
    (:HAND_LEFT
      (Default|CallInterfaceLHandGripPressed))
    (:HAND_RIGHT
      (Default|CallInterfaceRHandGripPressed))))

(event EventLeapHandUnpinched
  (params (strength :type Float%20%28single-precision%29) (hand :type Leap%20Hand%20Object%20Reference))
  (switch Utilities|FlowControl|Switch|SwitchonLeapHandType (Variables|/Script/LeapMotion.LeapHand|GetHandType hand)
    (:HAND_LEFT
      (Default|CallInterfaceLHandGripReleased))
    (:HAND_RIGHT
      (Default|CallInterfaceRHandGripReleased))))

(event EventLeapHandGrabbed
  (params (strength :type Float%20%28single-precision%29) (hand :type Leap%20Hand%20Object%20Reference))
  (switch Utilities|FlowControl|Switch|SwitchonLeapHandType (Variables|/Script/LeapMotion.LeapHand|GetHandType hand)
    (:HAND_LEFT
      (Default|CallInterfaceLHandTriggerPressed))
    (:HAND_RIGHT
      (Default|CallInterfaceRHandTriggerPressed))))

(fn ConstructionScript
  (|CallParentFunction))

(fn GetLeftHand
  (bind _lefthandmesh (Variables|Default|GetLeftHandMesh))
  (return _lefthandmesh _lefthandmesh (Variables|Default|GetL_Hand_TargetPoint)))

(fn GetRightHand
  (bind _righthandmesh (Variables|Default|GetRightHandMesh))
  (return _righthandmesh _righthandmesh (Variables|Default|GetR_Hand_TargetPoint)))