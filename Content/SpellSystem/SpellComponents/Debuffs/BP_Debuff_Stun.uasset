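; BP_Debuff_Stun is a spell-system debuff component that stuns an enemy by changing its speed while active.
; On Activate it attaches a lightning particle emitter to the owner's root component and passes StunSpeedFactor to SetSpeed on the owning BP_Enemy_Base.
; On Deactivate it stops the emitter and resets the speed to 1.0.
; Non-enemy owners receive only the visual effect, as the speed change depends on the cast.
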(event EventBeginPlay
  (|CallParentFunction))

(event Collision|EventActorBeginOverlap
  (params (OtherActor :type Actor%20Object%20Reference))
  (|CallParentFunction OtherActor))

(event EventDeactivate
  (bind _particlesystem (Variables|Default|GetParticleSystem))
  (|CallParentFunction)
  (Utilities|FlowControl|Sequence
    (:then_0
      ;[1 1 1] Stop Particle Effect
      (if (not (Class|ActorComponent|IsBeingDestroyed _particlesystem))
        (Components|Activation|Deactivate _particlesystem)))
    (:then_1
      ;[1 1 1] Unstun Enemy
      (bind _asbp_enemy_base (Utilities|Casting|CastToBP_Enemy_Base (Components|GetOwner)))
      (Default|SetSpeed _asbp_enemy_base 1.0))))

(event EventTick
  (params (DeltaSeconds :type Float%20%28single-precision%29))
  (|CallParentFunction DeltaSeconds))

(event EventActivate
  (|CallParentFunction)
  (Utilities|FlowControl|Sequence
    (:then_0
      ;[1 1 1] Spawn Particle Effect
      (bind _returnvalue (Effects|SpawnEmitterAttached "/Game/Assets/InfinityBladeEffects/Effects/FX_Combat_Lightning/P_DOT_Lightning_01.P_DOT_Lightning_01" (Variables|/Script/Engine.Actor|GetRootComponent (Components|GetOwner)) "None" "0,0.000000, 0"))
      (Variables|Default|SetParticleSystem _returnvalue))
    (:then_1
      ;[1 1 1] Stun Enemy
      (bind _asbp_enemy_base (Utilities|Casting|CastToBP_Enemy_Base (Components|GetOwner)))
      (Default|SetSpeed _asbp_enemy_base (Variables|Default|GetStunSpeedFactor)))))

(fn ConstructionScript
  (|CallParentFunction))