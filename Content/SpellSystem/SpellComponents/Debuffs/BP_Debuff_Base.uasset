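; BP_Debuff_Base is the spell system's base debuff, providing a timed active state with no gameplay effect of its own.
; Activate sets the active flag, resets the lifespan to its default and starts a looping one-second timer, first deactivating any run already in progress.
; Each tick of that timer decrements the remaining lifespan and calls Deactivate at zero, which clears the flag and timer.
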(event EventBeginPlay)

(event Collision|EventActorBeginOverlap
  (params (OtherActor :type Actor%20Object%20Reference)))

(event EventTick
  (params (DeltaSeconds :type Float%20%28single-precision%29)))

(fn ConstructionScript)

(fn Deactivate
  (Utilities|FlowControl|Sequence
    (:then_0
      ;[1 1 1] Manage Deactivation Status
      (Variables|Default|SetisActivated false))
    (:then_1
      ;[1 1 1] Manage Lifespan Counter
      (Utilities|Time|ClearandInvalidateTimerbyHandle (Variables|Default|GetLifespanTimer)))))

(fn Activate
  (Utilities|FlowControl|Sequence
    (:then_0
      ;[1 1 1] Manage Activation Status
      (if (Variables|Default|GetisActivated)
        (CallFunction|Deactivate))
      (Variables|Default|SetisActivated true))
    (:then_1
      ;[1 1 1] Manage Lifespan Counter
      (Variables|Default|SetCurrentLifespan (Variables|Default|GetDefaultLifespan))
      (bind _returnvalue (Utilities|Time|SetTimerbyFunctionName 0 "UpdateLifeSpan" 1.0 true))
      (Variables|Default|SetLifespanTimer _returnvalue))))

(fn UpdateLifeSpan
  (Utilities|FlowControl|Sequence
    (:then_0
      ;[1 1 1] Decrease Lifespan
      (Variables|Default|SetCurrentLifespan (- (Variables|Default|GetCurrentLifespan) 1.0)))
    (:then_1
      ;[1 1 1] Validate Lifespan
      (if (<= (Variables|Default|GetCurrentLifespan) 0.0)
        (CallFunction|Deactivate)))))