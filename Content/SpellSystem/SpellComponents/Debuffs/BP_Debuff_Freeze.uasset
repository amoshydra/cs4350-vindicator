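; Freeze debuff in the spell system that slows and visually freezes the enemy that owns it.
; On activation it attaches an ice particle at the capsule's base, applies the freeze speed factor and pauses mesh animation.
; On deactivation it destroys the particle, resumes animation and uses a timeline to ease speed back to normal, stopping that recovery if the freeze is reapplied.
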(event EventBeginPlay
  (|CallParentFunction))

(event Collision|EventActorBeginOverlap
  (params (OtherActor :type Actor%20Object%20Reference))
  (|CallParentFunction OtherActor))

(event EventTick
  (params (DeltaSeconds :type Float%20%28single-precision%29))
  (|CallParentFunction DeltaSeconds))

(event EventActivate
  (|CallParentFunction)
  (Utilities|FlowControl|Sequence
    (:then_0
      (Variables|Default|SetisFreezing true))
    (:then_1
      ;[1 1 1] Spawn Particle Effect
      (bind _asbp_enemy_base (Utilities|Casting|CastToBP_Enemy_Base (Components|GetOwner)))
      (bind _returnvalue (Effects|SpawnEmitterAttached "/Game/SpellSystem/SpellComponents/Debuffs/CustomAssets/P_levelUp_IceHold.P_levelUp_IceHold" (Variables|/Script/Engine.Actor|GetRootComponent _asbp_enemy_base) "" (Math|Vector|MakeVector 0.0 0.0 (* (Components|Capsule|GetScaledCapsuleHalfHeight (Variables|/Script/Engine.Character|GetCapsuleComponent _asbp_enemy_base)) -1.0)) "0, 0, 0" "KeepRelativeOffset" false))
      (bind _output_get (Variables|Default|SetParticle%20System _returnvalue))
      (Transformation|SetRelativeScale3D _output_get "0.500000,0.500000,0.500000"))
    (:then_2
      ;[1 1 1] Freeze Enemy
      (bind _asbp_enemy_base_2 (Utilities|Casting|CastToBP_Enemy_Base (Components|GetOwner)))
      (Default|SetSpeedFactor _asbp_enemy_base_2 (Variables|Default|GetFreezeSpeedFactor))
      (Variables|/Script/Engine.SkeletalMeshComponent|SetbPauseAnims (Variables|/Script/Engine.Character|GetMesh _asbp_enemy_base_2) true))))

(event EventDeactivate
  (bind _particle_system (Variables|Default|GetParticle%20System))
  (|CallParentFunction)
  (Utilities|FlowControl|Sequence
    (:then_0
      (Variables|Default|SetisFreezing false))
    (:then_1
      ;[1 1 1] Stop Particle Effect
      (if (Utilities|IsValid _particle_system)
        (Components|DestroyComponent _particle_system)))
    (:then_2
      ;[1 1 1] Unfreeze Enemy
      (bind _asbp_enemy_base (Utilities|Casting|CastToBP_Enemy_Base (Components|GetOwner)))
      (Variables|/Script/Engine.SkeletalMeshComponent|SetbPauseAnims (Variables|/Script/Engine.Character|GetMesh _asbp_enemy_base) false)
      (bind _rate (Timeline|Timeline_0 PlayFromStart)
        (:Update
          (if (not (Variables|Default|GetisFreezing))
            (Default|SetSpeedFactor _asbp_enemy_base (Math|Float|Lerp (Variables|Default|GetFreezeSpeedFactor) 1.0 _rate))
            (else
              (Timeline|Timeline_0 Stop))))))))

(fn ConstructionScript
  (|CallParentFunction))