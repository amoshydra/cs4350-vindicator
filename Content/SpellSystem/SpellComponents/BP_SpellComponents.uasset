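; BP_SpellComponents is a spell system Blueprint whose ConeSearch function picks out the enemies that fall inside a cone.
; It measures the angle between a forward vector and the direction from a given location to each supplied enemy, using the dot product and arccosine.
; Enemies within a hard-coded 30-degree half-angle are returned as an array, with no distance limit applied.
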(fn ConeSearch
  (params (Location :type Vector) (Forward%20Vector :type Vector) (AllEnemies :type Array%20of%20BP%20Enemy%20Base%20Object%20References))
  (bind _array (Utilities|Array|MakeArray 0))
  (for _array_element AllEnemies
    (if (<= (Math|Float|Absolute(Float) (Class|KismetMathLibrary|DegAcos (/ (Math|Vector|DotProduct (- (Transformation|GetActorLocation _array_element) Location) Forward%20Vector) (* (Math|Vector|VectorLength (- (Transformation|GetActorLocation _array_element) Location)) (Math|Vector|VectorLength Forward%20Vector))))) 3e+01)
      (Utilities|Array|Add _array _array_element)))
  (return _array))