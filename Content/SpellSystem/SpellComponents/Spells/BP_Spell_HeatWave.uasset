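; BP_Spell_HeatWave is a spell actor for a heat wave that drives a Spray component over the spell's lifetime.
; The Create event activates Spray, and Cast deactivates it and immediately destroys the actor.
; Destroy is an empty event, and a two-second delayed Cast is left unconnected, so nothing in this graph ends the spell on a timer.
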(event EventBeginPlay
  (|CallParentFunction))

(event Collision|EventActorBeginOverlap
  (params (OtherActor :type Actor%20Object%20Reference))
  (|CallParentFunction OtherActor))

(event EventTick
  (params (DeltaSeconds :type Float%20%28single-precision%29))
  (|CallParentFunction DeltaSeconds))

(event EventDestroy)

(event EventCast
  (Components|Activation|Deactivate (Variables|Default|Getspray))
  (Actor|DestroyActor))

(event EventCreate
  (Components|Activation|Activate (Variables|Default|Getspray) false))

(fn ConstructionScript
  (|CallParentFunction))