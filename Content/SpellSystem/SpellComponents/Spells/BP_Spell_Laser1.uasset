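; Laser beam spell actor that damages enemies along its forward line and expires after a few seconds or when Cast is called.
; Each tick a Visibility trace stretches the beam mesh to the impact and places the Hit effect there, shrinking it at close range.
; Enemies hit take Inflict every tick, switching to a fixed alternate damage once the same target has been held for two seconds.
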(event EventBeginPlay
  (|CallParentFunction)
  (Actor|SetLifeSpan 6.0))

(event Collision|EventActorBeginOverlap
  (params (OtherActor :type Actor%20Object%20Reference))
  (|CallParentFunction OtherActor))

(event EventTick
  (params (DeltaSeconds :type Float%20%28single-precision%29))
  (bind _returnvalue (Transformation|GetActorLocation))
  (bind _staticmesh (Variables|Default|GetStaticMesh))
  (bind _hit (Variables|Default|GetHit))
  (bind _hit_2 (Variables|Default|GetHit))
  (|CallParentFunction DeltaSeconds)
  (bind (_outhit _returnvalue_2) (Collision|LineTraceByChannel _returnvalue (+ _returnvalue (* (Math|Vector|GetForwardVector (Variables|Default|GetDefaultSceneRoot)) 1e+05)) "TraceTypeQuery1" false 0 "None"))
  (if _returnvalue_2
    (Components|Activation|Activate _hit_2 false)
    (Transformation|SetRelativeScale3D _staticmesh (Math|Vector|MakeVector 0.05 0.05 (/ (Math|Vector|VectorLength (- (.location _outhit) (Transformation|GetActorLocation))) 25.0)))
    (Transformation|SetWorldLocation _hit (.location _outhit) false false)
    (if (<= (Math|Vector|VectorLength (- (.location _outhit) (Transformation|GetActorLocation))) 5e+02)
      (Transformation|SetRelativeScale3D _hit (Math|Vector|MakeVector (Math|Float|Max(Float) (/ (Math|Vector|VectorLength (- (.location _outhit) (Transformation|GetActorLocation))) 5e+02) 0.4) (Math|Float|Max(Float) (/ (Math|Vector|VectorLength (- (.location _outhit) (Transformation|GetActorLocation))) 5e+02) 0.4) (Math|Float|Max(Float) (/ (Math|Vector|VectorLength (- (.location _outhit) (Transformation|GetActorLocation))) 5e+02) 0.4)))
      (else
        (Transformation|SetRelativeScale3D _hit "1.000000,1.000000,1.000000")))
    (bind _asbp_enemy_base (Utilities|Casting|CastToBP_Enemy_Base (.hitactor _outhit)))
    (bind _targetedenemy (Variables|Default|GetTargetedEnemy)
      (:then
        (if (== _targetedenemy _asbp_enemy_base)
          (if (>= (Actor|GetGameTimeSinceCreation) (Variables|Default|GetChargeTime))
            (CallFunction|Inflict _asbp_enemy_base true 0.1)
            (else
              (CallFunction|Inflict _asbp_enemy_base false 0.0 :!label _label)))
          (else
            (Variables|Default|SetTargetedEnemy _asbp_enemy_base :!label _label_2)
            (Variables|Default|SetChargeTime (+ (Actor|GetGameTimeSinceCreation) 2.0))
            (goto _label))))
      (:else
        (goto _label_2)))
    (else
      (Components|Activation|Deactivate _hit_2)
      (Transformation|SetRelativeScale3D _staticmesh (Math|Vector|MakeVector 0.05 0.05 1e+03)))))

(event EventCast
  (Actor|DestroyActor))

(event EventCreate)

(fn ConstructionScript
  (|CallParentFunction))