(event EventBeginPlay
  (|CallParentFunction))

(event Collision|EventActorBeginOverlap
  (params (OtherActor :type Actor%20Object%20Reference))
  (|CallParentFunction OtherActor))

(event EventTick
  (params (DeltaSeconds :type Float%20%28single-precision%29))
  (|CallParentFunction DeltaSeconds))

(event EventCreate
  (Audio|PlaySound2D "/Engine/VREditor/Sounds/VR_click1_Cue.VR_click1_Cue")
  (if (Variables|Default|GetshouldGrow)
    (bind _chargefactor (Timeline|ChargingAnimationTimeline Play)
      (:Update
        (Transformation|SetRelativeScale3D (Variables|Default|GetStaticMesh) (Math|Vector|Lerp(Vector) (Variables|Default|GetScaleBeginning) (Variables|Default|GetScaleEnd) _chargefactor))))))

(event EventDestroy
  (if (Variables|Default|GetshouldGrow)
    (bind _chargefactor (Timeline|DechargingAnimationTimeline Play)
      (:Update
        (Transformation|SetRelativeScale3D (Variables|Default|GetStaticMesh) (Math|Vector|Lerp(Vector) (Variables|Default|GetScaleEnd) (Variables|Default|GetScaleBeginning) _chargefactor)))
      (:Finished
        (Actor|DestroyActor :!label _label)))
    (else
      (goto _label))))

(fn ConstructionScript
  (|CallParentFunction)
  (Variables|Default|SetScaleEnd (Variables|/Script/Engine.SceneComponent|GetRelativeScale3D (Variables|Default|GetStaticMesh)))
  (if (Variables|Default|GetshouldGrow)
    (Transformation|SetRelativeScale3D (Variables|Default|GetStaticMesh) (Variables|Default|GetScaleBeginning))
    (else
      (Transformation|SetRelativeScale3D (Variables|Default|GetStaticMesh) (Variables|Default|GetScaleEnd)))))