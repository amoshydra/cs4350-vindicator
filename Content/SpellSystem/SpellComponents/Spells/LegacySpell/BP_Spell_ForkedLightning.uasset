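; Legacy forked lightning spell that stuns enemies in a cone in front of it, with no damage in the live path.
; On Create it swaps the initial shock visuals for an aftershock, detaches, and fans lightning emitters across the Degrees arc.
; A ConeSearch over the GameInstance's enemy list, filtered by Distance, applies the stun debuff and hit effects.
; Effects deactivate after a short delay; Cast is empty and older per-target code sits unconnected.
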(event EventBeginPlay
  (|CallParentFunction))

(event Collision|EventActorBeginOverlap
  (params (OtherActor :type Actor%20Object%20Reference))
  (|CallParentFunction OtherActor))

(event EventTick
  (params (DeltaSeconds :type Float%20%28single-precision%29))
  (|CallParentFunction DeltaSeconds))

(event EventCreate
  ;[1 1 1] Animation
  (Components|Activation|Deactivate (Variables|Default|GetInitialShock))
  (Rendering|SetVisibility (Variables|Default|GetStaticMesh) false false)
  (Components|Activation|Activate (Variables|Default|GetAfterShock) false)
  (Utilities|FlowControl|Delay 0.2)
  (Transformation|DetachFromActor "KeepWorld" "KeepWorld" "KeepWorld")
  (for _index (range 0 (* (/ (Variables|Default|GetDegrees) 10) 2))
    (bind _returnvalue (Effects|SpawnEmitteratLocation "/Game/Assets/InfinityBladeEffects/Effects/FX_Monsters/FX_Monster_Genno/P_Genno_Weapon_Lightning_01.P_Genno_Weapon_Lightning_01" (Transformation|GetActorLocation) (Math|Rotator|MakeRotator 0.0 -9e+01 (+ (Math|Conversions|ToFloat(Integer) (+ (* _index 10) (* (Variables|Default|GetDegrees) -1))) (.yaw (Transformation|GetActorRotation))))))
    (Transformation|SetRelativeScale3D _returnvalue "1.000000,3.000000,3.000000")
    (Transformation|AddLocalOffset _returnvalue "0.000000,0.000000,80.000000" false false)
    (Utilities|Array|Add (Variables|Default|GetParticles) _returnvalue))
  ;[1 1 1] Apply Debuff to Enemies
  (bind _asbp_game_instance (Utilities|Casting|CastToBP_GameInstance (Game|GetGameInstance)))
  (bind _enemies (CallFunction|ConeSearch (Transformation|GetActorLocation) (Transformation|GetActorForwardVector) (Variables|/Game/Blueprints/BP_GameInstance.BP_GameInstance_C|GetEnemies _asbp_game_instance) (Variables|Default|GetDegrees)))
  (for _array_element _enemies
    (if (<= (Transformation|GetDistanceTo _array_element) (Variables|Default|GetDistance))
      (Default|ActivateDebuff (Variables|/Game/AI/BP_Enemy_Base.BP_Enemy_Base_C|GetBP_Debuff_Manager _array_element) "/Game/SpellSystem/SpellComponents/Debuffs/BP_Debuff_Stun.BP_Debuff_Stun_C")
      (Effects|SpawnEmitteratLocation "/Game/Assets/InfinityBladeEffects/Effects/FX_Mobile/Lightning/P_LineToPoint_Spawn_Proj_Lightning_00.P_LineToPoint_Spawn_Proj_Lightning_00" (Transformation|GetActorLocation _array_element))))
  ;[1 1 1] Deactivate Particle Effects After X seconds
  (Utilities|FlowControl|Delay 1.0)
  (for _array_element_2 (Variables|Default|GetParticles)
    (Components|Activation|Deactivate _array_element_2))
  (Components|Activation|Deactivate (Variables|Default|GetAfterShock)))

(event EventCast)

(fn ConstructionScript
  (|CallParentFunction))