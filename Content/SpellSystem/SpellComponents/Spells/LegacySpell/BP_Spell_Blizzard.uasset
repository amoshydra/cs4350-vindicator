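; Legacy Blizzard spell actor that rains ice shards over an area in front of it and freezes enemies entering its box.
; On BeginPlay it scatters random scene-component spawn points, starts Aura and Snow effects, and spawns shards above those points on a looping timer.
; Box overlaps inflict zero alternate damage, apply the Freeze debuff and record enemies.
; After a timed duration, effects deactivate; on finishing, the actor destroys itself and clears those debuffs.
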(event OnComponentBeginOverlap(Box)
  (params (OverlappedComponent :type Primitive%20Component%20Object%20Reference) (OtherActor :type Actor%20Object%20Reference) (OtherComp :type Primitive%20Component%20Object%20Reference) (OtherBodyIndex :type Integer) (bFromSweep :type Boolean) (SweepResult :type Hit%20Result%20Structure%20%28by%20ref%29))
  (bind _asbp_enemy_base (Utilities|Casting|CastToBP_Enemy_Base OtherActor))
  (CallFunction|Inflict _asbp_enemy_base true 0.0)
  (Default|ActivateDebuff (Variables|/Game/AI/BP_Enemy_Base.BP_Enemy_Base_C|GetBP_Debuff_Manager _asbp_enemy_base) "/Game/SpellSystem/SpellComponents/Debuffs/BP_Debuff_Freeze.BP_Debuff_Freeze_C")
  (Utilities|Array|Add (Variables|Default|GetEnemiesHit) _asbp_enemy_base))

(event Custom|Spawn%20Projectile
  (bind _spawnpoints (Variables|Default|GetSpawnPoints))
  (bind _returnvalue (Utilities|Array|Length _spawnpoints))
  (bind _returnvalue_2 (- _returnvalue 1))
  (bind _returnvalue_3 (Math|Random|RandomIntegerinRange 0 _returnvalue_2))
  (bind _output (Utilities|Array|Get(acopy) _spawnpoints _returnvalue_3))
  (bind _returnvalue_4 (Transformation|GetWorldLocation _output))
  (if (Variables|Default|GetisActivated)
    (Game|SpawnActorfromClass "/Game/SpellSystem/SpellComponents/Spells/LegacySpell/BP_SpellComponent_Shard.BP_SpellComponent_Shard_C" (Math|Transform|MakeTransform (Math|Vector|MakeVector (.x _returnvalue_4) (.y _returnvalue_4) (+ (.z _returnvalue_4) 1.2e+03)) "0, 0, 0" "1,1,1") "Undefined" 0 0)))

(event Custom|OnSystemFinished_Event_0
  (params (PSystem :type Particle%20System%20Component%20Object%20Reference))
  (Actor|DestroyActor)
  (for _array_element (Variables|Default|GetEnemiesHit)
    (Default|DeactivateDebuff (Variables|/Game/AI/BP_Enemy_Base.BP_Enemy_Base_C|GetBP_Debuff_Manager _array_element) "/Game/SpellSystem/SpellComponents/Debuffs/BP_Debuff_Freeze.BP_Debuff_Freeze_C")))

(event Custom|Set%20Death
  (bind _aura (Variables|Default|GetAura))
  (Variables|Default|SetisActivated false)
  (Utilities|FlowControl|Delay 1.0)
  (EventDispatchers|AssignOnSystemFinished _aura (delegate Custom|OnSystemFinished_Event_0))
  (Components|Activation|Deactivate _aura))

(event EventBeginPlay
  (|CallParentFunction)
  (CallFunction|Create)
  (CallFunction|Cast))

(event Collision|EventActorBeginOverlap
  (params (OtherActor :type Actor%20Object%20Reference))
  (|CallParentFunction OtherActor))

(event EventTick
  (params (DeltaSeconds :type Float%20%28single-precision%29))
  (|CallParentFunction DeltaSeconds))

(event EventCast
  (Variables|Default|SetisActivated true)
  (Components|Activation|Activate (Variables|Default|GetAura) false)
  (Utilities|Time|SetTimerbyEvent (delegate Custom|Set%20Death) 6.0)
  (Utilities|Time|SetTimerbyEvent (delegate Custom|Spawn%20Projectile) 0.05 true))

(event EventCreate
  (for _index (range 1 80)
    (bind _returnvalue (AddComponent|AddSceneComponent false (Math|Transform|MakeTransform (Math|Vector|MakeVector (Math|Random|RandomFloatinRange 0.0 2e+03) (Math|Random|RandomFloatinRange -1e+03 1e+03) 0.0) "0, 0, 0" "1,1,1")))
    (Utilities|Array|Add (Variables|Default|GetSpawnPoints) _returnvalue)))

(fn ConstructionScript
  (|CallParentFunction))