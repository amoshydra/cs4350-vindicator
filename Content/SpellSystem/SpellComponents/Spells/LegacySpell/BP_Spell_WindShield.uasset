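; Legacy wind shield spell actor that can grow in on creation and shrink away when cast.
; It passes its SpellDetectionVolume to the parent spell class as the collision volume.
; The construction script stores the mesh's scale as the end size and, if ShouldGrow is set, starts it at the beginning scale.
; Timelines lerp the scale on Create and Cast, and Cast destroys the actor afterward, or immediately without growth.
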(event EventBeginPlay
  (|CallParentFunction))

(event EventCreate
  (if (Variables|Default|GetshouldGrow)
    (bind _chargefactor (Timeline|ChargingAnimationTimeline Play)
      (:Update
        (Transformation|SetRelativeScale3D (Variables|Default|GetStaticMesh) (Math|Vector|Lerp(Vector) (Variables|Default|GetScaleBeginning) (Variables|Default|GetScaleEnd) _chargefactor))))))

(event EventSetCollisionVolume
  (params (CollisionVolumeForEnemy :type Primitive%20Component%20Object%20Reference) (CollisionVolumeForSpell :type Primitive%20Component%20Object%20Reference))
  (|CallParentFunction 0 (Variables|Default|GetSpellDetectionVolume)))

(event EventCast
  (if (Variables|Default|GetshouldGrow)
    (bind _chargefactor (Timeline|DechargingAnimationTimeline Play)
      (:Update
        (Transformation|SetRelativeScale3D (Variables|Default|GetStaticMesh) (Math|Vector|Lerp(Vector) (Variables|Default|GetScaleEnd) (Variables|Default|GetScaleBeginning) _chargefactor)))
      (:Finished
        (Actor|DestroyActor :!label _label)))
    (else
      (goto _label))))

(event EventDestroy)

(fn ConstructionScript
  (|CallParentFunction)
  (Variables|Default|SetScaleEnd (Variables|/Script/Engine.SceneComponent|GetRelativeScale3D (Variables|Default|GetStaticMesh)))
  (if (Variables|Default|GetshouldGrow)
    (Transformation|SetRelativeScale3D (Variables|Default|GetStaticMesh) (Variables|Default|GetScaleBeginning))
    (else
      (Transformation|SetRelativeScale3D (Variables|Default|GetStaticMesh) (Variables|Default|GetScaleEnd)))))