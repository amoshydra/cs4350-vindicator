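; BP_SpellComponent_Shard is a legacy spell shard projectile that falls straight down until it hits something.
; Tick moves the root downward at a fixed speed.
; When its capsule overlaps anything other than another shard, it deactivates the Shard effect and plays a half-scale frozen-exit burst attached to it.
; The actor destroys itself when that burst finishes, and no damage is applied here.
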(event OnComponentBeginOverlap(Capsule)
  (params (OverlappedComponent :type Primitive%20Component%20Object%20Reference) (OtherActor :type Actor%20Object%20Reference) (OtherComp :type Primitive%20Component%20Object%20Reference) (OtherBodyIndex :type Integer) (bFromSweep :type Boolean) (SweepResult :type Hit%20Result%20Structure%20%28by%20ref%29))
  (bind _shard (Variables|Default|GetShard))
  (Utilities|Casting|CastToBP_SpellComponent_Shard OtherActor
    (:CastFailed
      (Components|Activation|Deactivate _shard)
      (bind _returnvalue (Effects|SpawnEmitterAttached "/Game/Assets/InfinityBladeEffects/Effects/FX_Combat_Ice/P_Player_Frozen_Exit_01.P_Player_Frozen_Exit_01" _shard "None"))
      (Transformation|SetRelativeScale3D _returnvalue "0.500000,0.500000,0.500000")
      (EventDispatchers|AssignOnSystemFinished _returnvalue (delegate Custom|OnSystemFinished_Event_0)))))

(event Custom|OnSystemFinished_Event_0
  (params (PSystem :type Particle%20System%20Component%20Object%20Reference))
  (Actor|DestroyActor))

(event EventBeginPlay)

(event Collision|EventActorBeginOverlap
  (params (OtherActor :type Actor%20Object%20Reference)))

(event EventTick
  (params (DeltaSeconds :type Float%20%28single-precision%29))
  (Transformation|AddLocalOffset (Variables|Default|GetDefaultSceneRoot) (Math|Vector|MakeVector 0.0 0.0 (* DeltaSeconds -1.2e+03)) false false))

(fn ConstructionScript)