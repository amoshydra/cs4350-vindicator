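; Shield spell that scales in on creation, reflects enemy ranged projectiles off its forward vector, and shrinks away when cast.
; Overlap with another spell's detection volume starts a merge, driven through the tick dispatcher and a runtime spline that measures separation.
; A second shield held close heals the player on a timer and tints the rings green.
; A fireball shrinks, reddens the shield and spawns an attached FireCyclone, reverting if separated before casting.
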(event OnComponentBeginOverlap(SpellDetectionVolume)
  (params (OverlappedComponent :type Primitive%20Component%20Object%20Reference) (OtherActor :type Actor%20Object%20Reference) (OtherComp :type Primitive%20Component%20Object%20Reference) (OtherBodyIndex :type Integer) (bFromSweep :type Boolean) (SweepResult :type Hit%20Result%20Structure%20%28by%20ref%29))
  (bind _incomingspell (CallFunction|IsOverlappingforMerging OtherActor OtherComp))
  (Utilities|IsValid _incomingspell
    (:Is%20Valid
      (bind _output_get (Variables|Default|SetIncomingSpell _incomingspell))
      (Variables|Default|SetIncomingSpellSweepLocation (.location SweepResult))
      (switch string (Utilities|GetClassDisplayName (Utilities|GetClass _output_get))
        (:BP_Spell_Fireball_C
          (CallFunction|BeginMergingforBPSpellFireball))
        (:BP_Spell_Shield_C
          (CallFunction|BeginMergingforBPSpellShield))))))

(event OnComponentBeginOverlap(BlockingZone)
  (params (OverlappedComponent :type Primitive%20Component%20Object%20Reference) (OtherActor :type Actor%20Object%20Reference) (OtherComp :type Primitive%20Component%20Object%20Reference) (OtherBodyIndex :type Integer) (bFromSweep :type Boolean) (SweepResult :type Hit%20Result%20Structure%20%28by%20ref%29))
  (bind _asbp_enemy_range_projectile (Utilities|Casting|CastToBP_Enemy_Range_Projectile OtherActor))
  (bind _returnvalue (Utilities|Set|Add (Variables|Default|GetpreviouslyHitActor) _asbp_enemy_range_projectile))
  (if _returnvalue
    (Utilities|FlowControl|Sequence
      (:then_0
        (Audio|PlaySoundatLocation "/Engine/VREditor/Sounds/VR_grab_Cue.VR_grab_Cue" (Transformation|GetActorLocation _asbp_enemy_range_projectile) "0, 0, 0" 0.5))
      (:then_1
        ;[1 1 1] Reflect Projectile
        (Variables|/Script/Engine.MovementComponent|SetVelocity (Variables|/Game/AI/Enemy_Grunt_Range/BP_Enemy_Range_Projectile.BP_Enemy_Range_Projectile_C|GetProjectileMovement _asbp_enemy_range_projectile) (* (Math|Vector|GetReflectionVector (Math|Vector|Normalize (Transformation|GetVelocity _asbp_enemy_range_projectile)) (Math|Vector|GetForwardVector (Variables|Default|GetForward%20Vector))) (Math|Vector|VectorLength (Transformation|GetVelocity _asbp_enemy_range_projectile))))))))

(event OnComponentEndOverlap(SpellDetectionVolume)
  (params (OverlappedComponent :type Primitive%20Component%20Object%20Reference) (OtherActor :type Actor%20Object%20Reference) (OtherComp :type Primitive%20Component%20Object%20Reference) (OtherBodyIndex :type Integer))
  (bind _incomingspell (CallFunction|IsOverlappingforMerging OtherActor OtherComp))
  (Utilities|IsValid _incomingspell
    (:Is%20Valid
      (switch string (Utilities|GetClassDisplayName (Utilities|GetClass _incomingspell))))))

(event Custom|Begin%20merging%20for%20BP_Spell_Fireball
  ;[1 1 1] Merging Fireball + Shield = Firecyclone
  (Utilities|FlowControl|DoOnce false
    (:Completed
      (Utilities|FlowControl|Sequence
        (:then_0
          (EventDispatchers|AssignOnDestroyed (delegate Custom|MergeSpellFn_Fireball_SelfDestroyed)))
        (:then_1
          (bind _returnvalue (AddComponent|AddSplineComponent false))
          (Spline|ClearSplinePoints _returnvalue true)
          (CallFunction|MergeSpellFnFireBallSpawnFireCyclone))
        (:then_2
          (EventDispatchers|AssignEventTickDispatcher (delegate Custom|MergeSpellFn_FireBall_EventTick)))))))

(event Custom|MergeSpellFn_Shield_SelfDestroyed
  (params (DestroyedActor :type Actor%20Object%20Reference))
  ;[1 1 1] Merging Shield + Shield = Heal
  (CallFunction|EndMergingforBPSpellShield))

(event Custom|End%20merging%20for%20BP_Spell_Fireball
  ;[1 1 1] Merging Fireball + Shield = Firecyclone
  (Utilities|FlowControl|Sequence
    (:then_0
      (EventDispatchers|UnbindEventfromEventTickDispatcher (delegate Custom|MergeSpellFn_FireBall_EventTick))
      (Utilities|IsValid (stale Custom|Begin%20merging%20for%20BP_Spell_Fireball _returnvalue)
        (:Is%20Valid
          (Components|DestroyComponent (stale Custom|Begin%20merging%20for%20BP_Spell_Fireball _returnvalue)))))
    (:then_1
      (Utilities|FlowControl|DoOnce false) ; enters at Reset
    )))

(event Custom|MergeSpellFn_FireBall_SpawnFireCyclone
  (bind _returnvalue (Game|SpawnActorfromClass "/Game/SpellSystem/SpellComponents/Spells/LegacySpell/BP_Spell_FireCyclone2.BP_Spell_FireCyclone2_C" (Math|Transform|MakeTransform "0, 0, 0" "0, 0, 0" "1,1,1") "Undefined" 0 0))
  (Utilities|FlowControl|Sequence
    (:then_0
      (Default|Create _returnvalue)
      (Variables|Default|SetFireCycloneCasted false)
      (Transformation|AttachComponentToComponent (Variables|/Script/Engine.Actor|GetRootComponent _returnvalue) (Variables|Default|GetForward%20Vector) "None" "KeepRelative" "KeepRelative" "KeepRelative" true))
    (:then_1
      (EventDispatchers|AssignCastedSpell _returnvalue (delegate Custom|MergeSpellFn_FireBall_CompleteCastingForFireCyclone)))))

(event Custom|MergeSpellFn_FireBall_CompleteCastingForFireCyclone
  (Variables|Default|SetFireCycloneCasted true)
  (Transformation|DetachFromActor (stale Custom|MergeSpellFn_FireBall_SpawnFireCyclone _returnvalue) "KeepWorld" "KeepWorld" "KeepWorld") ; Should detach child (firecyclone)
  (CallFunction|EndMergingforBPSpellFireball)
  (Actor|DestroyActor (Variables|Default|GetIncomingSpell))
  (CallFunction|MergeSpellFnFireBallShieldEndSequence))

(event Custom|MergeSpellFn_FireBall_DestroyFireCyclone
  (Utilities|IsValid (stale Custom|MergeSpellFn_FireBall_SpawnFireCyclone _returnvalue)
    (:Is%20Valid
      (if (not (Variables|Default|GetFireCycloneCasted))
        (Default|Destroy (stale Custom|MergeSpellFn_FireBall_SpawnFireCyclone _returnvalue))))))

(event Custom|MergeSpellFn_FireBall_ShieldEndSequence
  ;[1 1 1] Merging Fireball + Shield = Firecyclone
  (Utilities|IsValid self
    (:Is%20Valid
      (Rendering|Material|SetVectorParameterValue (Variables|Default|GetShieldMaterialInstance) "RingColor" (Math|Color|Lerp(LinearColor) "(R=1.000000,G=0.042311,B=0.000000,A=1.000000)" "(R=1.000000,G=1.000000,B=1.000000,A=1.000000)" 1.0) :!class /Script/Engine.MaterialInstanceDynamic))))

(event Custom|MergeSpellFn_FireBall_FireballEndSequence
  ;[1 1 1] Merging Fireball + Shield = Firecyclone
  (bind _restoretrack (Timeline|MergeSpellFn_FireBall_RestoreTimeline PlayFromStart)
    (:Update
      (bind _incomingspell (Variables|Default|GetIncomingSpell)
        (:then
          (Transformation|SetRelativeScale3D (Variables|/Game/SpellSystem/SpellComponents/Spells/LegacySpell/BP_Spell_Base.BP_Spell_Base_C|GetStaticMesh _incomingspell) (Math|Vector|Lerp(Vector) (Variables|/Script/Engine.SceneComponent|GetRelativeScale3D (Variables|/Game/SpellSystem/SpellComponents/Spells/LegacySpell/BP_Spell_Base.BP_Spell_Base_C|GetStaticMesh _incomingspell)) "0.200000,0.200000,0.200000" _restoretrack)))
        (:else
          (Timeline|MergeSpellFn_FireBall_RestoreTimeline Stop))))))

(event Custom|Begin%20merging%20for%20BP_Spell_Shield
  ;[1 1 1] Merging Shield + Shield = Heal
  (Utilities|FlowControl|DoOnce false
    (:Completed
      (Utilities|FlowControl|Sequence
        (:then_0
          (EventDispatchers|AssignOnDestroyed (delegate Custom|MergeSpellFn_Shield_SelfDestroyed)))
        (:then_1
          (bind _returnvalue (AddComponent|AddSplineComponent false))
          (Spline|ClearSplinePoints _returnvalue true)
          (EventDispatchers|AssignEventTickDispatcher (delegate Custom|MergeSpellFn_Shield_EventTick)))))))

(event Custom|MergeSpellFn_FireBall_EventTick
  (params (DeltaSeconds :type Float%20%28single-precision%29))
  (bind _returnvalue (* DeltaSeconds 0.05))
  (bind _incomingspell (Variables|Default|GetIncomingSpell))
  (bind _staticmesh (Variables|/Game/SpellSystem/SpellComponents/Spells/LegacySpell/BP_Spell_Base.BP_Spell_Base_C|GetStaticMesh _incomingspell))
  (bind _relativescale3d (Variables|/Script/Engine.SceneComponent|GetRelativeScale3D _staticmesh))
  (bind _returnvalue_2 (- _relativescale3d _returnvalue))
  (bind _returnvalue_3 (Class|KismetMathLibrary|GetMinElement _returnvalue_2))
  (bind _returnvalue_4 (> _returnvalue_3 0.0))
  (bind _returnvalue_5 (Math|Vector|SelectVector _returnvalue_2 "0, 0, 0" _returnvalue_4))
  ;[1 1 1] Merging Fireball + Shield = Firecyclone
  (Utilities|IsValid (Variables|Default|GetIncomingSpell)
    (:Is%20Valid
      (Utilities|FlowControl|Sequence
        (:then_0
          (Utilities|FlowControl|Sequence
            (:then_0
              (Spline|ClearSplinePoints (stale Custom|Begin%20merging%20for%20BP_Spell_Fireball _returnvalue) false)
              (Spline|AddSplinePoint (stale Custom|Begin%20merging%20for%20BP_Spell_Fireball _returnvalue) (Transformation|GetActorLocation (Variables|Default|GetIncomingSpell)) "World" false)
              (Spline|AddSplinePoint (stale Custom|Begin%20merging%20for%20BP_Spell_Fireball _returnvalue) (Variables|Default|GetIncomingSpellSweepLocation) "Local" true))
            (:then_1
              (if (> (Spline|GetSplineLength (stale Custom|Begin%20merging%20for%20BP_Spell_Fireball _returnvalue)) 8e+01)
                (CallFunction|MergeSpellFnFireBallRestoretoDefaultState true true true)))))
        (:then_1
          (Transformation|SetRelativeScale3D _staticmesh _returnvalue_5)
          (Rendering|Material|SetVectorParameterValue (Variables|Default|GetShieldMaterialInstance) "RingColor" (Math|Color|Lerp(LinearColor) "(R=1.000000,G=1.000000,B=1.000000,A=1.000000)" "(R=1.000000,G=0.046773,B=0.000000,A=1.000000)" (- 1.0 (/ (Math|Vector|GetMaxElement _returnvalue_5) 0.2))) :!class /Script/Engine.MaterialInstanceDynamic))))
    (:Is%20Not%20Valid
      (CallFunction|MergeSpellFnFireBallRestoretoDefaultState true true true))))

(event Custom|End%20merging%20for%20BP_Spell_Shield
  ;[1 1 1] Merging Shield + Shield = Heal
  (Utilities|FlowControl|Sequence
    (:then_0
      (CallFunction|MergeSpellFnShieldEndHealPlayer)
      (EventDispatchers|UnbindEventfromEventTickDispatcher (delegate Custom|MergeSpellFn_Shield_EventTick))
      (Utilities|IsValid (stale Custom|Begin%20merging%20for%20BP_Spell_Shield _returnvalue)
        (:Is%20Valid
          (Components|DestroyComponent (stale Custom|Begin%20merging%20for%20BP_Spell_Shield _returnvalue)))))
    (:then_1
      (Utilities|FlowControl|DoOnce false) ; enters at Reset
    )))

(event Custom|MergeSpellFn_Shield_EventTick
  (params (DeltaSeconds :type Float%20%28single-precision%29))
  ;[1 1 1] Merging Shield + Shield = Heal
  (Utilities|IsValid (stale Custom|Begin%20merging%20for%20BP_Spell_Shield _returnvalue)
    (:Is%20Valid
      (Variables|Default|GetIncomingSpell
        (:then
          (Utilities|FlowControl|Sequence
            (:then_0
              (Spline|ClearSplinePoints (stale Custom|Begin%20merging%20for%20BP_Spell_Shield _returnvalue) false)
              (Spline|AddSplinePoint (stale Custom|Begin%20merging%20for%20BP_Spell_Shield _returnvalue) (Transformation|GetActorLocation (Variables|Default|GetIncomingSpell)) "World" false)
              (Spline|AddSplinePoint (stale Custom|Begin%20merging%20for%20BP_Spell_Shield _returnvalue) (Transformation|GetActorLocation self) "World" true))
            (:then_1
              (if (Math|Float|InRange(Float) (Spline|GetSplineLength (stale Custom|Begin%20merging%20for%20BP_Spell_Shield _returnvalue)) 0.0 1e+02)
                (if (Math|Float|InRange(Float) (Spline|GetSplineLength (stale Custom|Begin%20merging%20for%20BP_Spell_Shield _returnvalue)) 0.0 3e+01)
                  (CallFunction|MergeSpellFnShieldStartHealPlayer)
                  (else
                    (CallFunction|MergeSpellFnShieldEndHealPlayer)))
                (else
                  (CallFunction|EndMergingforBPSpellShield))))))
        (:else
          (CallFunction|EndMergingforBPSpellShield :!label _label))))
    (:Is%20Not%20Valid
      (goto _label))))

(event Custom|MergeSpellFn_Fireball_SelfDestroyed
  (params (DestroyedActor :type Actor%20Object%20Reference))
  ;[1 1 1] Merging Fireball + Shield = Firecyclone
  (CallFunction|MergeSpellFnFireBallRestoretoDefaultState false true true))

(event Custom|MergeSpellFn_Shield_HealPlayer
  ;[1 1 1] Merging Shield + Shield = Heal
  (bind _asbp_vr_pawn (Utilities|Casting|CastToBP_VR_Pawn (Game|Player|GetPlayerPawn 0)))
  (Default|DamagePlayer _asbp_vr_pawn -1.0))

(event Custom|MergeSpellFn_FireBall_RestoreToDefaultState
  (params (RestoreShield :type Boolean) (RestoreFireball :type Boolean) (RestoreFireCyclone :type Boolean))
  ;[1 1 1] Merging Fireball + Shield = Firecyclone
  (CallFunction|EndMergingforBPSpellFireball)
  (Utilities|FlowControl|Sequence
    (:then_0
      (if RestoreShield
        (CallFunction|MergeSpellFnFireBallShieldEndSequence)))
    (:then_1
      (if RestoreFireball
        (CallFunction|MergeSpellFnFireBallFireballEndSequence)))
    (:then_2
      (if RestoreFireCyclone
        (CallFunction|MergeSpellFnFireBallDestroyFireCyclone)))))

(event Custom|MergeSpellFn_Shield_EndHealPlayer
  ;[1 1 1] Merging Shield + Shield = Heal
  (Utilities|FlowControl|Sequence
    (:then_0
      (Utilities|FlowControl|DoOnce false) ; enters at Reset
    )
    (:then_1
      (Utilities|Time|ClearandInvalidateTimerbyHandle (stale Custom|MergeSpellFn_Shield_StartHealPlayer _returnvalue))
      (Rendering|Material|SetVectorParameterValue (Variables|Default|GetShieldMaterialInstance) "RingColor" "(R=1.000000,G=1.000000,B=1.000000,A=1.000000)" :!class /Script/Engine.MaterialInstanceDynamic))))

(event Custom|MergeSpellFn_Shield_StartHealPlayer
  ;[1 1 1] Merging Shield + Shield = Heal
  (Utilities|FlowControl|DoOnce false
    (:Completed
      (bind _returnvalue (Utilities|Time|SetTimerbyEvent (delegate Custom|MergeSpellFn_Shield_HealPlayer) 1.5 true))
      (Rendering|Material|SetVectorParameterValue (Variables|Default|GetShieldMaterialInstance) "RingColor" "(R=0.552068,G=1.000000,B=0.515429,A=1.000000)" :!class /Script/Engine.MaterialInstanceDynamic))))

(event EventBeginPlay
  (|CallParentFunction)
  (bind _returnvalue (Rendering|Material|CreateDynamicMaterialInstance (Variables|Default|GetStaticMesh) 0 "/Game/SpellSystem/SpellComponents/Spells/CustomAssets/Shield/shield-rings-2_Mat.shield-rings-2_Mat" :!class /Script/Engine.PrimitiveComponent))
  (Variables|Default|SetShieldMaterialInstance _returnvalue))

(event EventCreate
  (bind _shieldmaterialinstance (Variables|Default|GetShieldMaterialInstance))
  (if (Variables|Default|GetshouldGrow)
    (bind _chargefactor (Timeline|ChargingAnimationTimeline Play)
      (:Update
        (Transformation|SetRelativeScale3D (Variables|Default|GetStaticMesh) (Math|Vector|Lerp(Vector) (Variables|Default|GetScaleBeginning) (Variables|Default|GetScaleEnd) _chargefactor))
        (Rendering|Material|SetScalarParameterValue _shieldmaterialinstance "RingVisibility" _chargefactor :!class /Script/Engine.MaterialInstanceDynamic)
        (Rendering|Material|SetScalarParameterValue _shieldmaterialinstance "GlypseVisibility" _chargefactor :!class /Script/Engine.MaterialInstanceDynamic)
        (Rendering|Material|SetScalarParameterValue _shieldmaterialinstance "OuterElementVisibility" _chargefactor :!class /Script/Engine.MaterialInstanceDynamic)))))

(event EventSetCollisionVolume
  (params (CollisionVolumeForEnemy :type Primitive%20Component%20Object%20Reference) (CollisionVolumeForSpell :type Primitive%20Component%20Object%20Reference))
  (|CallParentFunction 0 (Variables|Default|GetSpellDetectionVolume)))

(event EventCast
  (bind _incomingspell (Variables|Default|GetIncomingSpell)
    (:then
      (switch string (Utilities|GetClassDisplayName (Utilities|GetClass _incomingspell))
        (:Default
          _)
        (:BP_Spell_Fireball_C
          (bind _asbp_spell_fireball (Utilities|Casting|CastToBP_Spell_Fireball (Variables|Default|GetIncomingSpell))
            (:then
              (Default|RestoretoDefaultSize _asbp_spell_fireball))
            (:CastFailed
              _)))
        (:BP_Spell_ElectricFist_C
          _)
        (:BP_Spell_Shield_C
          _)))
    (:else
      _))
  (if (Variables|Default|GetshouldGrow)
    (bind _chargefactor (Timeline|DechargingAnimationTimeline Play)
      (:Update
        (Transformation|SetRelativeScale3D (Variables|Default|GetStaticMesh) (Math|Vector|Lerp(Vector) (Variables|Default|GetScaleEnd) (Variables|Default|GetScaleBeginning) _chargefactor)))
      (:Finished
        (Actor|DestroyActor :!label _label)))
    (else
      (goto _label))))

(event EventTick
  (params (DeltaSeconds :type Float%20%28single-precision%29))
  (Default|CallEventTickDispatcher DeltaSeconds))

(event EventDestroy)

(fn ConstructionScript
  (bind _scene (Variables|Default|GetScene))
  (|CallParentFunction)
  (Utilities|FlowControl|Sequence
    (:then_0
      (Variables|Default|SetScaleEnd (Variables|/Script/Engine.SceneComponent|GetRelativeScale3D (Variables|Default|GetStaticMesh)))
      (if (Variables|Default|GetshouldGrow)
        (Transformation|SetRelativeScale3D (Variables|Default|GetStaticMesh) (Variables|Default|GetScaleBeginning))
        (else
          (Transformation|SetRelativeScale3D (Variables|Default|GetStaticMesh) (Variables|Default|GetScaleEnd)))))
    (:then_1
      (Rendering|SetVisibility _scene (Variables|/Script/Engine.SceneComponent|GetbVisible _scene) true))))

(fn IsOverlappingforMerging
  (params (Other%20Actor :type Actor%20Object%20Reference) (Other%20Component :type Primitive%20Component%20Object%20Reference))
  (if (!= Other%20Actor self)
    (bind _asbp_spell_base (Utilities|Casting|CastToBP_Spell_Base Other%20Actor))
    (if (== Other%20Component (Variables|/Game/SpellSystem/SpellComponents/Spells/LegacySpell/BP_Spell_Base.BP_Spell_Base_C|GetCollisionVolumeForSpell _asbp_spell_base))
      (return _asbp_spell_base)
      (else
        _)))
  (return 0))