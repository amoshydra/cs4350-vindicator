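; Legacy forked lightning spell actor that damages and stuns every enemy within a cone and distance in front of it.
; On Create it detaches, hides its meshes, switches to the aftershock effect and cone-searches the game instance's enemy list.
; Each hit gets an impact emitter and a lightning emitter rotated, stretched and offset to span the gap.
; The lightning and aftershock deactivate after a short delay.
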(event Custom|SpawnLightning
  (params (Enemy :type BP%20Enemy%20Base%20Object%20Reference))
  (bind _returnvalue (Transformation|GetActorLocation))
  (bind _capsulecomponent (Variables|/Script/Engine.Character|GetCapsuleComponent Enemy))
  (bind _returnvalue_2 (Physics|GetCenterOfMass _capsulecomponent "None"))
  (bind _returnvalue_3 (- _returnvalue_2 _returnvalue))
  (bind _returnvalue_4 (Math|Conversions|RotationFromXVector _returnvalue_3))
  (bind _returnvalue_5 (Math|Vector|VectorLength _returnvalue_3))
  (bind _returnvalue_6 (/ _returnvalue_5 3.5e+02))
  (bind _returnvalue_7 (Effects|SpawnEmitteratLocation "/Game/Assets/InfinityBladeEffects/Effects/FX_Monsters/FX_Monster_Genno/P_Genno_Weapon_Lightning_01.P_Genno_Weapon_Lightning_01" (Transformation|GetActorLocation) (Math|Rotator|MakeRotator (.roll _returnvalue_4) (+ (.pitch _returnvalue_4) -9e+01) (.yaw _returnvalue_4)) false))
  (Utilities|FlowControl|Sequence
    (:then_0
      (Utilities|Array|Add (Variables|Default|GetParticles) _returnvalue_7))
    (:then_1
      (Transformation|SetRelativeScale3D _returnvalue_7 (Math|Vector|MakeVector 1.0 _returnvalue_6 1.0)))
    (:then_2
      (Transformation|AttachComponentToComponent _returnvalue_7 (Variables|Default|GetDefaultSceneRoot) "None" "KeepRelative" "KeepRelative" "KeepRelative" true))
    (:then_3
      (Transformation|AddRelativeLocation _returnvalue_7 (Math|Vector|MakeVector (.x (* (Math|Vector|GetUpVector _returnvalue_7) (* (- _returnvalue_6 1.0) 2.6e+02))) (.y (* (Math|Vector|GetUpVector _returnvalue_7) (* (- _returnvalue_6 1.0) 2.6e+02))) (- (.z (* (Math|Vector|GetUpVector _returnvalue_7) (* (- _returnvalue_6 1.0) 2.6e+02))) 2e+01)) false false))))

(event EventBeginPlay
  (|CallParentFunction)
  (Math|Random|SetRandomStreamSeed (Variables|Default|GetNewVar_2) 0))

(event Collision|EventActorBeginOverlap
  (params (OtherActor :type Actor%20Object%20Reference))
  (|CallParentFunction OtherActor))

(event EventCreate
  ;[1 1 1] Animation
  (Components|Activation|Deactivate (Variables|Default|GetInitialShock))
  (Rendering|SetVisibility (Variables|Default|GetStaticMesh) false false)
  (Components|Activation|Activate (Variables|Default|GetAfterShock) false)
  (Transformation|DetachFromActor "KeepWorld" "KeepWorld" "KeepWorld")
  ;[1 1 1] Apply Debuff to Enemies
  (bind _asbp_game_instance (Utilities|Casting|CastToBP_GameInstance (Game|GetGameInstance)))
  (bind _enemies (CallFunction|ConeSearch (Transformation|GetActorLocation) (Transformation|GetActorForwardVector) (Variables|/Game/Blueprints/BP_GameInstance.BP_GameInstance_C|GetEnemies _asbp_game_instance) (Variables|Default|GetDegrees)))
  (for _array_element _enemies
    (if (<= (Transformation|GetDistanceTo _array_element) (Variables|Default|GetDistance))
      (CallFunction|Inflict _array_element false 0.0)
      (Default|ActivateDebuff (Variables|/Game/AI/BP_Enemy_Base.BP_Enemy_Base_C|GetBP_Debuff_Manager _array_element) "/Game/SpellSystem/SpellComponents/Debuffs/BP_Debuff_Stun.BP_Debuff_Stun_C")
      (Effects|SpawnEmitteratLocation "/Game/Assets/InfinityBladeEffects/Effects/FX_Mobile/Lightning/P_LineToPoint_Spawn_Proj_Lightning_00.P_LineToPoint_Spawn_Proj_Lightning_00" (Transformation|GetActorLocation _array_element))
      (CallFunction|SpawnLightning _array_element)))
  (Utilities|FlowControl|Delay 1.0)
  (for _array_element_2 (Variables|Default|GetParticles)
    (Components|Activation|Deactivate _array_element_2))
  (Components|Activation|Deactivate (Variables|Default|GetAfterShock)))

(event EventTick
  (params (DeltaSeconds :type Float%20%28single-precision%29))
  (|CallParentFunction DeltaSeconds))

(fn ConstructionScript
  (|CallParentFunction))