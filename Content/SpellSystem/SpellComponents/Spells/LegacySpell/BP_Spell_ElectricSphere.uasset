(event OnComponentBeginOverlap(CollisionVolumeForEnemy)
  (params (OverlappedComponent :type Primitive%20Component%20Object%20Reference) (OtherActor :type Actor%20Object%20Reference) (OtherComp :type Primitive%20Component%20Object%20Reference) (OtherBodyIndex :type Integer) (bFromSweep :type Boolean) (SweepResult :type Hit%20Result%20Structure%20%28by%20ref%29))
  (if (not (Variables|Default|GethasInflictDebuff))
    (bind _asbp_enemy_base (Utilities|Casting|CastToBP_Enemy_Base OtherActor))
    (CallFunction|CreateImpactonEnemy _asbp_enemy_base)))

(event Custom|CreateImpactOnEnemy
  (params (Enemy :type BP%20Enemy%20Base%20Object%20Reference))
  (bind _returnvalue (Transformation|GetActorLocation Enemy))
  (bind _self self)
  (bind _returnvalue_2 (Transformation|GetActorLocation _self))
  (bind _returnvalue_3 (- _returnvalue _returnvalue_2))
  ;[1 1 1] Check is existing overlapped enemy
  (bind _returnvalue_4 (Utilities|Set|Add (Variables|Default|GetOverlappedEnemy) Enemy))
  (if _returnvalue_4
    (Utilities|FlowControl|Sequence
      (:then_0
        (Default|ActivateDebuff (Variables|/Game/AI/BP_Enemy_Base.BP_Enemy_Base_C|GetBP_Debuff_Manager Enemy) "/Game/SpellSystem/SpellComponents/Debuffs/BP_Debuff_Stun.BP_Debuff_Stun_C"))
      (:then_1
        (Pawn|Components|CharacterMovement|SetMovementMode (Variables|/Script/Engine.Character|GetCharacterMovement Enemy) "MOVE_Falling" 0)
        (Character|LaunchCharacter Enemy (* (Math|Vector|Normalize _returnvalue_3) (* (/ 1.0 (Math|Vector|VectorLengthSquared _returnvalue_3)) 1e+06 (Variables|Default|GetKnockBackVelocity))) true true)))))

(event EventBeginPlay
  (|CallParentFunction))

(event Collision|EventActorBeginOverlap
  (params (OtherActor :type Actor%20Object%20Reference))
  (|CallParentFunction OtherActor))

(event EventTick
  (params (DeltaSeconds :type Float%20%28single-precision%29))
  (|CallParentFunction DeltaSeconds))

(event EventCreate
  (for _array_element (Collision|GetOverlappingActors "/Game/AI/BP_Enemy_Base.BP_Enemy_Base_C" :!class /Script/Engine.Actor)
    (bind _asbp_enemy_base (Utilities|Casting|CastToBP_Enemy_Base _array_element))
    (CallFunction|CreateImpactonEnemy _asbp_enemy_base))
  (bind _spheregrowfactor (Timeline|SpellGrowFactor PlayFromStart)
    (:Update
      (Transformation|SetRelativeScale3D (Variables|Default|GetStaticMesh) (Math|Vector|Lerp(Vector) (Variables|Default|GetScaleStart) (Variables|Default|GetScaleEnd) _spheregrowfactor)))
    (:Finished
      (Variables|Default|SethasInflictDebuff true)
      (bind _spheregrowfactor_2 (Timeline|SpellFinishTimeline Play)
        (:Update
          (Transformation|SetRelativeScale3D (Variables|Default|GetStaticMesh) (Math|Vector|Lerp(Vector) (Variables|Default|GetScaleEnd) (* (Variables|Default|GetScaleEnd) 5.0) _spheregrowfactor_2)))
        (:Finished
          (Utilities|Set|Clear (Variables|Default|GetOverlappedEnemy))
          (Actor|DestroyActor))))))

(event EventCast)

(event EventSetCollisionVolume
  (params (CollisionVolumeForEnemy :type Primitive%20Component%20Object%20Reference) (CollisionVolumeForSpell :type Primitive%20Component%20Object%20Reference))
  (|CallParentFunction (Variables|Default|GetStaticMesh) 0))

(fn ConstructionScript
  (|CallParentFunction)
  (CallFunction|DuplicateActor))

(fn DuplicateActor
  (bind _staticmesh (Variables|Default|GetStaticMesh))
  (bind _returnvalue (AddComponent|AddChildActorComponent false))
  (ChildActorComponent|SetChildActorClass _returnvalue (LocalVariables|GetMirrorActorClass))
  (LocalVariables|SetMirrorChildActorComponent _returnvalue)
  (Utilities|FlowControl|Sequence
    (:then_0
      ;[1 1 1] Initialising variables
      (Utilities|FlowControl|Sequence
        (:then_0
          (bind _asbp_spell_wind_shield (Utilities|Casting|CastToBP_Spell_WindShield (Variables|/Script/Engine.ChildActorComponent|GetChildActor (LocalVariables|GetMirrorChildActorComponent))))
          (LocalVariables|SetMirrorActor _asbp_spell_wind_shield))
        (:then_1
          (LocalVariables|SetMirrorStaticMesh (Variables|/Game/SpellSystem/SpellComponents/Spells/LegacySpell/BP_Spell_Base.BP_Spell_Base_C|GetStaticMesh (LocalVariables|GetMirrorActor))))
        (:then_2
          (Variables|Default|SetScaleStart (Variables|/Game/SpellSystem/SpellComponents/Spells/LegacySpell/BP_Spell_WindShield.BP_Spell_WindShield_C|GetScaleEnd (LocalVariables|GetMirrorActor))))))
    (:then_1
      ;[1 1 1] Perform Duplication
      (Utilities|FlowControl|Sequence
        (:then_0
          (Components|StaticMesh|SetStaticMesh (Variables|Default|GetStaticMesh) (Variables|/Script/Engine.StaticMeshComponent|GetStaticMesh (LocalVariables|GetMirrorStaticMesh))))
        (:then_1
          (Transformation|SetRelativeScale3D _staticmesh (Variables|Default|GetScaleStart))
          (Transformation|SetRelativeRotation _staticmesh "-90.000000, 0, 0" false false))
        (:then_2
          (Rendering|Material|SetMaterial (Variables|Default|GetStaticMesh) 0 (Rendering|Material|GetMaterial (LocalVariables|GetMirrorStaticMesh) 0)))))
    (:then_2
      ;[1 1 1] Clean up variables
      (Components|DestroyComponent (LocalVariables|GetMirrorChildActorComponent)))))