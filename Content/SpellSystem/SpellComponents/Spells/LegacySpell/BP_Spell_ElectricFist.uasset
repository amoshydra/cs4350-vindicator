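; Legacy Electric Fist spell that shocks, damages and launches enemies.
; On Create, it launches overlapping enemies along its forward vector and deals damage scaled from a fixed velocity; Cast destroys the actor.
; Capsule overlaps track enemies in OverlappedEnemy, applying light damage with a spark effect on entry.
; The physics-velocity punch with a retrigger cooldown is disconnected, and CreateImpact is empty.
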(event OnComponentEndOverlap(CapsuleCollision)
  (params (OverlappedComponent :type Primitive%20Component%20Object%20Reference) (OtherActor :type Actor%20Object%20Reference) (OtherComp :type Primitive%20Component%20Object%20Reference) (OtherBodyIndex :type Integer))
  (bind _asbp_enemy_base (Utilities|Casting|CastToBP_Enemy_Base OtherActor))
  (Utilities|Set|Remove (Variables|Default|GetOverlappedEnemy) _asbp_enemy_base))

(event OnComponentBeginOverlap(CapsuleCollision)
  (params (OverlappedComponent :type Primitive%20Component%20Object%20Reference) (OtherActor :type Actor%20Object%20Reference) (OtherComp :type Primitive%20Component%20Object%20Reference) (OtherBodyIndex :type Integer) (bFromSweep :type Boolean) (SweepResult :type Hit%20Result%20Structure%20%28by%20ref%29))
  (bind _asbp_enemy_base (Utilities|Casting|CastToBP_Enemy_Base OtherActor))
  (bind _returnvalue (Utilities|Set|Add (Variables|Default|GetOverlappedEnemy) _asbp_enemy_base))
  (if _returnvalue
    (Default|DamageEnemyEvent _asbp_enemy_base 0.25)
    (Effects|SpawnEmitteratLocation "/Game/Assets/InfinityBladeEffects/Effects/FX_Monsters/FX_Monster_Ausar/P_AU_Taunt_sparks.P_AU_Taunt_sparks" (Transformation|GetActorLocation _asbp_enemy_base))))

(event Custom|CreateImpact
  (params (Enemy :type BP%20Enemy%20Base%20Object%20Reference)))

(event Custom|ResetImpactTimer
  (Variables|Default|SetisRetriggerable true))

(event EventBeginPlay
  (|CallParentFunction))

(event EventSetCollisionVolume
  (params (CollisionVolumeForEnemy :type Primitive%20Component%20Object%20Reference) (CollisionVolumeForSpell :type Primitive%20Component%20Object%20Reference))
  (|CallParentFunction 0 (Variables|Default|GetSpellCollisionVolume)))

(event EventCast
  (Actor|DestroyActor))

(event EventCreate
  (bind _forward_vector (Variables|Default|GetForward%20Vector))
  (bind _returnvalue (Math|Vector|GetForwardVector _forward_vector))
  (bind _returnvalue_2 (* _returnvalue 300))
  (for _array_element (Collision|GetOverlappingActors "/Game/AI/BP_Enemy_Base.BP_Enemy_Base_C" :!class /Script/Engine.Actor)
    (bind _asbp_enemy_base (Utilities|Casting|CastToBP_Enemy_Base _array_element))
    (CallFunction|KnockEnemywithVelocity _returnvalue_2 _asbp_enemy_base)
    (CallFunction|DamageEnemywithVelocity _returnvalue_2 _asbp_enemy_base)))

(fn ConstructionScript
  (|CallParentFunction))

(fn DamageEnemywithVelocity
  (params (Velocity :type Vector) (Enemy :type BP%20Enemy%20Base%20Object%20Reference))
  (Utilities|FlowControl|Sequence
    (:then_0
      (CallFunction|Inflict Enemy true (* (/ (Math|Vector|VectorLength Velocity) 1e+03) 5.0))
      (Components|Activation|Activate (Variables|Default|GetImpactSpark) true))
    (:then_1)))

(fn KnockEnemywithVelocity
  (params (Velocity :type Vector) (Enemy :type BP%20Enemy%20Base%20Object%20Reference))
  (bind _strength (Variables|Default|GetStrength))
  (Utilities|FlowControl|Sequence
    (:then_0
      (Pawn|Components|CharacterMovement|SetMovementMode (Variables|/Script/Engine.Character|GetCharacterMovement Enemy) "MOVE_Falling" 0))
    (:then_1
      (Character|LaunchCharacter Enemy (+ (* Velocity (Math|Vector|MakeVector _strength _strength 0.0)) (Math|Vector|MakeVector 0.0 0.0 1.6e+02)) true true))))