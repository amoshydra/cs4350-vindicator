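; BP_Spell_Base is a base Blueprint for spells in the legacy spell system, providing shared hooks and damage delivery.
; Create, Cast and Destroy are empty stubs, and the event graph has no active logic.
; Inflict sends either the default Damage or an alternate value to a BP_Enemy_Base through DamageEnemyEvent.
; SetCollisionVolume, called from the construction script, stores separate collision volumes for enemies and spells.
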(event EventBeginPlay)

(event Collision|EventActorBeginOverlap
  (params (OtherActor :type Actor%20Object%20Reference)))

(event EventTick
  (params (DeltaSeconds :type Float%20%28single-precision%29)))

(fn ConstructionScript
  (CallFunction|SetCollisionVolume))

(fn Create)

(fn Cast)

(fn Destroy)

(fn Inflict
  (params (EnemyRef :type Actor%20Object%20Reference) (UseAlternateDamage :type Boolean) (AlternateDamage :type Float%20%28single-precision%29))
  (if UseAlternateDamage
    (LocalVariables|SetEffectiveDamage AlternateDamage)
    (else
      (LocalVariables|SetEffectiveDamage (Variables|Default|GetDamage))))
  (bind _asbp_enemy_base (Utilities|Casting|CastToBP_Enemy_Base EnemyRef))
  (Default|DamageEnemyEvent _asbp_enemy_base (LocalVariables|GetEffectiveDamage)))

(fn SetCollisionVolume
  (params (CollisionVolumeForEnemy :type Primitive%20Component%20Object%20Reference) (CollisionVolumeForSpell :type Primitive%20Component%20Object%20Reference))
  (Utilities|FlowControl|Sequence
    (:then_0
      (Variables|Default|SetCollisionVolumeForEnemy CollisionVolumeForEnemy))
    (:then_1
      (Variables|Default|SetCollisionVolumeForSpell CollisionVolumeForSpell))))