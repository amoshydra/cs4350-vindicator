(event OnComponentBeginOverlap(CollisionVolume)
  (params (OverlappedComponent :type Primitive%20Component%20Object%20Reference) (OtherActor :type Actor%20Object%20Reference) (OtherComp :type Primitive%20Component%20Object%20Reference) (OtherBodyIndex :type Integer) (bFromSweep :type Boolean) (SweepResult :type Hit%20Result%20Structure%20%28by%20ref%29))
  (bind _returnvalue (Transformation|GetActorForwardVector))
  (bind _returnvalue_2 (* _returnvalue 3e+03))
  (bind _asbp_enemy_base (Utilities|Casting|CastToBP_Enemy_Base OtherActor))
  (Character|LaunchCharacter _asbp_enemy_base (Math|Vector|MakeVector (.x _returnvalue_2) (.y _returnvalue_2) 0.0) true false)
  (Effects|SpawnEmitteratLocation "/Game/Assets/InfinityBladeEffects/Effects/FX_Mobile/Impacts/P_Impact_Shie_2.P_Impact_Shie_2" (Transformation|GetActorLocation _asbp_enemy_base))
  (CallFunction|Inflict _asbp_enemy_base false 0.0))

(event Custom|End%20Particle
  (bind _cyclone (Variables|Default|GetCyclone))
  (EventDispatchers|AssignOnSystemFinished _cyclone (delegate Custom|OnSystemFinished_Event_0))
  (Components|Activation|Deactivate _cyclone)
  (Variables|/Script/Engine.PrimitiveComponent|SetbGenerateOverlapEvents (Variables|Default|GetCollisionVolume) false))

(event Custom|OnSystemFinished_Event_0
  (params (PSystem :type Particle%20System%20Component%20Object%20Reference))
  (Actor|DestroyActor self))

(event EventBeginPlay
  (|CallParentFunction))

(event Collision|EventActorBeginOverlap
  (params (OtherActor :type Actor%20Object%20Reference))
  (|CallParentFunction OtherActor))

(event EventTick
  (params (DeltaSeconds :type Float%20%28single-precision%29))
  (|CallParentFunction DeltaSeconds))

(event Collision|EventHit
  (params (MyComp :type Primitive%20Component%20Object%20Reference) (Other :type Actor%20Object%20Reference) (OtherComp :type Primitive%20Component%20Object%20Reference) (bSelfMoved :type Boolean) (HitLocation :type Vector :default "0, 0, 0") (HitNormal :type Vector :default "0, 0, 0") (NormalImpulse :type Vector :default "0, 0, 0") (Hit :type Hit%20Result%20Structure%20%28by%20ref%29)))

(event EventCreate
  (bind _returnvalue (Game|Player|GetPlayerPawn 0))
  (bind _projectilemovement (Variables|Default|GetProjectileMovement))
  (bind _p_au_shieldslam_aoe (Variables|Default|GetP_AU_ShieldSlam_AOE))
  (bind _returnvalue_2 (Transformation|GetActorLocation _returnvalue))
  (Components|Activation|Activate _p_au_shieldslam_aoe false)
  (Transformation|SetWorldLocation _p_au_shieldslam_aoe (Math|Vector|MakeVector (.x _returnvalue_2) (.y _returnvalue_2) (- (.z _returnvalue_2) 1.1e+02)) false false)
  (Utilities|FlowControl|Delay 0.5)
  (Components|Activation|Activate _projectilemovement false)
  (Transformation|DetachFromActor "KeepWorld" "KeepWorld" "KeepWorld")
  (Variables|/Script/Engine.MovementComponent|SetVelocity _projectilemovement (* (Transformation|GetActorForwardVector) 6e+02))
  (Utilities|Time|SetTimerbyEvent (delegate Custom|End%20Particle) 2.0))

(event EventCast)

(fn ConstructionScript
  (|CallParentFunction))