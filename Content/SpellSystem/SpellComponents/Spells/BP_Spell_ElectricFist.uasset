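; Electric Fist spell actor that knocks back an enemy its sphere overlaps.
; A timeline repeatedly launches the enemy along the static mesh's physics velocity, scaled by the curve and Strength, with Strength divided back out of Z.
; The empty ActorBeginOverlap override defers the parent's overlap logic until the timeline finishes, when it is called on that enemy.
; The Cast event only destroys the actor, and Create is empty.
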(event OnComponentBeginOverlap(Sphere)
  (params (OverlappedComponent :type Primitive%20Component%20Object%20Reference) (OtherActor :type Actor%20Object%20Reference) (OtherComp :type Primitive%20Component%20Object%20Reference) (OtherBodyIndex :type Integer) (bFromSweep :type Boolean) (SweepResult :type Hit%20Result%20Structure%20%28by%20ref%29))
  (bind _asbp_enemy_base (Utilities|Casting|CastToBP_Enemy_Base OtherActor))
  (Variables|Default|SetEnemyRef _asbp_enemy_base)
  (bind _returnvalue (Physics|GetPhysicsLinearVelocity (Variables|Default|GetStaticMesh) "None"))
  (bind _newtrack_0 (Timeline|Timeline_0 PlayFromStart)
    (:Update
      (Character|LaunchCharacter (Variables|Default|GetEnemyRef) (Math|Vector|MakeVector (.X (Math|Vector|BreakVector (* _returnvalue (* _newtrack_0 (Variables|Default|GetStrength))))) (.Y (Math|Vector|BreakVector (* _returnvalue (* _newtrack_0 (Variables|Default|GetStrength))))) (/ (.Z (Math|Vector|BreakVector (* _returnvalue (* _newtrack_0 (Variables|Default|GetStrength))))) (Variables|Default|GetStrength))) true true))
    (:Finished
      (|CallParentFunction (Variables|Default|GetEnemyRef)))))

(event EventBeginPlay
  (|CallParentFunction))

(event Collision|EventActorBeginOverlap
  (params (OtherActor :type Actor%20Object%20Reference)))

(event EventCast
  (Actor|DestroyActor))

(event EventCreate)

(fn ConstructionScript
  (|CallParentFunction))