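; Lightning Blade spell: a sword that scales up on Create and shrinks away on Cast before destroying itself.
; Its damage volume hurts enemies on overlap entry, tracking them to avoid repeat hits, and destroys enemy ranged projectiles.
; Overlapping another spell hides the blade and spawns an attached laser while a timeline drives fireball charging.
; When that timeline finishes or the fireball strays too far, laser, fireball and blade are ended.
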(event OnComponentEndOverlap(DamageCollisionVolume)
  (params (OverlappedComponent :type Primitive%20Component%20Object%20Reference) (OtherActor :type Actor%20Object%20Reference) (OtherComp :type Primitive%20Component%20Object%20Reference) (OtherBodyIndex :type Integer))
  (bind _asbp_enemy_base (Utilities|Casting|CastToBP_Enemy_Base OtherActor))
  (Utilities|Set|Remove (Variables|Default|GetOverlappedEnemy) _asbp_enemy_base))

(event OnComponentEndOverlap(SpellCollisionVolume)
  (params (OverlappedComponent :type Primitive%20Component%20Object%20Reference) (OtherActor :type Actor%20Object%20Reference) (OtherComp :type Primitive%20Component%20Object%20Reference) (OtherBodyIndex :type Integer)))

(event OnComponentBeginOverlap(DamageCollisionVolume)
  (params (OverlappedComponent :type Primitive%20Component%20Object%20Reference) (OtherActor :type Actor%20Object%20Reference) (OtherComp :type Primitive%20Component%20Object%20Reference) (OtherBodyIndex :type Integer) (bFromSweep :type Boolean) (SweepResult :type Hit%20Result%20Structure%20%28by%20ref%29))
  (if (not (Variables|Default|GetJustSpawned))
    (bind _asbp_enemy_base (Utilities|Casting|CastToBP_Enemy_Base OtherActor)
      (:then
        (bind _returnvalue (Utilities|Set|Add (Variables|Default|GetOverlappedEnemy) _asbp_enemy_base))
        (if _returnvalue
          (CallFunction|Inflict _asbp_enemy_base false 0.0)
          (Effects|SpawnEmitteratLocation "/Game/Assets/InfinityBladeEffects/Effects/FX_Monsters/FX_Monster_Ausar/P_AU_Taunt_sparks.P_AU_Taunt_sparks" (Transformation|GetActorLocation _asbp_enemy_base))
          (Audio|PlaySoundatLocation "/Game/SoundAsset/Spell/Spell_BladeSlash.Spell_BladeSlash" (Transformation|GetActorLocation _asbp_enemy_base))))
      (:CastFailed
        (bind _asbp_enemy_range_projectile (Utilities|Casting|CastToBP_Enemy_Range_Projectile OtherActor))
        (Effects|SpawnEmitteratLocation "/Game/Assets/InfinityBladeEffects/Effects/FX_Monsters/FX_Monster_Ausar/P_AU_Taunt_sparks.P_AU_Taunt_sparks" (Transformation|GetActorLocation _asbp_enemy_range_projectile))
        (Actor|DestroyActor _asbp_enemy_range_projectile)))))

(event OnComponentBeginOverlap(SpellCollisionVolume)
  (params (OverlappedComponent :type Primitive%20Component%20Object%20Reference) (OtherActor :type Actor%20Object%20Reference) (OtherComp :type Primitive%20Component%20Object%20Reference) (OtherBodyIndex :type Integer) (bFromSweep :type Boolean) (SweepResult :type Hit%20Result%20Structure%20%28by%20ref%29))
  (bind _asbp_spell_base (Utilities|Casting|CastToBP_Spell_Base OtherActor))
  (switch string (Utilities|GetClassDisplayName (Utilities|GetClass _asbp_spell_base))
    (:BP_Spell_Fireball_C
      (Variables|Default|SetIncomingSpell _asbp_spell_base)
      (Variables|Default|GetSpellLaserRef
        (:then)
        (:else
          (Rendering|SetVisibility (Variables|Default|GetSkeletalMesh) false false)
          (Rendering|SetVisibility (Variables|Default|GetParticleSystem) false false)
          (Variables|/Script/Engine.PrimitiveComponent|SetbGenerateOverlapEvents (Variables|Default|GetDamageCollisionVolume) false)
          (CallFunction|BeginMergeFireball)
          (CallFunction|SpawnLaser)
          (Variables|Default|SetLaserActive true))))))

(event Custom|BeginMergeFireball
  (bind _alpha (Timeline|MergingFireball PlayFromStart)
    (:Update
      (bind _incomingspell (Variables|Default|GetIncomingSpell)
        (:then
          (bind _asbp_spell_fireball (Utilities|Casting|CastToBP_Spell_Fireball _incomingspell))
          (Default|ChargingLaser _asbp_spell_fireball _alpha))
        (:else)))
    (:Finished
      (CallFunction|EndLaserSequence))))

(event Custom|EndLaserSequence
  (CallFunction|EndMergeFireball)
  (CallFunction|DestroyLaser)
  (Actor|DestroyActor))

(event Custom|DestroyLaser
  (bind _spelllaserref (Variables|Default|GetSpellLaserRef)
    (:then
      (Default|Cast _spelllaserref))
    (:else)))

(event Custom|SpawnLaser
  (Variables|Default|GetSpellLaserRef
    (:then)
    (:else
      (bind _returnvalue (Game|SpawnActorfromClass "/Game/SpellSystem/SpellComponents/Spells/BP_Spell_Laser1.BP_Spell_Laser1_C" (Math|Transform|MakeTransform "0, 0, 0" "0, 0, 0" "1,1,1") "Undefined" 0 0))
      (bind _output_get (Variables|Default|SetSpellLaserRef _returnvalue))
      (Transformation|AttachComponentToComponent _output_get (Transformation|GetAttachParent (Variables|Default|GetDefaultSceneRoot)) "None" "KeepRelative" "KeepRelative" "KeepRelative" true)
      (Default|Create (Variables|Default|GetSpellLaserRef)))))

(event Custom|EndMergeFireball
  (bind _incomingspell (Variables|Default|GetIncomingSpell)
    (:then
      (bind _asbp_spell_fireball (Utilities|Casting|CastToBP_Spell_Fireball _incomingspell))
      (Default|DestroyFireball _asbp_spell_fireball))
    (:else)))

(event EventBeginPlay
  (|CallParentFunction))

(event EventSetCollisionVolume
  (params (CollisionVolumeForEnemy :type Primitive%20Component%20Object%20Reference) (CollisionVolumeForSpell :type Primitive%20Component%20Object%20Reference))
  (|CallParentFunction 0 (Variables|Default|GetSpellCollisionVolume)))

(event EventTick
  (params (DeltaSeconds :type Float%20%28single-precision%29))
  (if (Variables|Default|GetLaserActive)
    (bind _incomingspell (Variables|Default|GetIncomingSpell)
      (:then
        (Utilities|Casting|CastToBP_Spell_Fireball _incomingspell)
        (if (>= (Math|Vector|VectorLength (- (Transformation|GetActorLocation) (Transformation|GetActorLocation _incomingspell))) 3e+01)
          (CallFunction|EndLaserSequence)))
      (:else))))

(event EventCast
  (bind (_direction _newtrack_0) (Timeline|Timeline_0 Reverse)
    (:Update
      (Transformation|SetRelativeScale3D (Variables|Default|GetSkeletalMesh) (Math|Vector|Lerp(Vector) (Variables|Default|GetSwordInitialSize) (Variables|Default|GetSwordFinalSize) _newtrack_0)))
    (:Finished
      (switch Utilities|FlowControl|Switch|SwitchonETimelineDirection _direction
        (:Backward
          (CallFunction|EndMergeFireball)
          (CallFunction|DestroyLaser)
          (Transformation|DetachFromActor "KeepRelative" "KeepRelative" "KeepRelative")
          (Actor|DestroyActor))))))

(event EventCreate
  (for _array_element (Collision|GetOverlappingActors "/Game/AI/BP_Enemy_Base.BP_Enemy_Base_C" :!class /Script/Engine.Actor)
    (bind _asbp_enemy_base (Utilities|Casting|CastToBP_Enemy_Base _array_element))
    (Utilities|Set|Add (Variables|Default|GetOverlappedEnemy) _asbp_enemy_base))
  (Variables|Default|SetJustSpawned false)
  (Audio|PlaySound2D "/Game/SoundAsset/Spell/Spell_BladeUnshealth.Spell_BladeUnshealth")
  (bind (_direction _newtrack_0) (Timeline|Timeline_0 Play)
    (:Update
      (Transformation|SetRelativeScale3D (Variables|Default|GetSkeletalMesh) (Math|Vector|Lerp(Vector) (Variables|Default|GetSwordInitialSize) (Variables|Default|GetSwordFinalSize) _newtrack_0)))
    (:Finished
      (switch Utilities|FlowControl|Switch|SwitchonETimelineDirection _direction
        (:Backward
          (CallFunction|EndMergeFireball)
          (CallFunction|DestroyLaser)
          (Transformation|DetachFromActor "KeepRelative" "KeepRelative" "KeepRelative")
          (Actor|DestroyActor))))))

(fn ConstructionScript
  (|CallParentFunction)
  (if true
    (Transformation|SetRelativeScale3D (Variables|Default|GetSkeletalMesh) (Variables|Default|GetSwordFinalSize))))