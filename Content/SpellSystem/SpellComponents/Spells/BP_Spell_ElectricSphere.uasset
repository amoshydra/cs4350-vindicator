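; Electric Sphere spell actor that takes its look from a Wind Shield spell and is meant to grow when cast.
; The construction script copies mesh, first material and end scale from a MirroringActor child actor, using that scale as ScaleStart, then destroys the component.
; Cast plays the SpellGrowFactor timeline, but it drives nothing: the scale lerp is unused and Create is empty.
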(event EventBeginPlay
  (|CallParentFunction))

(event Collision|EventActorBeginOverlap
  (params (OtherActor :type Actor%20Object%20Reference))
  (|CallParentFunction OtherActor))

(event EventTick
  (params (DeltaSeconds :type Float%20%28single-precision%29))
  (|CallParentFunction DeltaSeconds))

(event EventCreate)

(event EventCast
  (bind _spheregrowfactor (Timeline|SpellGrowFactor Play)))

(fn ConstructionScript
  (bind _staticmesh (Variables|Default|GetStaticMesh))
  (|CallParentFunction)
  (bind _asbp_spell_wind_shield (Utilities|Casting|CastToBP_Spell_WindShield (Variables|/Script/Engine.ChildActorComponent|GetChildActor (Variables|Default|GetMirroringActor))))
  (Utilities|FlowControl|Sequence
    (:then_0
      (Components|StaticMesh|SetStaticMesh _staticmesh (Variables|/Script/Engine.StaticMeshComponent|GetStaticMesh (Variables|/Game/SpellSystem/SpellComponents/Spells/BP_Spell_Base.BP_Spell_Base_C|GetStaticMesh _asbp_spell_wind_shield))))
    (:then_1
      (bind _output_get (Variables|Default|SetScaleStart (Variables|/Game/SpellSystem/SpellComponents/Spells/BP_Spell_WindShield.BP_Spell_WindShield_C|GetScaleEnd _asbp_spell_wind_shield)))
      (Transformation|SetRelativeScale3D _staticmesh _output_get))
    (:then_2
      (Rendering|Material|SetMaterial _staticmesh 0 (Rendering|Material|GetMaterial (Variables|/Game/SpellSystem/SpellComponents/Spells/BP_Spell_Base.BP_Spell_Base_C|GetStaticMesh _asbp_spell_wind_shield) 0)))
    (:then_3
      (Components|DestroyComponent (Variables|Default|GetMirroringActor)))))