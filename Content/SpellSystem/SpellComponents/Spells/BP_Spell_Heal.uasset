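; Heal spell actor for the spell system, currently providing only the visual effect, with no healing logic in this graph.
; On Create, the Expand timeline plays from the start and drives a uniform relative scale on the particle system.
; The Cast event is an empty stub, and BeginPlay, overlap and Tick are disabled.
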(event EventBeginPlay
  (|CallParentFunction))

(event Collision|EventActorBeginOverlap
  (params (OtherActor :type Actor%20Object%20Reference))
  (|CallParentFunction OtherActor))

(event EventTick
  (params (DeltaSeconds :type Float%20%28single-precision%29))
  (|CallParentFunction DeltaSeconds))

(event EventCreate
  (bind _newtrack_0 (Timeline|Expand PlayFromStart)
    (:Update
      (Transformation|SetRelativeScale3D (Variables|Default|GetParticleSystem) (Math|Vector|MakeVector _newtrack_0 _newtrack_0 _newtrack_0)))))

(event EventCast)

(fn ConstructionScript
  (|CallParentFunction))