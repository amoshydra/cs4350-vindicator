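; BP_Spell_WindBlast is a spell actor that releases an expanding wind effect and slows enemies around it.
; On Cast it activates the Wind particle effect and applies the slow debuff through each enemy's debuff manager, for game instance enemies within Radius.
; An Expand timeline scales the effect up, then deactivates it and destroys the actor once the particle system finishes.
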(event Custom|OnSystemFinished_Event_0
  (params (PSystem :type Particle%20System%20Component%20Object%20Reference))
  (Actor|DestroyActor))

(event EventBeginPlay
  (|CallParentFunction))

(event Collision|EventActorBeginOverlap
  (params (OtherActor :type Actor%20Object%20Reference))
  (|CallParentFunction OtherActor))

(event EventTick
  (params (DeltaSeconds :type Float%20%28single-precision%29))
  (|CallParentFunction DeltaSeconds))

(event EventCast
  (Components|Activation|Activate (Variables|Default|GetWind) false)
  (bind _asbp_game_instance (Utilities|Casting|CastToBP_GameInstance (Game|GetGameInstance)))
  (for _array_element (Variables|/Game/Blueprints/BP_GameInstance.BP_GameInstance_C|GetEnemies _asbp_game_instance)
    (if (<= (Transformation|GetDistanceTo _array_element) (Variables|Default|GetRadius))
      (Default|ActivateDebuff (Variables|/Game/AI/BP_Enemy_Base.BP_Enemy_Base_C|GetBP_Debuff_Manager _array_element) "/Game/SpellSystem/SpellComponents/Debuffs/BP_Debuff_Slow.BP_Debuff_Slow_C")))
  (bind _newtrack_0 (Timeline|Expand PlayFromStart)
    (:Update
      (Transformation|SetRelativeScale3D (Variables|Default|GetWind) (Math|Vector|MakeVector (Math|Float|Lerp 0.25 4.0 _newtrack_0) (Math|Float|Lerp 0.25 4.0 _newtrack_0) (Math|Float|Lerp 0.25 4.0 _newtrack_0))))
    (:Finished
      (CallFunction|Destroy))))

(event EventDestroy
  (bind _wind (Variables|Default|GetWind))
  (EventDispatchers|AssignOnSystemFinished _wind (delegate Custom|OnSystemFinished_Event_0))
  (Components|Activation|Deactivate _wind))

(fn ConstructionScript
  (|CallParentFunction))