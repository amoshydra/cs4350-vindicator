(event OnComponentBeginOverlap(Box)
  (params (OverlappedComponent :type Primitive%20Component%20Object%20Reference) (OtherActor :type Actor%20Object%20Reference) (OtherComp :type Primitive%20Component%20Object%20Reference) (OtherBodyIndex :type Integer) (bFromSweep :type Boolean) (SweepResult :type Hit%20Result%20Structure%20%28by%20ref%29))
  (bind _asbp_enemy_base (Utilities|Casting|CastToBP_Enemy_Base OtherActor))
  (bind _returnvalue (Effects|SpawnEmitterAttached "/Game/Assets/InfinityBladeEffects/Effects/FX_Monsters/FX_Monster_Elemental/Fire/P_Beam_Laser_Fire_Hit.P_Beam_Laser_Fire_Hit" (Variables|/Script/Engine.Character|GetCapsuleComponent _asbp_enemy_base) "None"))
  (Utilities|Map|Add (Variables|Default|GetHitParticles) _asbp_enemy_base _returnvalue)
  (CallFunction|Inflict _asbp_enemy_base false 0.0))

(event OnComponentEndOverlap(Box)
  (params (OverlappedComponent :type Primitive%20Component%20Object%20Reference) (OtherActor :type Actor%20Object%20Reference) (OtherComp :type Primitive%20Component%20Object%20Reference) (OtherBodyIndex :type Integer))
  (bind _asbp_enemy_base (Utilities|Casting|CastToBP_Enemy_Base OtherActor))
  (Components|Activation|Deactivate (.Value (Utilities|Map|Find (Variables|Default|GetHitParticles) _asbp_enemy_base))))

(event EventBeginPlay
  (|CallParentFunction)
  (Collision|SetCollisionEnabled (Variables|Default|GetBox) "NoCollision"))

(event Collision|EventActorBeginOverlap
  (params (OtherActor :type Actor%20Object%20Reference))
  (|CallParentFunction OtherActor))

(event EventTick
  (params (DeltaSeconds :type Float%20%28single-precision%29))
  (|CallParentFunction DeltaSeconds))

(event EventCast
  (Collision|SetCollisionEnabled (Variables|Default|GetBox) "QueryAndPhysics")
  (Components|Activation|Activate (Variables|Default|GetLaser) false)
  (Components|Activation|Deactivate (Variables|Default|GetInitial%20Charge))
  (Utilities|FlowControl|Delay 5.0)
  (Actor|DestroyActor))

(event EventCreate
  (Components|Activation|Activate (Variables|Default|GetInitial%20Charge) false))

(fn ConstructionScript
  (|CallParentFunction))