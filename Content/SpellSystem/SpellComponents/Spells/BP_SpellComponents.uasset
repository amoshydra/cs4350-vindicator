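; Spell helper Blueprint whose ConeSearch function picks out the enemies inside a cone from a given location and forward vector.
; It loops over the supplied enemies, finding each one's angle off the forward vector with a normalized dot product and arccosine.
; Enemies within a hardcoded 20-degree half-angle are returned, with no range check.
; Each computed angle is also printed for debugging.
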(fn ConeSearch
  (params (Location :type Vector) (Forward%20Vector :type Vector) (AllEnemies :type Array%20of%20BP%20Enemy%20Base%20Object%20References))
  (bind _filtered_enemies (LocalVariables|GetFiltered%20Enemies))
  (for _array_element AllEnemies
    (Development|PrintString 0 (Utilities|String|ToString(Float) (Math|Float|Absolute(Float) (Class|KismetMathLibrary|DegAcos (/ (Math|Vector|DotProduct (- (Transformation|GetActorLocation _array_element) Location) Forward%20Vector) (* (Math|Vector|VectorLength (- (Transformation|GetActorLocation _array_element) Location)) (Math|Vector|VectorLength Forward%20Vector)))))))
    (if (<= (Math|Float|Absolute(Float) (Class|KismetMathLibrary|DegAcos (/ (Math|Vector|DotProduct (- (Transformation|GetActorLocation _array_element) Location) Forward%20Vector) (* (Math|Vector|VectorLength (- (Transformation|GetActorLocation _array_element) Location)) (Math|Vector|VectorLength Forward%20Vector))))) 2e+01)
      (Utilities|Array|Add _filtered_enemies _array_element)))
  (return _filtered_enemies))