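; Blizzard spell actor that casts itself on spawn and damages and freezes enemies entering its box.
; Cast starts the snow, aura and initial effects, then the impact and damage field effects after a short delay.
; Box overlaps apply damage, call Inflict, activate the Freeze debuff and record each enemy.
; A timer winds down the effects; when Snow finishes, the actor destroys itself and lifts Freeze from recorded enemies.
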(event OnComponentBeginOverlap(Box)
  (params (OverlappedComponent :type Primitive%20Component%20Object%20Reference) (OtherActor :type Actor%20Object%20Reference) (OtherComp :type Primitive%20Component%20Object%20Reference) (OtherBodyIndex :type Integer) (bFromSweep :type Boolean) (SweepResult :type Hit%20Result%20Structure%20%28by%20ref%29))
  (bind _asbp_enemy_base (Utilities|Casting|CastToBP_Enemy_Base OtherActor))
  (Default|DamageEnemyEvent _asbp_enemy_base 2e+01)
  (CallFunction|Inflict _asbp_enemy_base true 0.0)
  (Default|ActivateDebuff (Variables|/Game/AI/BP_Enemy_Base.BP_Enemy_Base_C|GetBP_Debuff_Manager _asbp_enemy_base) "/Game/SpellSystem/SpellComponents/Debuffs/BP_Debuff_Freeze.BP_Debuff_Freeze_C")
  (Utilities|Array|Add (Variables|Default|GetEnemiesHit) _asbp_enemy_base))

(event Custom|OnSystemFinished_Event_0
  (params (PSystem :type Particle%20System%20Component%20Object%20Reference))
  (Actor|DestroyActor)
  (for _array_element (Variables|Default|GetEnemiesHit)
    (Default|DeactivateDebuff (Variables|/Game/AI/BP_Enemy_Base.BP_Enemy_Base_C|GetBP_Debuff_Manager _array_element) "/Game/SpellSystem/SpellComponents/Debuffs/BP_Debuff_Freeze.BP_Debuff_Freeze_C")))

(event Custom|Set%20Death
  (bind _snow (Variables|Default|GetSnow))
  (Variables|Default|SetisActivated false)
  (EventDispatchers|AssignOnSystemFinished _snow (delegate Custom|OnSystemFinished_Event_0))
  (Components|Activation|Deactivate _snow))

(event EventBeginPlay
  (|CallParentFunction)
  (CallFunction|Create)
  (CallFunction|Cast))

(event Collision|EventActorBeginOverlap
  (params (OtherActor :type Actor%20Object%20Reference))
  (|CallParentFunction OtherActor))

(event EventTick
  (params (DeltaSeconds :type Float%20%28single-precision%29))
  (|CallParentFunction DeltaSeconds))

(event EventCast
  (Variables|Default|SetisActivated true)
  (Components|Activation|Activate (Variables|Default|GetSnow) false)
  (Utilities|FlowControl|Delay 0.7)
  (Components|Activation|Activate (Variables|Default|GetImpact) false)
  (Utilities|Time|SetTimerbyEvent (delegate Custom|Set%20Death) 4.0))

(event EventCreate)

(fn ConstructionScript
  (|CallParentFunction))