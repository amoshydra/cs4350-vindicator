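; VR fireball spell that is held in the hand, thrown on cast and explodes on overlap, inflicting damage and destroying enemy projectiles.
; Cast scales the mesh's physics velocity into a launch velocity for ProjectileMovement.
; Auto-aim picks the enemy nearest the throw direction within an angle tolerance and, if visible and within speed-based reach, substitutes a SuggestProjectileVelocity arc.
; Merge hooks shrink it for laser charging or destroy it after shield merges.
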(event OnComponentBeginOverlap(CollisionVolumeForEnemy)
  (params (OverlappedComponent :type Primitive%20Component%20Object%20Reference) (OtherActor :type Actor%20Object%20Reference) (OtherComp :type Primitive%20Component%20Object%20Reference) (OtherBodyIndex :type Integer) (bFromSweep :type Boolean) (SweepResult :type Hit%20Result%20Structure%20%28by%20ref%29))
  (CallFunction|Inflict OtherActor false 0.0)
  (bind _asbp_enemy_range_projectile (Utilities|Casting|CastToBP_Enemy_Range_Projectile OtherActor)
    (:then
      (Effects|SpawnEmitteratLocation "/Game/Assets/InfinityBladeEffects/Effects/FX_Monsters/FX_Monster_Ausar/P_AU_Taunt_sparks.P_AU_Taunt_sparks" (Transformation|GetActorLocation _asbp_enemy_range_projectile))
      (Actor|DestroyActor _asbp_enemy_range_projectile)
      (Audio|Components|Audio|Stop (Variables|Default|GetOnHandSound)))
    (:CastFailed
      (Utilities|Casting|CastToBP_CI_Steam OtherActor
        (:CastFailed
          (Utilities|Casting|CastToBP_VR_Pawn OtherActor
            (:CastFailed
              (Utilities|Casting|CastToBP_Spell_Base OtherActor
                (:CastFailed
                  (Effects|SpawnEmitteratLocation "/Game/Assets/InfinityBladeEffects/Effects/FX_Monsters/FX_Monster_Ausar/P_AU_Taunt_sparks.P_AU_Taunt_sparks" (Transformation|GetActorLocation))))))))))
  (Audio|PlaySoundatLocation "/Game/SoundAsset/Spell/FireBall_Explosion.FireBall_Explosion" (Transformation|GetActorLocation))
  (Actor|DestroyActor))

(event Custom|ChargingLaser
  (params (Alpha :type Float%20%28single-precision%29))
  (Transformation|SetRelativeScale3D (Variables|Default|GetStaticMesh) (Math|Vector|Lerp(Vector) "0.200000,0.200000,0.200000" "0, 0, 0" Alpha)))

(event Custom|MergeSpell_Shield_EndSequence
  (CallFunction|DestroyFireball))

(event Custom|DestroyFireball
  (Effects|SpawnEmitteratLocation "/Game/Assets/InfinityBladeEffects/Effects/FX_Monsters/FX_Monster_Ausar/P_AU_Taunt_sparks.P_AU_Taunt_sparks" (Transformation|GetActorLocation))
  (Audio|Components|Audio|Stop (Variables|Default|GetOnHandSound))
  (Actor|DestroyActor))

(event Custom|RestoreToDefaultSize
  (Variables|Default|SetInitialScale (Variables|/Script/Engine.SceneComponent|GetRelativeScale3D (Variables|Default|GetStaticMesh)))
  (bind _restoretrack (Timeline|Timeline_0 PlayFromStart)
    (:Update
      (Transformation|SetRelativeScale3D (Variables|Default|GetStaticMesh) (Math|Vector|Lerp(Vector) (Variables|Default|GetInitialScale) "0.200000,0.200000,0.200000" _restoretrack)))))

(event EventBeginPlay
  (|CallParentFunction))

(event EventSetCollisionVolume
  (params (CollisionVolumeForEnemy :type Primitive%20Component%20Object%20Reference) (CollisionVolumeForSpell :type Primitive%20Component%20Object%20Reference))
  (|CallParentFunction (Variables|Default|GetEnemyCollisionVolume) (Variables|Default|GetSpellCollisionVolume)))

(event EventCast
  (Variables|Default|SetisCasted true)
  (Transformation|DetachFromActor "KeepWorld" "KeepWorld" "KeepWorld")
  (bind _returnvalue (Physics|GetPhysicsLinearVelocity (Variables|Default|GetStaticMesh) "None"))
  (Variables|Default|SetInitialVelocity (* _returnvalue (Variables|Default|GetMagnitude)))
  (bind _asbp_game_instance (Utilities|Casting|CastToBP_GameInstance (Game|GetGameInstance)))
  (for _array_element (Variables|/Game/Blueprints/BP_GameInstance.BP_GameInstance_C|GetEnemies _asbp_game_instance)
    (Utilities|IsValid _array_element
      (:Is%20Valid
        (Variables|Default|SetEnemyLocation (Transformation|GetActorLocation _array_element))
        ;[1 1 1] Check if fireball should be auto-targeted to enemy
        (bind _angle (CallFunction|AngleBetweenTwoVectors (- (Variables|Default|GetEnemyLocation) (Transformation|GetActorLocation)) (Math|Vector|Normalize (Variables|Default|GetInitialVelocity))))
        (if (< _angle (Variables|Default|GetAngleTolerance))
          (Variables|Default|SetAngleTolerance _angle)
          (Variables|Default|SetTargetedEnemy _array_element)))))
  (if (Utilities|IsValid (Variables|Default|GetTargetedEnemy))
    (Variables|Default|SetEnemyLocation (Transformation|GetActorLocation (Variables|Default|GetTargetedEnemy)))
    (bind _isvisible (CallFunction|IsEnemyVisible))
    (if _isvisible
      (bind _ispowerfulenough (CallFunction|IsFireballPowerfulEnough))
      (if _ispowerfulenough
        (bind (_tossvelocity _returnvalue_2) (Class|GameplayStatics|BlueprintSuggestProjectileVelocity (Transformation|GetActorLocation) (Variables|Default|GetEnemyLocation) (Math|Vector|VectorLength (Variables|Default|GetInitialVelocity)) 0.0 "DoNotTrace" 0.0 false false))
        (if _returnvalue_2
          (Variables|Default|SetInitialVelocity _tossvelocity)))))
  (CallFunction|SetNewProjectileVelocity (Variables|Default|GetInitialVelocity))
  (Actor|SetLifeSpan 1e+01))

(event Collision|EventHit
  (params (MyComp :type Primitive%20Component%20Object%20Reference) (Other :type Actor%20Object%20Reference) (OtherComp :type Primitive%20Component%20Object%20Reference) (bSelfMoved :type Boolean) (HitLocation :type Vector :default "0, 0, 0") (HitNormal :type Vector :default "0, 0, 0") (NormalImpulse :type Vector :default "0, 0, 0") (Hit :type Hit%20Result%20Structure%20%28by%20ref%29))
  ;[1 1 1] This does not work as no physics is involved
  (Actor|DestroyActor))

(event EventCreate
  (Audio|PlaySoundatLocation "/Game/SoundAsset/Spell/FireBall_Create.FireBall_Create" (Transformation|GetActorLocation))
  (Audio|Components|Audio|Play (Variables|Default|GetOnHandSound) 0.0))

(fn ConstructionScript
  (|CallParentFunction))

(fn AngleBetweenTwoVectors
  (params (Target%20Vector :type Vector) (Directional%20Vector :type Vector))
  (return (Math|Float|Absolute(Float) (Class|KismetMathLibrary|DegAcos (/ (Math|Vector|DotProduct Target%20Vector Directional%20Vector) (* (Math|Vector|VectorLength Target%20Vector) (Math|Vector|VectorLength Directional%20Vector)))))))

(fn CalculateNewVelocity
  (params (InitialVelocity :type Vector) (Target :type Vector) (Origin :type Vector) (Magnitude :type Float%20%28single-precision%29))
  (return (* (Math|Vector|Normalize (- Target Origin)) (* Magnitude (Math|Vector|VectorLength InitialVelocity)))))

(fn SetNewProjectileVelocity
  (params (NewVelocity :type Vector))
  (bind _projectilemovement (Variables|Default|GetProjectileMovement))
  (Variables|/Script/Engine.MovementComponent|SetVelocity _projectilemovement NewVelocity)
  (Variables|/Script/Engine.ProjectileMovementComponent|SetInitialSpeed _projectilemovement 0.0)
  (Variables|/Script/Engine.ProjectileMovementComponent|SetProjectileGravityScale _projectilemovement 1.0)
  (return))

(fn IsEnemyVisible
  (bind _outhit (Collision|LineTraceByChannel (Transformation|GetActorLocation) (Variables|Default|GetEnemyLocation) "TraceTypeQuery1" false 0 "None" true "(R=0.000000,G=0.238765,B=1.000000,A=1.000000)" "(R=0.950359,G=0.000000,B=1.000000,A=1.000000)"))
  (return (== (Variables|Default|GetTargetedEnemy) (.hitactor _outhit))))

(fn IsFireballPowerfulEnough
  (return (>= (* (Math|Vector|VectorLength (Variables|Default|GetInitialVelocity)) 2.0) (Math|Vector|VectorLength (- (Variables|Default|GetEnemyLocation) (Transformation|GetActorLocation))))))