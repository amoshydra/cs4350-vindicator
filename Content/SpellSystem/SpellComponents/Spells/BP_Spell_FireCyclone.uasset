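; Fire cyclone spell actor that waits briefly after spawning, then travels along its relative Y axis.
; A MoveForward timeline scales ProjectileSpeed on each update to offset the root component without sweeping.
; When the timeline finishes, it deactivates the Cyclone, disables collision and destroys itself after a delay.
; Collision overlaps cast to BP_Enemy_Base, but no damage or other effect follows.
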(event OnComponentBeginOverlap(CollisionVolume)
  (params (OverlappedComponent :type Primitive%20Component%20Object%20Reference) (OtherActor :type Actor%20Object%20Reference) (OtherComp :type Primitive%20Component%20Object%20Reference) (OtherBodyIndex :type Integer) (bFromSweep :type Boolean) (SweepResult :type Hit%20Result%20Structure%20%28by%20ref%29))
  (Utilities|Casting|CastToBP_Enemy_Base OtherActor))

(event EventBeginPlay
  (|CallParentFunction)
  (Utilities|FlowControl|Delay 2.0)
  (CallFunction|Cast))

(event Collision|EventActorBeginOverlap
  (params (OtherActor :type Actor%20Object%20Reference))
  (|CallParentFunction OtherActor))

(event EventTick
  (params (DeltaSeconds :type Float%20%28single-precision%29))
  (|CallParentFunction DeltaSeconds))

(event EventCast
  (bind _newtrack_0 (Timeline|Move%20Forward PlayFromStart)
    (:Update
      (Transformation|AddRelativeLocation (Variables|Default|GetDefaultSceneRoot) (* (Math|Vector|MakeVector 0.0 (Variables|Default|GetProjectileSpeed) 0.0) _newtrack_0) false false))
    (:Finished
      (CallFunction|Destroy))))

(event EventDestroy
  (Components|Activation|Deactivate (Variables|Default|GetCyclone))
  (Collision|SetCollisionEnabled (Variables|Default|GetCollisionVolume) "NoCollision")
  (Utilities|FlowControl|Delay 2.0)
  (Actor|DestroyActor))

(fn ConstructionScript
  (|CallParentFunction))