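; Forked lightning spell actor that stuns enemies within a cone in front of it, casting two seconds after spawn.
; Casting swaps the initial shock and sphere visuals for an aftershock effect, then cone-searches the GameInstance's enemy list.
; Each target gets a lightning emitter rotated toward it from the spell, a stun debuff and a zero-value damage event.
; After another short delay, the stored emitters and aftershock deactivate.
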(event EventBeginPlay
  (|CallParentFunction)
  (Utilities|FlowControl|Delay 2.0)
  (CallFunction|Cast))

(event Collision|EventActorBeginOverlap
  (params (OtherActor :type Actor%20Object%20Reference))
  (|CallParentFunction OtherActor))

(event EventTick
  (params (DeltaSeconds :type Float%20%28single-precision%29))
  (|CallParentFunction DeltaSeconds))

(event EventCast
  (bind _returnvalue (Transformation|GetActorLocation))
  (bind _particles (Variables|Default|Getparticles))
  (Components|Activation|Deactivate (Variables|Default|GetInitialShock))
  (Rendering|SetVisibility (Variables|Default|GetStaticMesh) false false)
  (bind _asbp_game_instance (Utilities|Casting|CastToBP_GameInstance (Game|GetGameInstance)))
  (bind _enemies (CallFunction|ConeSearch (Transformation|GetActorLocation) (Transformation|GetActorForwardVector) (Variables|/Game/Blueprints/BP_GameInstance.BP_GameInstance_C|GetEnemies _asbp_game_instance) 2e+01))
  (Components|Activation|Activate (Variables|Default|GetAfterShock) false)
  (for _array_element _enemies
    (bind _returnvalue_2 (Effects|SpawnEmitteratLocation "/Game/Assets/InfinityBladeEffects/Effects/FX_Monsters/FX_Monster_Genno/P_Genno_Weapon_Lightning_01.P_Genno_Weapon_Lightning_01" _returnvalue (Math|Rotator|MakeRotator (.roll (Math|Rotator|FindLookatRotation _returnvalue (Transformation|GetActorLocation _array_element))) (- (.pitch (Math|Rotator|FindLookatRotation _returnvalue (Transformation|GetActorLocation _array_element))) 9e+01) (.yaw (Math|Rotator|FindLookatRotation _returnvalue (Transformation|GetActorLocation _array_element))))))
    (Utilities|Array|Add _particles _returnvalue_2)
    (Default|ActivateDebuff (Variables|/Game/AI/BP_Enemy_Base.BP_Enemy_Base_C|GetBP_Debuff_Manager _array_element) "/Game/SpellSystem/SpellComponents/Debuffs/BP_Debuff_Stun.BP_Debuff_Stun_C")
    (Default|DamageEnemyEvent _array_element 0.0))
  (Utilities|FlowControl|Delay 2.0)
  (for _array_element_2 _particles
    (Components|Activation|Deactivate _array_element_2))
  (Components|Activation|Deactivate (Variables|Default|GetAfterShock)))

(fn ConstructionScript
  (|CallParentFunction))