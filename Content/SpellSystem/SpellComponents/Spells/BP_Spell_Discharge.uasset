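; Discharge spell actor that inflicts its effect on enemies overlapping its sphere.
; BeginPlay spawns a discharge particle burst at the actor's location.
; Each overlapping BP_Enemy_Base receives Inflict without alternate damage and gets an enlarged hit emitter attached to its root.
; The Create event plays the cast sound and immediately destroys the actor.
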(event OnComponentBeginOverlap(Sphere)
  (params (OverlappedComponent :type Primitive%20Component%20Object%20Reference) (OtherActor :type Actor%20Object%20Reference) (OtherComp :type Primitive%20Component%20Object%20Reference) (OtherBodyIndex :type Integer) (bFromSweep :type Boolean) (SweepResult :type Hit%20Result%20Structure%20%28by%20ref%29))
  (bind _asbp_enemy_base (Utilities|Casting|CastToBP_Enemy_Base OtherActor))
  (CallFunction|Inflict _asbp_enemy_base false 0.0)
  (bind _returnvalue (Effects|SpawnEmitterAttached "/Game/SpellSystem/SpellComponents/Spells/CustomAssets/Discharge/P_HitDischarge.P_HitDischarge" (Variables|/Script/Engine.Actor|GetRootComponent _asbp_enemy_base) "None"))
  (Transformation|SetRelativeScale3D _returnvalue "3.000000,3.000000,3.000000"))

(event EventBeginPlay
  (|CallParentFunction)
  (Effects|SpawnEmitteratLocation "/Game/SpellSystem/SpellComponents/Spells/CustomAssets/Discharge/P_Discharge.P_Discharge" (Transformation|GetActorLocation)))

(event Collision|EventActorBeginOverlap
  (params (OtherActor :type Actor%20Object%20Reference))
  (|CallParentFunction OtherActor))

(event EventCreate
  (Audio|PlaySoundatLocation "/Game/SoundAsset/Spell/Discharge_Cast.Discharge_Cast" (Transformation|GetActorLocation))
  (Actor|DestroyActor))

(event EventTick
  (params (DeltaSeconds :type Float%20%28single-precision%29))
  (|CallParentFunction DeltaSeconds))

(fn ConstructionScript
  (|CallParentFunction))