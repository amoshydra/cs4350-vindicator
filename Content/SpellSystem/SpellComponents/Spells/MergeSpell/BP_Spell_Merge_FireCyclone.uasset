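; Fire Cyclone merge spell, built from two spells and cast as a forward-moving projectile that knocks enemies away.
; A creation timeline scales the mesh up while driving both source spells' effects, then casts on completion.
; Overlapped BP_Enemy_Base actors are launched along its forward vector, get an impact emitter and receive damage.
; A timer ends the particle and overlaps, destroying the actor when the system finishes; Destroy instead shrinks it away.
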(event OnComponentBeginOverlap(EnemyDetecionVolume)
  (params (OverlappedComponent :type Primitive%20Component%20Object%20Reference) (OtherActor :type Actor%20Object%20Reference) (OtherComp :type Primitive%20Component%20Object%20Reference) (OtherBodyIndex :type Integer) (bFromSweep :type Boolean) (SweepResult :type Hit%20Result%20Structure%20%28by%20ref%29))
  (bind _returnvalue (Transformation|GetActorForwardVector))
  (bind _returnvalue_2 (* _returnvalue 3e+03))
  (bind _asbp_enemy_base (Utilities|Casting|CastToBP_Enemy_Base OtherActor))
  (Character|LaunchCharacter _asbp_enemy_base (Math|Vector|MakeVector (.x _returnvalue_2) (.y _returnvalue_2) 0.0) true false)
  (Effects|SpawnEmitteratLocation "/Game/Assets/InfinityBladeEffects/Effects/FX_Mobile/Impacts/P_Impact_Shie_2.P_Impact_Shie_2" (Transformation|GetActorLocation _asbp_enemy_base))
  (CallFunction|Inflict _asbp_enemy_base false 0.0))

(event Custom|End%20Particle
  (bind _cyclone (Variables|Default|GetCyclone))
  (EventDispatchers|AssignOnSystemFinished _cyclone (delegate Custom|OnSystemFinished_Event_0))
  (Components|Activation|Deactivate _cyclone)
  (Variables|/Script/Engine.PrimitiveComponent|SetbGenerateOverlapEvents (Variables|Default|GetEnemyDetecionVolume) false))

(event Custom|InteruptCreationProcess
  (bind _creationtrack (Timeline|FireCycloneCreation Stop)
    (:Update
      (if (Utilities|Name|Equal(Name) (Variables|Default|GetcurrentState) "Creating")
        (Transformation|SetRelativeScale3D (Variables|Default|GetStaticMesh) (Math|Vector|Lerp(Vector) (Variables|Default|GetInitialSize) (Variables|Default|GetFinalSize) _creationtrack))
        (Default|ActivateEffect (Variables|Default|GetSpellRef1) 0 _creationtrack)
        (Default|ActivateEffect (Variables|Default|GetSpellRef2) 0 _creationtrack)
        (else
          (CallFunction|InteruptCreationProcess))))
    (:Finished
      (CallFunction|Cast))))

(event Custom|OnSystemFinished_Event_0
  (params (PSystem :type Particle%20System%20Component%20Object%20Reference))
  (Actor|DestroyActor self))

(event EventBeginPlay
  (|CallParentFunction))

(event Collision|EventActorBeginOverlap
  (params (OtherActor :type Actor%20Object%20Reference))
  (|CallParentFunction OtherActor))

(event EventSpawnMergeSpell
  (params (Spell1 :type BP%20Spell%20Basic%20Object%20Reference) (Spell2 :type BP%20Spell%20Basic%20Object%20Reference))
  (Variables|Default|SetSpellRef1 Spell1)
  (Variables|Default|SetSpellRef2 Spell2)
  (CallFunction|Create))

(event EventTick
  (params (DeltaSeconds :type Float%20%28single-precision%29))
  (|CallParentFunction DeltaSeconds)
  (Default|CallEventTickDispatcher))

(event Collision|EventHit
  (params (MyComp :type Primitive%20Component%20Object%20Reference) (Other :type Actor%20Object%20Reference) (OtherComp :type Primitive%20Component%20Object%20Reference) (bSelfMoved :type Boolean) (HitLocation :type Vector :default "0, 0, 0") (HitNormal :type Vector :default "0, 0, 0") (NormalImpulse :type Vector :default "0, 0, 0") (Hit :type Hit%20Result%20Structure%20%28by%20ref%29)))

(event EventCreate
  (Variables|Default|SetcurrentState "Creating")
  (CallFunction|InteruptCreationProcess)
  (bind _creationtrack (Timeline|FireCycloneCreation PlayFromStart)
    (:Update
      (if (Utilities|Name|Equal(Name) (Variables|Default|GetcurrentState) "Creating")
        (Transformation|SetRelativeScale3D (Variables|Default|GetStaticMesh) (Math|Vector|Lerp(Vector) (Variables|Default|GetInitialSize) (Variables|Default|GetFinalSize) _creationtrack))
        (Default|ActivateEffect (Variables|Default|GetSpellRef1) 0 _creationtrack)
        (Default|ActivateEffect (Variables|Default|GetSpellRef2) 0 _creationtrack)
        (else
          (CallFunction|InteruptCreationProcess))))
    (:Finished
      (CallFunction|Cast))))

(event EventDestroy
  (Variables|Default|SetcurrentState "Destroying")
  (bind _creationtrack (Timeline|Timeline_0 PlayFromStart)
    (:Update
      (Transformation|SetRelativeScale3D (Variables|Default|GetStaticMesh) (Math|Vector|Lerp(Vector) (Variables|/Script/Engine.SceneComponent|GetRelativeScale3D (Variables|Default|GetStaticMesh)) (Variables|Default|GetInitialSize) _creationtrack)))
    (:Finished
      (Actor|DestroyActor))))

(event EventCast
  (bind _projectilemovement (Variables|Default|GetProjectileMovement))
  (Variables|Default|SetcurrentState "Casting")
  (Components|Activation|Activate _projectilemovement false)
  (Transformation|SetRelativeScale3D (Variables|Default|GetStaticMesh) (Variables|Default|GetCastingSize))
  (Variables|/Script/Engine.MovementComponent|SetVelocity _projectilemovement (* (Transformation|GetActorForwardVector) 6e+02))
  (Utilities|Time|SetTimerbyEvent (delegate Custom|End%20Particle) 2.0))

(fn ConstructionScript
  (bind _staticmesh (Variables|Default|GetStaticMesh))
  (|CallParentFunction)
  (Transformation|SetRelativeScale3D _staticmesh (Variables|Default|GetInitialSize))
  (if (Variables|Default|GetCheckFinalSize)
    (Variables|Default|SetCheckFinalSize false)
    (Transformation|SetRelativeScale3D _staticmesh (Variables|Default|GetFinalSize))))