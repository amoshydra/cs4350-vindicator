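; Basic lightning blade spell that extends on Create and, on Cast, retracts, then detaches and destroys itself.
; A timeline scales the skeletal mesh along X, played forward to extend and in reverse to retract.
; Enemies overlapping at Create are only recorded; later entries into the damage volume are tracked, inflicted with damage and given sparks.
; Spell collider handlers are empty, with fireball-to-laser and projectile-destroying interactions left disconnected.
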(event OnComponentEndOverlap(DamageCollisionVolume)
  (params (OverlappedComponent :type Primitive%20Component%20Object%20Reference) (OtherActor :type Actor%20Object%20Reference) (OtherComp :type Primitive%20Component%20Object%20Reference) (OtherBodyIndex :type Integer))
  (bind _asbp_enemy_base (Utilities|Casting|CastToBP_Enemy_Base OtherActor))
  (Utilities|Set|Remove (Variables|Default|GetOverlappedEnemy) _asbp_enemy_base))

(event OnComponentEndOverlap(SpellCollider)
  (params (OverlappedComponent :type Primitive%20Component%20Object%20Reference) (OtherActor :type Actor%20Object%20Reference) (OtherComp :type Primitive%20Component%20Object%20Reference) (OtherBodyIndex :type Integer)))

(event OnComponentBeginOverlap(DamageCollisionVolume)
  (params (OverlappedComponent :type Primitive%20Component%20Object%20Reference) (OtherActor :type Actor%20Object%20Reference) (OtherComp :type Primitive%20Component%20Object%20Reference) (OtherBodyIndex :type Integer) (bFromSweep :type Boolean) (SweepResult :type Hit%20Result%20Structure%20%28by%20ref%29))
  (if (not (Variables|Default|GetJustSpawned))
    (bind _asbp_enemy_base (Utilities|Casting|CastToBP_Enemy_Base OtherActor))
    (bind _returnvalue (Utilities|Set|Add (Variables|Default|GetOverlappedEnemy) _asbp_enemy_base))
    (if _returnvalue
      (CallFunction|Inflict _asbp_enemy_base false 0.0)
      (Effects|SpawnEmitteratLocation "/Game/Assets/InfinityBladeEffects/Effects/FX_Monsters/FX_Monster_Ausar/P_AU_Taunt_sparks.P_AU_Taunt_sparks" (Transformation|GetActorLocation _asbp_enemy_base)))))

(event OnComponentBeginOverlap(SpellCollider)
  (params (OverlappedComponent :type Primitive%20Component%20Object%20Reference) (OtherActor :type Actor%20Object%20Reference) (OtherComp :type Primitive%20Component%20Object%20Reference) (OtherBodyIndex :type Integer) (bFromSweep :type Boolean) (SweepResult :type Hit%20Result%20Structure%20%28by%20ref%29)))

(event Custom|SetCollisionVolume
  (params (CollisionVolumeForEnemy :type Primitive%20Component%20Object%20Reference) (CollisionVolumeForSpell :type Primitive%20Component%20Object%20Reference)))

(event EventBeginPlay
  (|CallParentFunction))

(event EventCast
  (bind (_direction _newtrack_0) (Timeline|Timeline_0 Reverse)
    (:Update
      (Transformation|SetRelativeScale3D (Variables|Default|GetSkeletalMesh) (Math|Vector|Lerp(Vector) "0.010000,0.187500,0.156250" "0.312500,0.187500,0.156250" _newtrack_0)))
    (:Finished
      (switch Utilities|FlowControl|Switch|SwitchonETimelineDirection _direction
        (:Backward
          (Transformation|DetachFromActor "KeepRelative" "KeepRelative" "KeepRelative")
          (Actor|DestroyActor))))))

(event EventCreate
  (for _array_element (Collision|GetOverlappingActors "/Game/AI/BP_Enemy_Base.BP_Enemy_Base_C" :!class /Script/Engine.Actor)
    (bind _asbp_enemy_base (Utilities|Casting|CastToBP_Enemy_Base _array_element))
    (Utilities|Set|Add (Variables|Default|GetOverlappedEnemy) _asbp_enemy_base))
  (Variables|Default|SetJustSpawned false)
  (bind (_direction _newtrack_0) (Timeline|Timeline_0 Play)
    (:Update
      (Transformation|SetRelativeScale3D (Variables|Default|GetSkeletalMesh) (Math|Vector|Lerp(Vector) "0.010000,0.187500,0.156250" "0.312500,0.187500,0.156250" _newtrack_0)))
    (:Finished
      (switch Utilities|FlowControl|Switch|SwitchonETimelineDirection _direction
        (:Backward
          (Transformation|DetachFromActor "KeepRelative" "KeepRelative" "KeepRelative")
          (Actor|DestroyActor))))))

(fn ConstructionScript
  (|CallParentFunction))